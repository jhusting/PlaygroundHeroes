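; SimpleHurtBox is a damage volume that hurts overlapping JHero actors by subtracting DamageInflicted directly from their Health.
; While DamageActive is set, overlap begin either applies a single hit or, in ContinuousDamage mode, only registers the hero in OtherActors.
; Tick uses a Delay to pace repeated hits on every tracked hero in continuous mode.
; Overlap end removes actors from the list.
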(event EventBeginPlay)

(event Collision|EventActorBeginOverlap
  (params (OtherActor :type Actor%20Object%20Reference))
  (if (Variables|Default|GetDamageActive)
    (bind _asjhero (Utilities|Casting|CastToJHero OtherActor))
    (if (Variables|Default|GetContinuousDamage)
      _
      (else
        ;[1 1 1] Deal damage once
        (Variables|/Script/PlaygroundHeroes.JHero|SetHealth _asjhero (- (Variables|/Script/PlaygroundHeroes.JHero|GetHealth _asjhero) (Variables|Default|GetDamageInflicted)))))
    (Utilities|Array|AddUnique (Variables|Default|GetOtherActors) _asjhero)))

(event EventTick
  (params (DeltaSeconds :type Float%20%28single-precision%29))
  (if (Variables|Default|GetContinuousDamage)
    (if (Variables|Default|GetDamageActive)
      (Utilities|FlowControl|Delay (Variables|Default|GetDelayBetweenDamageHits))
      (for _array_element (Variables|Default|GetOtherActors)
        (bind _asjhero (Utilities|Casting|CastToJHero _array_element))
        (Variables|/Script/PlaygroundHeroes.JHero|SetHealth _asjhero (- (Variables|/Script/PlaygroundHeroes.JHero|GetHealth _asjhero) (Variables|Default|GetDamageInflicted)))))))

(event Collision|EventActorEndOverlap
  (params (OtherActor :type Actor%20Object%20Reference))
  (Utilities|Array|RemoveItem (Variables|Default|GetOtherActors) OtherActor))

(fn ConstructionScript)