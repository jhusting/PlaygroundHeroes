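; Shooting wall actor that fires an ArrowBP roughly every five seconds, using a Delay on Tick as a repeating timer.
; Each arrow spawns at the root's location plus a rotated SpawnOffset, facing the root's rotation.
; An impulse of InitialSpawnSpeed, not rotated to the wall's facing, launches the Arrow component, and a debug message prints per shot.
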(event EventBeginPlay)

(event Collision|EventActorBeginOverlap
  (params (OtherActor :type Actor%20Object%20Reference)))

(event EventTick
  (params (DeltaSeconds :type Float%20%28single-precision%29))
  (bind _defaultsceneroot (Variables|Default|GetDefaultSceneRoot))
  (bind _returnvalue (Transformation|GetWorldRotation _defaultsceneroot))
  (Utilities|FlowControl|Delay 5.0)
  (bind _returnvalue_2 (Game|SpawnActorfromClass "/Game/Blueprints/Warriors/ArrowBP.ArrowBP_C" (Math|Transform|MakeTransform (+ (Transformation|GetWorldLocation _defaultsceneroot) (Math|Vector|RotateVector (Variables|Default|GetSpawnOffset) _returnvalue)) _returnvalue) "Undefined" 0 0))
  (Physics|AddImpulse (Variables|/Game/Blueprints/Warriors/ArrowBP.ArrowBP_C|GetArrow _returnvalue_2) (Variables|Default|GetInitialSpawnSpeed) "None" false)
  (Development|PrintString "Shooting Wall: Arrow shot" true true "(R=0.000000,G=0.660000,B=1.000000,A=1.000000)" 0.5))

(fn ConstructionScript)