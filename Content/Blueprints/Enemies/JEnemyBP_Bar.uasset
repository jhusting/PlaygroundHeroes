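; Enemy actor Blueprint with health bars, regeneration and death, plus yaw-only target turning and Knight/Archer hit sounds.
; BeginPlay links the health bar widget to itself and adds a second one owned by player index 1, or hides it when bars are off.
; Tick computes health percent, then calls Die at zero if allowed, otherwise regenerates per frame, independent of delta time.
; AddHealthBP forwards health changes unless the enemy is invincible.
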(event EventBeginPlay
  (if (Variables|Default|GetbBarsVisible)
    (bind _aspolished_health_bar (Utilities|Casting|CastToPolishedHealthBar (UserInterface|GetUserWidgetObject (Variables|Default|GetHealthBarWidget))))
    (Variables|/Game/Blueprints/UI/PolishedHealthBar.PolishedHealthBar_C|SetEnemyBP _aspolished_health_bar self)
    (Utilities|FlowControl|Delay 0.2)
    (bind _returnvalue (AddComponent|AddWidgetComponent false))
    (Class|UserWidget|SetOwningPlayer (UserInterface|GetUserWidgetObject _returnvalue) (Game|GetPlayerController 1))
    (Class|WidgetComponent|SetOwnerPlayer _returnvalue (Class|Widget|GetOwningLocalPlayer (UserInterface|GetUserWidgetObject _returnvalue)))
    (bind _aspolished_health_bar_2 (Utilities|Casting|CastToPolishedHealthBar (UserInterface|GetUserWidgetObject _returnvalue)))
    (Variables|/Game/Blueprints/UI/PolishedHealthBar.PolishedHealthBar_C|SetEnemyBP _aspolished_health_bar_2 self)
    (else
      (Rendering|SetVisibility (Variables|Default|GetHealthBarWidget) false false))))

(event Collision|EventActorBeginOverlap
  (params (OtherActor :type Actor%20Object%20Reference)))

(event EventTick
  (params (DeltaSeconds :type Float%20%28single-precision%29))
  (Class|JEnemy|UpdateHitTimes 0.0)
  ;[1 1 1] Update Health Percentage (thus updatingHealth Bar)
  (bind _output_get (Variables|Default|SetHealthPercent (Math|Float|Clamp(Float) (/ (Variables|Default|GetHealth) (Variables|Default|GetmaxHealth)))))
  ;[1 1 1] <DEATH>: If 0.0%, destroy parent
  (if (== 0.0 _output_get)
    (if (Variables|Default|GetbCanDie)
      (CallFunction|Die))
    (else
      ;[1 1 1] <REGEN> Add N% every tick
      (Variables|Default|SetHealth (Math|Float|Clamp(Float) (+ (Variables|Default|GetHealth) (/ (Variables|Default|GetHealthRegenSpeed) 1e+02)) 0.0 (Variables|Default|GetmaxHealth))))))

(fn ConstructionScript)

(fn Die
  (Actor|DestroyActor))

(fn RotateTowardsTarget
  (params (DeltaTime :type Float%20%28single-precision%29) (Focus :type Actor%20Object%20Reference) (Instant? :type Boolean))
  (if (Utilities|IsValid Focus)
    (Transformation|SetActorRotation (Class|KismetMathLibrary|RInterptoConstant (Transformation|GetActorRotation) (Math|Rotator|MakeRotator 0.0 0.0 (.Yaw (Math|Rotator|BreakRotator (Math|Rotator|FindLookatRotation (Transformation|GetActorLocation) (Transformation|GetActorLocation Focus))))) DeltaTime (Variables|Default|GetRotationSpeed)))))

(fn PlayHitSound
  (params (moveName :type String) (hitLocation :type Vector))
  (switch string moveName
    (:KnightAttack1
      (Audio|PlaySoundatLocation (Variables|sounds|GetSwordHitSound) hitLocation "0, 0, 0" (Variables|Sounds|GetSwordHitVolume) (Variables|Sounds|GetSwordHitPitch) 0.0 0 0 0 :!label _label))
    (:KnightAttack2
      (goto _label))
    (:KnightAttack3
      (Audio|PlaySoundatLocation (Variables|Sounds|GetswordCritSound) hitLocation "0, 0, 0" (Variables|Sounds|GetSwordCritVolume) (Variables|Sounds|GetSwordCritPitch) 0.0 0 0 0))
    (:ArcherHit
      (Audio|PlaySoundatLocation (Variables|Sounds|GetarrowHitSound) hitLocation "0, 0, 0" (Variables|Sounds|GetarrowHitVolume) (Variables|Sounds|GetarrowHitPitch) 0.0 0 0 0))
    (:ArcherCrit
      (Audio|PlaySoundatLocation (Variables|Sounds|GetarrowCritSound) hitLocation "0, 0, 0" (Variables|Sounds|GetarrowCritVolume) (Variables|Sounds|GetarrowCritPitch) 0.0 0 0 0))))

(fn AddHealthBP
  (params (Change :type Float%20%28single-precision%29) (MoveName :type String))
  (if (not (Variables|Default|Getinvincible))
    (Class|JEnemy|AddHealth self Change MoveName)))