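; Enemy Blueprint with regenerating health and two health bars, one on a widget component and one on the second player's screen.
; BeginPlay links the double-layer bar widget to this enemy.
; Each Tick updates hit times and health percent, destroys the actor at zero, otherwise regenerates health up to max.
; Tick also creates the second player's TestBar once, then updates it; an on-screen projection check is left unconnected.
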(event EventBeginPlay
  (bind _asdouble_layer_enemy_health_bar (Utilities|Casting|CastToDoubleLayerEnemyHealthBar (UserInterface|GetUserWidgetObject (Variables|Default|GetHealthBarWidget))))
  (Variables|/Game/Blueprints/UI/DoubleLayerEnemyHealthBar.DoubleLayerEnemyHealthBar_C|SetEnemyBP _asdouble_layer_enemy_health_bar self))

(event Collision|EventActorBeginOverlap
  (params (OtherActor :type Actor%20Object%20Reference)))

(event EventTick
  (params (DeltaSeconds :type Float%20%28single-precision%29))
  (Class|JEnemy|UpdateHitTimes 0.0)
  ;[1 1 1] Update Health Percentage (thus updatingHealth Bar)
  (bind _asjenemy (Utilities|Casting|CastToJEnemy self))
  (bind _output_get (Variables|/Script/PlaygroundHeroes.JEnemy|SetHealthPercent _asjenemy (/ (Variables|/Script/PlaygroundHeroes.JEnemy|GetHealth _asjenemy) (Variables|/Script/PlaygroundHeroes.JEnemy|GetmaxHealth _asjenemy))))
  ;[1 1 1] <DEATH>: If 0.0%, destroy parent
  (if (== _output_get 0.0)
    (Actor|DestroyActor)
    (else
      ;[1 1 1] <REGEN> Add N% every tick
      (Variables|/Script/PlaygroundHeroes.JEnemy|SetHealth _asjenemy (+ (Variables|/Script/PlaygroundHeroes.JEnemy|GetHealth _asjenemy) (/ (Variables|Default|GetHealthRegenSpeed) 1e+02)))
      ;[1 1 1] If Health>Max Health: Health = Max Health
      (if (> (Variables|/Script/PlaygroundHeroes.JEnemy|GetHealth _asjenemy) (Variables|/Script/PlaygroundHeroes.JEnemy|GetmaxHealth _asjenemy))
        (Variables|/Script/PlaygroundHeroes.JEnemy|SetHealth _asjenemy (Variables|/Script/PlaygroundHeroes.JEnemy|GetmaxHealth _asjenemy)))
      (if (Utilities|IsValid (Variables|Default|GetPlayer2HealthBar))
        (Default|Update (Variables|Default|GetPlayer2HealthBar))
        (else
          (Utilities|FlowControl|DoOnce false
            (:Completed
              (bind _returnvalue (UserInterface|CreateWidget "/Game/Blueprints/UI/TestBar.TestBar_C" (Game|GetPlayerController 1)))
              (Variables|/Game/Blueprints/UI/TestBar.TestBar_C|SetEnemy _returnvalue self)
              (UserInterface|Viewport|AddtoPlayerScreen _returnvalue)
              (Variables|Default|SetPlayer2HealthBar _returnvalue))))))))

(fn ConstructionScript)