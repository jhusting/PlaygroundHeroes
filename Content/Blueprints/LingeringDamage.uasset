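; LingeringDamage is an actor that applies a damage-over-time effect to a Host for a limited lifetime.
; Each tick it counts LifeSpan down, destroying itself at zero, and snaps its transform to the Host's without sweep.
; It also passes Damage scaled by delta time to the Host's AddHealth, so the sign of Damage decides whether health drops or rises.
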(event EventBeginPlay)

(event Collision|EventActorBeginOverlap
  (params (OtherActor :type Actor%20Object%20Reference)))

(event EventTick
  (params (DeltaSeconds :type Float%20%28single-precision%29))
  (bind _host (Variables|Default|GetHost))
  (CallFunction|LifeTimer DeltaSeconds)
  (Transformation|SetActorTransform (Transformation|GetActorTransform _host))
  (CallFunction|DoDamage _host DeltaSeconds))

(fn ConstructionScript)

(fn LifeTimer
  (params (DeltaSeconds :type Float%20%28single-precision%29))
  (bind _output_get (Variables|Default|SetlifeSpan (- (Variables|Default|GetlifeSpan) DeltaSeconds)))
  (if (>= 0.0 _output_get)
    (Actor|DestroyActor)))

(fn DoDamage
  (params (victim :type J%20Hero%20Object%20Reference) (DeltaSeconds :type Float%20%28single-precision%29))
  (Class|JHero|AddHealth victim (* DeltaSeconds (Variables|Default|Getdamage))))