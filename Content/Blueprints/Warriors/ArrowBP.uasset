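; Arrow projectile for the archer that damages JEnemyBP_Bar enemies on overlap, plays their hit sound and destroys itself.
; Once projectile movement starts simulating, it enables capsule overlaps, activates particles and plays a charge-dependent release sound.
; Crit is evaluated on impact from the first-found JArcherBP's hold time, setting impact effect size and the "ArcherCrit" move name.
; Floating combat text and trail functions exist but never run here.
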(event EventBeginPlay
  (bind _outactors (Actor|GetAllActorsOfClass "/Game/Blueprints/Warriors/JArcherBP.JArcherBP_C"))
  (bind _output_get (Variables|Default|SetArcherReference (Utilities|Array|Get(acopy) _outactors)))
  (Utilities|IsValid _output_get
    (:Is%20Not%20Valid
      (Development|PrintString "ArrowBP: JArcher BP not found"))))

(event EventTick
  (params (DeltaSeconds :type Float%20%28single-precision%29))
  (if (Variables|/Script/Engine.ProjectileMovementComponent|GetbSimulationEnabled (Variables|Default|GetProjectileMovement))
    (Utilities|FlowControl|DoOnce false
      (:Completed
        (Variables|/Script/Engine.PrimitiveComponent|SetbGenerateOverlapEvents (Variables|Default|GetCapsule) true)
        (Components|Activation|Activate (Variables|Default|GetParticleSystem) false)
        (CallFunction|MakeRealeaseNoise)))))

(event Collision|EventActorBeginOverlap
  (params (OtherActor :type Actor%20Object%20Reference))
  (bind _asjenemy_bp_bar (Utilities|Casting|CastToJEnemyBP_Bar OtherActor))
  (CallFunction|SpawnParticleEffectonCrit _asjenemy_bp_bar)
  (if (Variables|Default|GetisCrit)
    (Variables|Default|SetmoveName "ArcherCrit"))
  (Default|AddHealthBP _asjenemy_bp_bar (* (Variables|Default|GetArrowDamage) -1.0) (Variables|Default|GetmoveName))
  (Default|PlayHitSound _asjenemy_bp_bar (Variables|Default|GetmoveName) (Transformation|GetActorLocation))
  (Actor|DestroyActor))

(fn ConstructionScript)

(fn SpawnFloatingCombatText
  (params (Damage :type Float%20%28single-precision%29) (HitActor :type J%20Enemy%20Object%20Reference))
  (bind _returnvalue (UserInterface|CreateWidget "/Game/Blueprints/UI/FloatingDamageNumbers.FloatingDamageNumbers_C" (Game|GetPlayerController 0) Damage HitActor))
  (UserInterface|Viewport|AddtoPlayerScreen _returnvalue)
  (bind _returnvalue_2 (UserInterface|CreateWidget "/Game/Blueprints/UI/FloatingDamageNumbers.FloatingDamageNumbers_C" (Game|GetPlayerController 1) Damage HitActor))
  (UserInterface|Viewport|AddtoPlayerScreen _returnvalue_2))

(fn SpawnParticleEffectonCrit
  (params (HitActor :type Actor%20Object%20Reference))
  (bind _returnvalue (Transformation|GetActorRotation))
  (bind _returnvalue_2 (Transformation|GetActorRotation))
  (bind _archerreference (Variables|Default|GetArcherReference))
  (bind (_roll _pitch _yaw) (Math|Rotator|BreakRotator _returnvalue))
  (bind (_roll_2 _pitch_2 _yaw_2) (Math|Rotator|BreakRotator _returnvalue_2))
  (bind _output_get (Variables|Default|SetisCrit (>= (/ (Variables|/Script/PlaygroundHeroes.JArcher|GettimeHeld _archerreference) (Variables|/Script/PlaygroundHeroes.JArcher|GetHoldTimeNeeded _archerreference)) 1.0)))
  (if _output_get
    (Effects|SpawnEmitteratLocation (Variables|Default|GetCritParticle) (Transformation|GetActorLocation) (Math|Rotator|MakeRotator _roll (+ _pitch 9e+01) _yaw) "0.400000,0.400000,0.400000")
    (else
      (Effects|SpawnEmitteratLocation (Variables|Default|GetCritParticle) (Transformation|GetActorLocation) (Math|Rotator|MakeRotator _roll_2 (+ _pitch_2 9e+01) _yaw_2) "0.200000,0.200000,0.200000"))))

(fn ArrowParticleTrail
  (if (not (Variables|/Script/PlaygroundHeroes.JHero|GetbAttacking (Variables|Default|GetArcherReference)))
    (bind _returnvalue (AddComponent|AddParticleSystemComponent false))
    (Effects|Components|ParticleSystem|SetTemplate _returnvalue (Variables|Default|GetArrowTrailParticle))))

(fn MakeRealeaseNoise
  (bind _archerreference (Variables|Default|GetArcherReference))
  (bind _timeheld (Variables|/Script/PlaygroundHeroes.JArcher|GettimeHeld _archerreference))
  (bind _holdtimeneeded (Variables|/Script/PlaygroundHeroes.JArcher|GetHoldTimeNeeded _archerreference))
  (bind _returnvalue (/ _timeheld _holdtimeneeded))
  (if (>= _returnvalue 1.0)
    (Audio|PlaySoundatLocation (Variables|/Script/Engine.AudioComponent|GetSound (Variables|Default|GetstrongRelease)) (Transformation|GetActorLocation) "0, 0, 0" 0.7 1.0 0.0 0 0 0)
    (elif (>= _returnvalue 0.5)
      (Audio|PlaySoundatLocation (Variables|/Script/Engine.AudioComponent|GetSound (Variables|Default|GetstrongRelease)) (Transformation|GetActorLocation) "0, 0, 0" 0.5 0.7 0.0 0 0 0)
      (else
        (Audio|PlaySoundatLocation (Variables|/Script/Engine.AudioComponent|GetSound (Variables|Default|GetweakRelease)) (Transformation|GetActorLocation) "0, 0, 0" 0.5 0.8 0.0 0 0 0)))))