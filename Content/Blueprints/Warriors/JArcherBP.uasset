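; Player archer Blueprint, paired with a JKnightBP it finds on BeginPlay, layering UI, input and shared healing over CppTick.
; SetupUI creates the bars, arrow-draw and healing-supply widgets; inputs handle interact, pause, and a health/stamina reset.
; Holding heal sets CanHeal on both characters; Tick then heals while the Knight is in range, draining the widget-held HealingPool.
; The Knight heals only while the Archer is below max health; Invincible pins Archer health at maximum.
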(event Custom|PlayAnimation
  (Development|PrintString "Anim"))

(event EventBeginPlay
  (CallFunction|SetupUI)
  (bind _outactors (Actor|GetAllActorsOfClass "/Game/Blueprints/Warriors/JKnightBP.JKnightBP_C"))
  (Variables|Default|SetKnight (Utilities|Array|Get(acopy) _outactors))
  (bind _output_get (Variables|Default|SetStaggerMontage "/Game/CharacterAssets/NewArcher/Animation/archer_hit_front_montage.archer_hit_front_montage"))
  (bind _returnvalue (Animation|GetPlayLength _output_get))
  (Variables|Default|SetStaggerMontageDuration _returnvalue)
  (if (Variables|Combat|GetInvincible)
    (Variables|Default|SetMaxHealth 1e+05)))

(event Collision|EventActorBeginOverlap
  (params (OtherActor :type Actor%20Object%20Reference)))

(event EventTick
  (params (DeltaSeconds :type Float%20%28single-precision%29))
  (Class|JHero|CppTick DeltaSeconds)
  (if (Variables|Combat|GetInvincible)
    (Variables|Default|SetHealth (Variables|Default|GetMaxHealth)))
  (if (Variables|Healing|GetCanHeal)
    (CallFunction|ActuallyHealPlayer)))

(event Input|GamepadEvents|GamepadFaceButtonBottom
  (params (Key :type Key%20Structure))
  (:Pressed
    (Variables|Default|Setinteracting true))
  (:Released
    (Variables|Default|Setinteracting false)))

(event Input|GamepadEvents|GamepadSpecialLeft
  (params (Key :type Key%20Structure))
  (:Pressed
    (Variables|Default|SetbAttacking false)
    (Variables|Default|SetHealth (Variables|Default|GetMaxHealth))
    (Variables|Default|SetStamina (Variables|Default|GetMaxStamina))))

(event Input|GamepadEvents|GamepadSpecialRight
  (params (Key :type Key%20Structure))
  (:Pressed
    (Utilities|IsValid (Variables|Default|GetpauseMenuRef)
      (:Is%20Valid
        _)
      (:Is%20Not%20Valid
        (bind _returnvalue (UserInterface|CreateWidget "/Game/Blueprints/UI/JPauseMenu.JPauseMenu_C"))
        (Variables|Default|SetpauseMenuRef _returnvalue)))
    (Input|SetInputModeUIOnly (Game|GetPlayerController 0) (Variables|Default|GetpauseMenuRef) "DoNotLock")
    (UserInterface|Viewport|AddtoViewport (Variables|Default|GetpauseMenuRef) 0)
    (Game|SetGamePaused true)))

(event Input|KeyboardEvents|A
  (params (Key :type Key%20Structure))
  (:Pressed
    (Variables|Default|Setinteracting true))
  (:Released
    (Variables|Default|Setinteracting false)))

(event Input|GamepadEvents|GamepadFaceButtonLeft
  (params (Key :type Key%20Structure))
  (:Pressed
    (CallFunction|DetermineifCanHeal true))
  (:Released
    (CallFunction|DetermineifCanHeal false)))

(fn ConstructionScript)

(fn SetupUI
  (bind _self self)
  (bind _returnvalue (UserInterface|CreateWidget "/Game/Blueprints/UI/ArcherBars.ArcherBars_C"))
  (Variables|/Game/Blueprints/UI/ArcherBars.ArcherBars_C|SetArcher _returnvalue self)
  (UserInterface|Viewport|AddtoViewport _returnvalue 0)
  (Variables|Default|SetdeathMovementModifier 0.05)
  (bind _returnvalue_2 (UserInterface|CreateWidget "/Game/Blueprints/UI/arrowDrawProgress.arrowDrawProgress_C" 0 self))
  (UserInterface|Viewport|AddtoViewport _returnvalue_2 0)
  (Widget|SetRenderOpacity _returnvalue_2 0.0)
  (bind _returnvalue_3 (UserInterface|CreateWidget "/Game/Blueprints/UI/HealingBar.HealingBar_C" (Game|GetPlayerController 0) _self (* (Variables|Default|GetMaxHealth _self) 2.0)))
  (bind _output_get (Variables|Default|SetHealingSupplyWidget _returnvalue_3))
  (UserInterface|Viewport|AddtoViewport _output_get 0))

(fn DetermineifCanHeal
  (params (Pressed :type Boolean))
  (if Pressed
    (Variables|Healing|SetHoldingDownHeal true)
    (CallFunction|IsWithinHealingRange)
    (bind _output_get (Variables|Healing|SetCanHeal true))
    (Variables|/Game/Blueprints/Warriors/JKnightBP.JKnightBP_C|SetCanHeal (Variables|Default|GetKnight) _output_get)
    (else
      (Variables|Healing|SetHoldingDownHeal false)
      (bind _output_get_2 (Variables|Healing|SetCanHeal false))
      (Variables|/Game/Blueprints/Warriors/JKnightBP.JKnightBP_C|SetCanHeal (Variables|Default|GetKnight) _output_get_2))))

(fn ActuallyHealPlayer
  (bind _healrate (Variables|Healing|GetHealRate))
  (bind _healingsupplywidget (Variables|Default|GetHealingSupplyWidget))
  (bind _knight (Variables|Default|GetKnight))
  (bind _healingsupplywidget_2 (Variables|Default|GetHealingSupplyWidget))
  (bind _healrate_2 (Variables|Healing|GetHealRate))
  (bind _withinrange (CallFunction|IsWithinHealingRange))
  (if (and _withinrange (Variables|Healing|GetCanHeal))
    ;[1 1 1] Heal Yourself
    (if (< (Variables|Default|GetHealth) (Variables|Default|GetMaxHealth))
      (Class|JHero|AddHealth _healrate_2 0.0)
      (Variables|/Game/Blueprints/UI/HealingBar.HealingBar_C|SetHealingPool _healingsupplywidget (- (Variables|/Game/Blueprints/UI/HealingBar.HealingBar_C|GetHealingPool _healingsupplywidget) _healrate_2))
      ;[1 1 1] Heal Other Player
      (if (< (Variables|/Script/PlaygroundHeroes.JHero|GetHealth _knight) (Variables|/Script/PlaygroundHeroes.JHero|GetMaxHealth _knight))
        (Class|JHero|AddHealth _knight _healrate 0.0)
        (Variables|/Game/Blueprints/UI/HealingBar.HealingBar_C|SetHealingPool _healingsupplywidget_2 (- (Variables|/Game/Blueprints/UI/HealingBar.HealingBar_C|GetHealingPool _healingsupplywidget_2) _healrate))))))

(fn IsWithinHealingRange
  (if (<= (Transformation|GetDistanceTo (Variables|Default|GetKnight) self) (Variables|Healing|GetDistanceForHealing))
    (return true)
    (else
      (return false))))