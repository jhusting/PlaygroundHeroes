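; JKnightBP is the Blueprint for a knight warrior, handling player HUD setup, sword damage and interact input.
; On BeginPlay it adds Player 1 health and stamina bar widgets to the viewport.
; Sword collider overlaps with a JEnemy, while CanDamage is set, subtract SwordDamage unless the enemy's CheckHit returns true for the current hit type.
; The gamepad bottom face button or A key holds the Interacting flag.
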(event OnComponentBeginOverlap(SwordBodyCollider)
  (params (OverlappedComponent :type Primitive%20Component%20Object%20Reference) (OtherActor :type Actor%20Object%20Reference) (OtherComp :type Primitive%20Component%20Object%20Reference) (OtherBodyIndex :type Integer) (bFromSweep :type Boolean) (SweepResult :type Hit%20Result%20Structure%20%28by%20ref%29))
  (bind _asjenemy (Utilities|Casting|CastToJEnemy OtherActor))
  (if (Variables|Default|GetbCanDamage)
    (bind _returnvalue (Class|JEnemy|CheckHit _asjenemy (Variables|Default|GetCurrentHitType)))
    (if (not _returnvalue)
      (Class|JEnemy|AddHealth _asjenemy (* (Variables|Default|GetSwordDamage) -1.0) (Variables|Default|GetCurrentHitType)))))

(event EventBeginPlay
  (bind _returnvalue (UserInterface|CreateWidget "/Game/Blueprints/UI/Player1HealthBar.Player1HealthBar_C"))
  (UserInterface|Viewport|AddtoViewport _returnvalue 0)
  (bind _returnvalue_2 (UserInterface|CreateWidget "/Game/Blueprints/UI/Player1StaminaBar.Player1StaminaBar_C"))
  (UserInterface|Viewport|AddtoViewport _returnvalue_2 0))

(event Collision|EventActorBeginOverlap
  (params (OtherActor :type Actor%20Object%20Reference)))

(event EventTick
  (params (DeltaSeconds :type Float%20%28single-precision%29)))

(event Input|GamepadEvents|GamepadFaceButtonBottom
  (params (Key :type Key%20Structure))
  (:Pressed
    (Variables|Default|Setinteracting true))
  (:Released
    (Variables|Default|Setinteracting false)))

(event Input|KeyboardEvents|A
  (params (Key :type Key%20Structure))
  (:Pressed
    (Variables|Default|Setinteracting true))
  (:Released
    (Variables|Default|Setinteracting false)))

(fn ConstructionScript)