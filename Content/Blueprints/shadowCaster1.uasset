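; shadowCaster1 is a short-lived actor whose Cylinder mesh grows over time until the actor destroys itself about 1.5 seconds after it starts ticking.
; The construction script caches the cylinder's world scale and applies a SpawnRotation to the actor.
; Tick accumulates elapsed time and sets the scale to the cached base times time squared and GrowthRate, so growth accelerates from near zero.
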(event EventBeginPlay)

(event Collision|EventActorBeginOverlap
  (params (OtherActor :type Actor%20Object%20Reference)))

(event EventTick
  (params (DeltaSeconds :type Float%20%28single-precision%29))
  ;[1 1 1] x^2
  (bind _output_get (Variables|Default|SettimeTrack (+ DeltaSeconds (Variables|Default|GettimeTrack))))
  (if (>= (Variables|Default|GettimeTrack) 1.5)
    (Actor|DestroyActor)
    (else
      (Transformation|SetWorldScale3D (Variables|Default|GetCylinder) (* (Variables|Default|GetBaseScale) (* (* (Math|Float|Power _output_get 2.0) 1.0) (Variables|Default|GetGrowthRate)))))))

(fn ConstructionScript
  (Variables|Default|SetBaseScale (Transformation|GetWorldScale (Variables|Default|GetCylinder)))
  (Transformation|SetActorRotation (Variables|Default|GetspawnRotation) true))