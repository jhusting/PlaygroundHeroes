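; Spline camera actor that takes over player 0's view at BeginPlay and moves its camera along a spline.
; A Development function sets the view target to this actor, then a timeline starts.
; Each update scales the timeline's AnimationAlpha by spline length and sets the camera's world transform from that distance.
; Despite the asset name, the camera takes the spline's rotation as well as its location.
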(event EventBeginPlay
  (bind _spline (Variables|Default|GetSpline))
  (CallFunction|Development)
  (bind _animationalpha (Timeline|Timeline_0 Play)
    (:Update
      (Transformation|SetWorldTransform (Variables|Default|GetCamera) (Math|Transform|MakeTransform (Spline|GetLocationatDistanceAlongSpline _spline (* _animationalpha (Spline|GetSplineLength _spline)) "World") (Spline|GetRotationatDistanceAlongSpline _spline (* _animationalpha (Spline|GetSplineLength _spline)) "World")) false false))))

(event Collision|EventActorBeginOverlap
  (params (OtherActor :type Actor%20Object%20Reference)))

(event EventTick
  (params (DeltaSeconds :type Float%20%28single-precision%29)))

(fn ConstructionScript)

(fn Development
  (Game|Player|SetViewTargetwithBlend (Game|GetPlayerController 0) self 0.0 "VTBlend_Linear" 0.0 false))