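; Spline camera actor that takes over the first player's view and flies a camera along a path when play begins.
; On BeginPlay, Development sets the actor as view target, then a timeline plays an alpha scaled by the MovementSpline length.
; Each update moves the Camera to the spline's world location and rotation at that distance.
; A RotationSpline length calculation exists but is unused, so rotation also follows MovementSpline.
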(event EventBeginPlay
  (bind _movementspline (Variables|Default|GetMovementSpline))
  (CallFunction|Development)
  (bind _animationalpha (Timeline|Timeline_0 Play)
    (:Update
      (Transformation|SetWorldTransform (Variables|Default|GetCamera) (Math|Transform|MakeTransform (Spline|GetLocationatDistanceAlongSpline _movementspline (* _animationalpha (Spline|GetSplineLength _movementspline)) "World") (Spline|GetRotationatDistanceAlongSpline _movementspline (* _animationalpha (Spline|GetSplineLength _movementspline)) "World")) false false))))

(event Collision|EventActorBeginOverlap
  (params (OtherActor :type Actor%20Object%20Reference)))

(event EventTick
  (params (DeltaSeconds :type Float%20%28single-precision%29)))

(fn ConstructionScript)

(fn Development
  (Game|Player|SetViewTargetwithBlend (Game|GetPlayerController 0) self 0.0 "VTBlend_Linear" 0.0 false))