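; Actor Blueprint that shows the main menu once the intro level sequence finishes.
; On BeginPlay it takes the first LevelSequenceActor found in the level and binds ShowMainMenu to its player's finished event.
; CreateMainMenu then creates the JMainMenu widget, switches input to UI-only, adds it to the viewport, plays its FadeIn animation and unpauses the game.
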(event Custom|ShowMainMenu
  (CallFunction|CreateMainMenu))

(event EventBeginPlay
  (bind _outactors (Actor|GetAllActorsOfClass "/Script/LevelSequence.LevelSequenceActor"))
  (EventDispatchers|BindEventtoOnFinished (Variables|/Script/LevelSequence.LevelSequenceActor|GetSequencePlayer (Utilities|Array|Get(acopy) _outactors)) (delegate Custom|ShowMainMenu)))

(event Collision|EventActorBeginOverlap
  (params (OtherActor :type Actor%20Object%20Reference)))

(event EventTick
  (params (DeltaSeconds :type Float%20%28single-precision%29)))

(fn ConstructionScript)

(fn CreateMainMenu
  (bind _returnvalue (UserInterface|CreateWidget "/Game/Blueprints/UI/JMainMenu.JMainMenu_C" (Game|GetPlayerController 0)))
  (Input|SetInputModeUIOnly (Game|GetPlayerController 0) _returnvalue "DoNotLock")
  (UserInterface|Viewport|AddtoViewport _returnvalue 0)
  (UserInterface|Animation|PlayAnimation _returnvalue (Variables|/Game/Blueprints/UI/JMainMenu.JMainMenu_C|GetFadeIn _returnvalue) 0.0 1 "Forward" 1.0)
  (Game|SetGamePaused false))