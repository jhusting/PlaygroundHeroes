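; Cutscene level actor that opens a target level when the cutscene's maximum length runs out or a player skips it.
; BeginPlay caches all JHero actors, falls back to the current level name if LevelToGoTo is empty, then waits MaxCutsceneLength before loading.
; Tick polls the first two heroes' Interacting flags and jumps straight to the same level load when either is set.
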(event EventBeginPlay
  (bind _outactors (Actor|GetAllActorsOfClass "/Script/PlaygroundHeroes.JHero"))
  (Variables|Default|SetPlayers _outactors)
  (CallFunction|CheckEmptyGotoLevel)
  (Utilities|FlowControl|Delay (Variables|Default|GetMaxCutsceneLength))
  (Game|OpenLevel(byName) (Utilities|String|StringToName (Variables|Default|GetLevelToGoTo))))

(event Collision|EventActorBeginOverlap
  (params (OtherActor :type Actor%20Object%20Reference)))

(event EventTick
  (params (DeltaSeconds :type Float%20%28single-precision%29))
  (bind _players (Variables|Default|GetPlayers))
  (if (or (Variables|/Script/PlaygroundHeroes.JHero|Getinteracting (Utilities|Array|Get(acopy) _players)) (Variables|/Script/PlaygroundHeroes.JHero|Getinteracting (Utilities|Array|Get(acopy) _players 1)))
    (Game|OpenLevel(byName) (Utilities|String|StringToName (Variables|Default|GetLevelToGoTo)))))

(fn ConstructionScript)

(fn CheckEmptyGotoLevel
  (if (Utilities|Enum|Equal(Enum) (Variables|Default|GetLevelToGoTo) "")
    (bind _returnvalue (Game|GetCurrentLevelName true))
    (Variables|Default|SetLevelToGoTo _returnvalue)))