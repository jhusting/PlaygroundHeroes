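; Dialogue handler actor that shows timed lines of dialogue on screen, with center text and split text for two players.
; BeginPlay submits the Lines, Durations and Fonts sequence, then creates one JDialogueTextDisplay widget for player 0 and stores its reference.
; Tick calls UpdateDialogue, then pushes the current texts, fonts, render flag and split mode into that widget.
; The sequencing logic lives outside these graphs.
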(event EventBeginPlay
  (Class|DialogueHandler|SendNewdialogueSequence (Variables|Default|GetLines) (Variables|Default|GetDurations) (Variables|Default|GetFonts))
  (Utilities|FlowControl|DoOnce false
    (:Completed
      ;[1 1 1] Create Widget, Add to Viewport, store reference for destruction
      (bind _returnvalue (UserInterface|CreateWidget "/Game/Blueprints/UI/JDialogueTextDisplay.JDialogueTextDisplay_C" (Game|GetPlayerController 0) (Variables|Default|GetrenderWidget) (Variables|Default|GetsplitMode) (Utilities|Array|MakeArray (Variables|Default|GetcenterText) (Variables|Default|Getplayer1Text) (Variables|Default|Getplayer2Text)) (Utilities|Array|MakeArray (Variables|Default|GetcenterFont) (Variables|Default|Getplayer1Font) (Variables|Default|Getplayer2Font))))
      (UserInterface|Viewport|AddtoViewport _returnvalue 0)
      (Variables|Default|SetWidgetReference _returnvalue))))

(event Collision|EventActorBeginOverlap
  (params (OtherActor :type Actor%20Object%20Reference)))

(event EventTick
  (params (DeltaSeconds :type Float%20%28single-precision%29))
  ;[1 1 1] Update Widget Text
  (Class|DialogueHandler|UpdateDialogue DeltaSeconds)
  (Variables|/Game/Blueprints/UI/JDialogueTextDisplay.JDialogueTextDisplay_C|SetsentText (stale EventBeginPlay _returnvalue) (Utilities|Array|MakeArray (Variables|Default|GetcenterText) (Variables|Default|Getplayer1Text) (Variables|Default|Getplayer2Text)))
  (Variables|/Game/Blueprints/UI/JDialogueTextDisplay.JDialogueTextDisplay_C|SetdeclaredFonts (stale EventBeginPlay _returnvalue) (Utilities|Array|MakeArray (Variables|Default|GetcenterFont) (Variables|Default|Getplayer1Font) (Variables|Default|Getplayer2Font)))
  (Variables|/Game/Blueprints/UI/JDialogueTextDisplay.JDialogueTextDisplay_C|SetshouldRender (stale EventBeginPlay _returnvalue) (Variables|Default|GetrenderWidget))
  (Variables|/Game/Blueprints/UI/JDialogueTextDisplay.JDialogueTextDisplay_C|Set2Boxes (stale EventBeginPlay _returnvalue) (Variables|Default|GetsplitMode)))

(fn ConstructionScript)