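; Enemy actor with a single health bar widget that regenerates health and destroys itself at zero health.
; BeginPlay hides the scrumboard whiteboard mesh unless PhysicalIndicator is set and passes itself to the EnemyHealthBar widget.
; Tick updates hit times and health percent, adds capped regen per frame without DeltaSeconds scaling, then refreshes OldHealthPercent after a five-second Delay, with no visible effect on this bar.
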(event EventBeginPlay
  ;[1 1 1] Determine whether to show sphere mesh or not
  (if (Variables|Default|GetPhysicalIndicator)
    _
    (else
      (Rendering|SetVisibility (Variables|Default|GetScrumboardNotes1_WhiteBoard) false false)))
  (bind _asenemy_health_bar (Utilities|Casting|CastToEnemyHealthBar (UserInterface|GetUserWidgetObject (Variables|Default|GetHealthBarWidget))))
  (Variables|/Game/Blueprints/UI/EnemyHealthBar.EnemyHealthBar_C|SetEnemyBP _asenemy_health_bar self))

(event Collision|EventActorBeginOverlap
  (params (OtherActor :type Actor%20Object%20Reference)))

(event EventTick
  (params (DeltaSeconds :type Float%20%28single-precision%29))
  (bind _self self)
  (bind _maxhealth (Variables|/Script/PlaygroundHeroes.JEnemy|GetmaxHealth _self))
  (Class|JEnemy|UpdateHitTimes DeltaSeconds)
  ;[1 1 1] Update Health Percentage (thus updatingHealth Bar)
  (bind _output_get (Variables|/Script/PlaygroundHeroes.JEnemy|SetHealthPercent _self (/ (Variables|/Script/PlaygroundHeroes.JEnemy|GetHealth _self) (Variables|/Script/PlaygroundHeroes.JEnemy|GetmaxHealth _self))))
  ;[1 1 1] If 0.0%, destroy parent
  (if (== _output_get 0.0)
    (Actor|DestroyActor)
    (else
      ;[1 1 1] Regen Health every tick
      (Variables|/Script/PlaygroundHeroes.JEnemy|SetHealth _self (+ (Variables|/Script/PlaygroundHeroes.JEnemy|GetHealth _self) (/ (Variables|Default|GetHealthRegenSpeed) 1e+02)))
      ;[1 1 1] If Health>Max Health: Health = Max Health
      (if (> (Variables|/Script/PlaygroundHeroes.JEnemy|GetHealth _self) _maxhealth)
        (Variables|/Script/PlaygroundHeroes.JEnemy|SetHealth _self _maxhealth))
      (Utilities|FlowControl|Delay 5.0)
      ;[1 1 1] Update Health Old Health Percentage (thus updating the lower Health Bar)<DOES NOTHING VISUALLY FOR SINGLE  HEALTHBAR BUT STILL UPDATES VALUE IN CODE>
      (Variables|Default|SetOldHealthPercent (/ (Variables|/Script/PlaygroundHeroes.JEnemy|GetHealth _self) (Variables|/Script/PlaygroundHeroes.JEnemy|GetmaxHealth _self))))))

(fn ConstructionScript)