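; StickyNotes is a short-lived hazard actor in ImpendingDeadline that applies its Damage value to JHero actors through AddHealth.
; It destroys itself after Lifetime, or when its Sphere hits a StaticMeshActor.
; A Box begin-overlap applies the health change only to heroes not already in Targets.
; A ReAttackDelay latent delay then removes the hero from that list, allowing a later overlap to hit again.
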(event OnComponentBeginOverlap(Box)
  (params (OverlappedComponent :type Primitive%20Component%20Object%20Reference) (OtherActor :type Actor%20Object%20Reference) (OtherComp :type Primitive%20Component%20Object%20Reference) (OtherBodyIndex :type Integer) (bFromSweep :type Boolean) (SweepResult :type Hit%20Result%20Structure%20%28by%20ref%29))
  (bind _targets (Variables|Default|Gettargets))
  (bind _asjhero (Utilities|Casting|CastToJHero OtherActor))
  (bind _returnvalue (Utilities|Array|AddUnique _targets _asjhero))
  (if (!= _returnvalue -1)
    (Class|JHero|AddHealth _asjhero (Variables|Default|Getdamage))
    (Utilities|FlowControl|Delay (Variables|Default|GetreAttackDelay))
    (Utilities|Array|RemoveItem _targets _asjhero)))

(event OnComponentHit(Sphere)
  (params (HitComponent :type Primitive%20Component%20Object%20Reference) (OtherActor :type Actor%20Object%20Reference) (OtherComp :type Primitive%20Component%20Object%20Reference) (NormalImpulse :type Vector :default "0, 0, 0") (Hit :type Hit%20Result%20Structure%20%28by%20ref%29))
  (Utilities|Casting|CastToStaticMeshActor OtherActor)
  (Actor|DestroyActor))

(event EventBeginPlay
  (Utilities|FlowControl|Delay (Variables|Default|GetLifetime))
  (Actor|DestroyActor))

(event Collision|EventActorBeginOverlap
  (params (OtherActor :type Actor%20Object%20Reference)))

(event EventTick
  (params (DeltaSeconds :type Float%20%28single-precision%29)))

(fn ConstructionScript)