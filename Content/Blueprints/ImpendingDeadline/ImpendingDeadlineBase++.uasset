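; Base boss actor for Impending Deadline, which fires Sap projectiles and is killed through three weakpoints.
; BeginPlay spawns three health-bar actors that store weakpoint health, and ArrowBP overlaps on each box collider subtract arrow damage.
; Tick uses Delays to alternate two attacks, paired side shots and randomly offset bursts, with randomized direction and speed.
; After phase changes it checks health, and with all three depleted it relocates randomly, then destroys itself.
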(event OnComponentBeginOverlap(WeakPoint0BoxCollider)
  (params (OverlappedComponent :type Primitive%20Component%20Object%20Reference) (OtherActor :type Actor%20Object%20Reference) (OtherComp :type Primitive%20Component%20Object%20Reference) (OtherBodyIndex :type Integer) (bFromSweep :type Boolean) (SweepResult :type Hit%20Result%20Structure%20%28by%20ref%29))
  ;[1 1 1] Settle hit detection for each weakpoint. (You give it the thing that is the parent of the collider as Deleted on 0HP)(or yourself if no parent)
  (bind _asarrow_bp (Utilities|Casting|CastToArrowBP OtherActor))
  (CallFunction|AttackonWeakpoint 0 _asarrow_bp))

(event OnComponentBeginOverlap(WeakPoint1BoxCollider)
  (params (OverlappedComponent :type Primitive%20Component%20Object%20Reference) (OtherActor :type Actor%20Object%20Reference) (OtherComp :type Primitive%20Component%20Object%20Reference) (OtherBodyIndex :type Integer) (bFromSweep :type Boolean) (SweepResult :type Hit%20Result%20Structure%20%28by%20ref%29))
  ;[1 1 1] Settle hit detection for each weakpoint. (You give it the thing that is the parent of the collider as Deleted on 0HP)(or yourself if no parent)
  (bind _asarrow_bp (Utilities|Casting|CastToArrowBP OtherActor))
  (CallFunction|AttackonWeakpoint 1 _asarrow_bp))

(event OnComponentBeginOverlap(WeakPoint2BoxCollider)
  (params (OverlappedComponent :type Primitive%20Component%20Object%20Reference) (OtherActor :type Actor%20Object%20Reference) (OtherComp :type Primitive%20Component%20Object%20Reference) (OtherBodyIndex :type Integer) (bFromSweep :type Boolean) (SweepResult :type Hit%20Result%20Structure%20%28by%20ref%29))
  ;[1 1 1] Settle hit detection for each weakpoint. (You give it the thing that is the parent of the collider as Deleted on 0HP)(or yourself if no parent)
  (bind _asarrow_bp (Utilities|Casting|CastToArrowBP OtherActor))
  (CallFunction|AttackonWeakpoint 2 _asarrow_bp))

(event EventBeginPlay
  (CallFunction|Spawn3JEnemyWeakpoints))

(event Collision|EventActorBeginOverlap
  (params (OtherActor :type Actor%20Object%20Reference)))

(event EventTick
  (params (DeltaSeconds :type Float%20%28single-precision%29))
  (bind _returnvalue (Math|Random|RandomUnitVector))
  (bind _projectilespawnoffset (Variables|Default|GetProjectileSpawnOffset))
  (bind _weakpoints (Variables|Default|GetWeakpoints))
  (bind _returnvalue_2 (* _projectilespawnoffset _returnvalue))
  (Utilities|FlowControl|Delay (Variables|Default|GetfireRate))
  (switch int (Variables|Default|GetBossPhase) ; Control boss phases
    (:0
      ;[1 1 1] Attack Pattern 1: Fire from both sides
      (Utilities|FlowControl|Delay (Variables|Default|GetfireRate))
      (CallFunction|ShootProjectiles (+ _projectilespawnoffset "50.000000,300.000000,100.000000"))
      (CallFunction|ShootProjectiles (- _projectilespawnoffset "50.000000,300.000000,100.000000"))
      ;[1 1 1] Increment through boss phases and loop around
      (Utilities|FlowControl|Delay 3.0 :!label _label)
      (Variables|Default|SetBossPhase (Math|Integer|%(Integer) (+ (Variables|Default|GetBossPhase) 1) 2))
      ;[1 1 1] If your weak points are out of health, delete self (This will delete everything attached to this Actor)
      (if (Math|Boolean|ANDBoolean (<= (Variables|/Script/PlaygroundHeroes.JEnemy|GetHealth (Utilities|Array|Get(acopy) _weakpoints)) 0.0) (<= (Variables|/Script/PlaygroundHeroes.JEnemy|GetHealth (Utilities|Array|Get(acopy) _weakpoints 1)) 0.0) (<= (Variables|/Script/PlaygroundHeroes.JEnemy|GetHealth (Utilities|Array|Get(acopy) _weakpoints 2)) 0.0))
        (Transformation|SetActorLocation (* (Math|Random|RandomUnitVector) (Transformation|GetActorLocation)) false false)
        (Utilities|FlowControl|Delay 5.0)
        (Actor|DestroyActor)))
    (:1
      ;[1 1 1] Attack Pattern 2: Burst fire from a single location
      (for _index (range 0 5)
        (Utilities|FlowControl|Delay (/ (Variables|Default|GetfireRate) 5.0))
        (CallFunction|ShootProjectiles _returnvalue_2)
        (CallFunction|ShootProjectiles _returnvalue_2)
        (goto _label)))))

(fn ConstructionScript)

(fn CreateFiringProperties
  (bind _projectileyforcerange (Variables|Default|GetProjectileYForceRange))
  (return (Math|Vector|MakeVector (Math|Random|RandomFloatinRange 0.0 (Variables|Default|GetProjectileXForceRange)) (Math|Random|RandomFloatinRange (* _projectileyforcerange -1.0) _projectileyforcerange) (Math|Random|RandomFloatinRange 5.0 15.0)) (Math|Random|RandomFloatinRange 2e+02 9e+02)))

(fn ShootProjectiles
  (params (Spawn%20Offset :type Vector))
  (bind (_directionvector _speed) (CallFunction|CreateFiringProperties))
  ;[1 1 1] Spawn at an offset location
  (Game|SpawnActorfromClass "/Game/Blueprints/TreeBoss/Sap.Sap_C" (Math|Transform|MakeTransform (+ Spawn%20Offset (Transformation|GetActorLocation)) (Transformation|GetActorRotation) (Transformation|GetActorScale3D)) "Undefined" 0 _directionvector _speed 0))

(fn AttackonWeakpoint
  (params (indexOfHealthsArray :type Integer) (OtherArctor :type Arrow%20BP%20Object%20Reference) (ObjectToBeDeletedOn0Hp :type Static%20Mesh%20Component%20Object%20Reference))
  (bind _weakpoints (Variables|Default|GetWeakpoints))
  (bind _output (Utilities|Array|Get(acopy) _weakpoints indexOfHealthsArray))
  (bind _health (Variables|/Script/PlaygroundHeroes.JEnemy|GetHealth _output))
  ;[1 1 1] Adjust health
  (Class|JEnemy|SetHealth _output (Math|Float|Clamp(Float) (- _health (Variables|/Game/Blueprints/Warriors/ArrowBP.ArrowBP_C|GetArrowDamage OtherArctor)) 0.0 (Variables|/Script/PlaygroundHeroes.JEnemy|GetmaxHealth (Utilities|Array|Get(acopy) _weakpoints indexOfHealthsArray))))
  ;[1 1 1] Destroy provided static actor, killing it and THIS (Use this to destroy visual meshes of weakpoints and collider too)
  (if (<= _health 0.0)
    (Rendering|SetVisibility ObjectToBeDeletedOn0Hp false false)))

(fn Spawn3JEnemyWeakpoints
  ;[1 1 1] JEnemy Health bar 0
  (bind _returnvalue (Game|SpawnActorfromClass "/Game/Blueprints/ImpendingDeadline/ImpendingDeadlineHBar0.ImpendingDeadlineHBar0_C" (Math|Transform|MakeTransform (+ (Utilities|Array|Get(acopy) (Variables|Default|GetWeakpointPositionOffsets)) (Transformation|GetActorLocation)) (Transformation|GetActorRotation) (Transformation|GetActorScale3D)) "Undefined" 0 true 0))
  (Variables|/Game/Blueprints/ImpendingDeadline/ImpendingDeadlineHBar0.ImpendingDeadlineHBar0_C|SetHealthRegenSpeed _returnvalue (Variables|Default|GetHealthRegen))
  (bind _output_get (Variables|/Script/PlaygroundHeroes.JEnemy|SetmaxHealth _returnvalue (Variables|Default|GetHealthPerWeakpoint)))
  (Class|JEnemy|SetHealth _returnvalue _output_get)
  (Utilities|Array|Add (Variables|Default|GetWeakpoints) _returnvalue)
  ;[1 1 1] Jenemy Health bar 1
  (bind _returnvalue_2 (Game|SpawnActorfromClass "/Game/Blueprints/ImpendingDeadline/ImpendingDeadlineHBar1.ImpendingDeadlineHBar1_C" (Math|Transform|MakeTransform (+ (Utilities|Array|Get(acopy) (Variables|Default|GetWeakpointPositionOffsets) 1) (Transformation|GetActorLocation)) (Transformation|GetActorRotation) (Transformation|GetActorScale3D)) "Undefined" 0 true 0))
  (Variables|/Game/Blueprints/ImpendingDeadline/ImpendingDeadlineHBar1.ImpendingDeadlineHBar1_C|SetHealthRegenSpeed _returnvalue_2 (Variables|Default|GetHealthRegen))
  (bind _output_get_2 (Variables|/Script/PlaygroundHeroes.JEnemy|SetmaxHealth _returnvalue_2 (Variables|Default|GetHealthPerWeakpoint)))
  (Class|JEnemy|SetHealth _returnvalue_2 _output_get_2)
  (Utilities|Array|Add (Variables|Default|GetWeakpoints) _returnvalue_2)
  ;[1 1 1] Jenemy Health bar 2
  (bind _returnvalue_3 (Game|SpawnActorfromClass "/Game/Blueprints/ImpendingDeadline/ImpendingDeadlineHBar2.ImpendingDeadlineHBar2_C" (Math|Transform|MakeTransform (+ (Utilities|Array|Get(acopy) (Variables|Default|GetWeakpointPositionOffsets) 2) (Transformation|GetActorLocation)) (Transformation|GetActorRotation) (Transformation|GetActorScale3D)) "Undefined" 0 true 0))
  (Variables|/Game/Blueprints/ImpendingDeadline/ImpendingDeadlineHBar2.ImpendingDeadlineHBar2_C|SetHealthRegenSpeed _returnvalue_3 (Variables|Default|GetHealthRegen))
  (bind _output_get_3 (Variables|/Script/PlaygroundHeroes.JEnemy|SetmaxHealth _returnvalue_3 (Variables|Default|GetHealthPerWeakpoint)))
  (Class|JEnemy|SetHealth _returnvalue_3 _output_get_3)
  (Utilities|Array|Add (Variables|Default|GetWeakpoints) _returnvalue_3))