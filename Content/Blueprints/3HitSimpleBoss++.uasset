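; Boss actor with three arrow-damaged weak points that fires randomized Sap projectiles and spawns falling leaves at BeginPlay.
; Each collider overlap with an ArrowBP feeds AttackOnWeakpoint, which lowers that point's health and hides, without destroying, its component at zero.
; Tick uses Delays to run two-sided fire or random-offset bursts by AttackMode.
; Only the two-sided branch advances the mode or destroys the boss once all points reach zero.
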(event OnComponentBeginOverlap(WeakPoint0BoxCollider)
  (params (OverlappedComponent :type Primitive%20Component%20Object%20Reference) (OtherActor :type Actor%20Object%20Reference) (OtherComp :type Primitive%20Component%20Object%20Reference) (OtherBodyIndex :type Integer) (bFromSweep :type Boolean) (SweepResult :type Hit%20Result%20Structure%20%28by%20ref%29))
  ;[1 1 1] Settle hit detection for each weakpoint. (You give it the thing that is the parent of the collider as Deleted on 0HP)(or yourself if no parent)
  (bind _asarrow_bp (Utilities|Casting|CastToArrowBP OtherActor))
  (CallFunction|AttackonWeakpoint 0 _asarrow_bp (Variables|Default|GetWeakPoint0)))

(event OnComponentBeginOverlap(WeakPoint1BoxCollider)
  (params (OverlappedComponent :type Primitive%20Component%20Object%20Reference) (OtherActor :type Actor%20Object%20Reference) (OtherComp :type Primitive%20Component%20Object%20Reference) (OtherBodyIndex :type Integer) (bFromSweep :type Boolean) (SweepResult :type Hit%20Result%20Structure%20%28by%20ref%29))
  ;[1 1 1] Settle hit detection for each weakpoint. (You give it the thing that is the parent of the collider as Deleted on 0HP)(or yourself if no parent)
  (bind _asarrow_bp (Utilities|Casting|CastToArrowBP OtherActor))
  (CallFunction|AttackonWeakpoint 1 _asarrow_bp (Variables|Default|GetWeakPoint1)))

(event OnComponentBeginOverlap(WeakPoint2BoxCollider)
  (params (OverlappedComponent :type Primitive%20Component%20Object%20Reference) (OtherActor :type Actor%20Object%20Reference) (OtherComp :type Primitive%20Component%20Object%20Reference) (OtherBodyIndex :type Integer) (bFromSweep :type Boolean) (SweepResult :type Hit%20Result%20Structure%20%28by%20ref%29))
  ;[1 1 1] Settle hit detection for each weakpoint. (You give it the thing that is the parent of the collider as Deleted on 0HP)(or yourself if no parent)
  (bind _asarrow_bp (Utilities|Casting|CastToArrowBP OtherActor))
  (CallFunction|AttackonWeakpoint 2 _asarrow_bp (Variables|Default|GetWeakPoint2)))

(event EventBeginPlay
  ;[1 1 1] Initialize the three hit points (flexbile for more too)
  (for _index (range 0 2)
    (Utilities|Array|Add (Variables|Default|GetWeakPointHealths) 1e+02)
    (Utilities|Array|Add (Variables|Default|GetWeakPointMaxHealths) 1e+02))
  (Game|SpawnActorfromClass "/Game/Blueprints/SpawnFallingLeaves.SpawnFallingLeaves_C" (Math|Transform|MakeTransform (+ (Variables|Default|GetSpawnOffset) "0, 0,100.000000")) "Undefined" 0 0))

(event Collision|EventActorBeginOverlap
  (params (OtherActor :type Actor%20Object%20Reference)))

(event EventTick
  (params (DeltaSeconds :type Float%20%28single-precision%29))
  (bind _returnvalue (Math|Random|RandomUnitVector))
  (bind _spawnoffset (Variables|Default|GetSpawnOffset))
  (bind _returnvalue_2 (* _spawnoffset _returnvalue))
  (switch int (Variables|Default|GetAttackMode)
    (:0
      ;[1 1 1] Attack Pattern 1: Fire from both sides
      (Utilities|FlowControl|Delay (Variables|Default|GetfireRate))
      (CallFunction|ShootProjectiles (+ _spawnoffset "0.000000,300.000000,100.000000"))
      (CallFunction|ShootProjectiles (- _spawnoffset "0.000000,300.000000,100.000000"))
      ;[1 1 1] If your weak points are out of health, delete self (This will delete everything attached to this Actor)
      (if (Math|Boolean|ANDBoolean (<= (Utilities|Array|Get(acopy) (Variables|Default|GetWeakPointHealths)) 0.0) (<= (Utilities|Array|Get(acopy) (Variables|Default|GetWeakPointHealths) 1) 0.0) (<= (Utilities|Array|Get(acopy) (Variables|Default|GetWeakPointHealths) 2) 0.0))
        (Actor|DestroyActor)
        (else
          (Utilities|FlowControl|Delay 2.0)
          (Variables|Default|SetAttackMode (Math|Integer|%(Integer) (+ (Variables|Default|GetAttackMode) 1) 2)))))
    (:1
      ;[1 1 1] Attack Pattern 2: Burst fire from a single location
      (for _index (range 0 5)
        (Utilities|FlowControl|Delay (/ (Variables|Default|GetfireRate) 5.0))
        (CallFunction|ShootProjectiles _returnvalue_2)
        (CallFunction|ShootProjectiles _returnvalue_2)))))

(fn ConstructionScript)

(fn CreateFiringProperties
  (bind _projectileangleyrange (Variables|Default|GetProjectileAngleYRange))
  (return (Math|Vector|MakeVector (Math|Random|RandomFloatinRange 0.0 (Variables|Default|GetProjectileAngleXMax)) (Math|Random|RandomFloatinRange (* _projectileangleyrange -1.0) _projectileangleyrange) 1e+01) (Math|Random|RandomFloatinRange 3.5e+02 8e+02)))

(fn ShootProjectiles
  (params (SpawnOffset :type Vector))
  (bind (_directionvector _speed) (CallFunction|CreateFiringProperties))
  ;[1 1 1] Spawn at an offset location
  (Game|SpawnActorfromClass "/Game/Blueprints/Sap.Sap_C" (Math|Transform|MakeTransform (+ SpawnOffset (Transformation|GetActorLocation)) (Transformation|GetActorRotation) (Transformation|GetActorScale3D)) "Undefined" 0 _directionvector _speed 0))

(fn AttackonWeakpoint
  (params (indexOfHealthsArray :type Integer) (OtherArctor :type Arrow%20BP%20Object%20Reference) (ObjectToBeDeletedOn0Hp :type Static%20Mesh%20Component%20Object%20Reference))
  (bind _weakpointhealths (Variables|Default|GetWeakPointHealths))
  ;[1 1 1] Adjust health
  (Utilities|Array|SetArrayElem _weakpointhealths indexOfHealthsArray (Math|Float|Clamp(Float) (- (Utilities|Array|Get(acopy) _weakpointhealths indexOfHealthsArray) (Variables|/Game/Blueprints/Warriors/ArrowBP.ArrowBP_C|GetArrowDamage OtherArctor)) 0.0 (Utilities|Array|Get(acopy) (Variables|Default|GetWeakPointMaxHealths) indexOfHealthsArray)))
  ;[1 1 1] Destroy provided static actor, killing it and THIS (Use this to destroy visual meshes of weakpoints and collider too)
  (if (<= (Utilities|Array|Get(acopy) (Variables|Default|GetWeakPointHealths) indexOfHealthsArray) 0.0)
    (Rendering|SetVisibility ObjectToBeDeletedOn0Hp false false)))