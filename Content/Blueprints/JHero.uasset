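; JHero is a player character with camera-relative movement, mouse look, jog, toggled crouch and prone, and a jump whose height depends on whether it is moving.
; Input events set state flags and walk speed, which gate one another: prone locks movement until a delay after rising, and crouch blocks jumping unless jogging.
; BeginPlay teleports it to the PlayerStart tagged with its player index and creates health and stamina widgets.
; Debug keys adjust health.
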(event EventBeginPlay
  (CallFunction|SpawnPlayer)
  (CallFunction|CreateUI))

(event Collision|EventActorBeginOverlap
  (params (OtherActor :type Actor%20Object%20Reference)))

(event EventTick
  (params (DeltaSeconds :type Float%20%28single-precision%29)))

(event Input|ActionEvents|InputActionJog
  (params (Key :type Key%20Structure))
  (bind _charactermovement (Variables|Character|GetCharacterMovement))
  ;[1 1 1] Jog (Modifier)
  (:Pressed
    (Variables|Default|SetJogPressed true)
    (Variables|/Script/Engine.CharacterMovementComponent|SetMaxWalkSpeed _charactermovement 375.0))
  (:Released
    (Variables|Default|SetJogPressed false)
    (if (Variables|Default|GetCrouchPressed)
      (Variables|/Script/Engine.CharacterMovementComponent|SetMaxWalkSpeed _charactermovement 1.6e+02)
      (else
        (Variables|/Script/Engine.CharacterMovementComponent|SetMaxWalkSpeed _charactermovement 2e+02)))))

(event Input|ActionEvents|InputActionCrouch
  (params (Key :type Key%20Structure))
  (bind _charactermovement (Variables|Character|GetCharacterMovement))
  ;[1 1 1] Crouch (Toggle)
  (:Pressed
    (if (not (Variables|Default|GetPronePressed))
      (Utilities|FlowControl|FlipFlop ; Press  once to toggle
        (:A
          (Variables|Default|SetCrouchPressed true)
          (Variables|/Script/Engine.CharacterMovementComponent|SetMaxWalkSpeed _charactermovement 1.6e+02))
        (:B
          (Variables|Default|SetCrouchPressed false)
          (if (Variables|Default|GetJogPressed)
            (Variables|/Script/Engine.CharacterMovementComponent|SetMaxWalkSpeed _charactermovement 375.0)
            (else
              (Variables|/Script/Engine.CharacterMovementComponent|SetMaxWalkSpeed _charactermovement 2e+02))))))))

(event Input|ActionEvents|InputActionProne
  (params (Key :type Key%20Structure))
  ;[1 1 1] Prone(Delays)
  (:Pressed
    (if (not (Variables|Default|GetCrouchPressed))
      (Utilities|FlowControl|FlipFlop
        (:A
          (Variables|Default|SetPronePressed true)
          (Variables|Default|SetDisableMovement true))
        (:B
          (Variables|Default|SetPronePressed false)
          (Utilities|FlowControl|Delay 1.4)
          (Variables|Default|SetDisableMovement false))))))

(event Input|ActionEvents|InputActionJump
  (params (Key :type Key%20Structure))
  (bind _charactermovement (Variables|Character|GetCharacterMovement))
  ;[1 1 1] Jump Height Based On Modifiers and Velocity
  (:Pressed
    (if (not (Variables|Default|GetDisableMovement))
      (if (Variables|Default|GetCrouchPressed)
        (if (> (Variables|/Script/Engine.CharacterMovementComponent|GetMaxWalkSpeed (Variables|Character|GetCharacterMovement)) 1.6e+02)
          (if (> (Math|Vector|VectorLength (Variables|/Script/Engine.MovementComponent|GetVelocity (Variables|Character|GetCharacterMovement))) 0.0) :!label _label
            (Character|Jump)
            (Variables|/Script/Engine.CharacterMovementComponent|SetJumpZVelocity _charactermovement 365.0)
            (Variables|Default|SetJumpPressed true)
            (else
              (Character|Jump)
              (Variables|/Script/Engine.CharacterMovementComponent|SetJumpZVelocity _charactermovement 3.4e+02)
              (Variables|Default|SetJumpPressed true))))
        (else
          (goto _label)))))
  (:Released
    (Variables|Default|SetJumpPressed false)))

(event Input|AxisEvents|InputAxisMoveForward
  (params (AxisValue :type Float%20%28single-precision%29))
  ;[1 1 1] Movement
  (if (not (Variables|Default|GetDisableMovement))
    (Pawn|Input|AddMovementInput (Math|Vector|GetForwardVector (Math|Rotator|MakeRotator 0.0 0.0 (.Yaw (Math|Rotator|BreakRotator (Pawn|GetControlRotation :!class /Script/Engine.Pawn))))) AxisValue false)))

(event Input|AxisEvents|InputAxisMoveRight
  (params (AxisValue :type Float%20%28single-precision%29))
  ;[1 1 1] Movement
  (if (not (Variables|Default|GetDisableMovement))
    (Pawn|Input|AddMovementInput (Math|Vector|GetRightVector (Math|Rotator|MakeRotator 0.0 0.0 (.Yaw (Math|Rotator|BreakRotator (Pawn|GetControlRotation :!class /Script/Engine.Pawn))))) AxisValue false)))

(event Input|AxisEvents|InputAxisLookUp
  (params (AxisValue :type Float%20%28single-precision%29))
  ;[1 1 1] Mouse Movement
  (Pawn|Input|AddControllerPitchInput AxisValue))

(event Input|AxisEvents|InputAxisTurn
  (params (AxisValue :type Float%20%28single-precision%29))
  ;[1 1 1] Mouse Movement
  (Pawn|Input|AddControllerYawInput AxisValue))

(event Input|KeyboardEvents|Subtract
  (params (Key :type Key%20Structure))
  ;[1 1 1] DEBUG: Adjust UI health manually
  (:Pressed
    (if (> (Variables|Default|GetCurrentHealth) 0.0)
      (bind _output_get (Variables|Default|SetCurrentHealth (- (Variables|Default|GetCurrentHealth) 5.0)))
      (Development|PrintString (Utilities|String|ToString(Float) _output_get)))))

(event Input|KeyboardEvents|Add
  (params (Key :type Key%20Structure))
  ;[1 1 1] DEBUG: Adjust UI health manually
  (:Pressed
    (if (< (Variables|Default|GetCurrentHealth) (Variables|Default|GetMaxHealth))
      (bind _output_get (Variables|Default|SetCurrentHealth (+ (Variables|Default|GetCurrentHealth) 5.0)))
      (Development|PrintString (Utilities|String|ToString(Float) _output_get)))))

(fn ConstructionScript)

(fn SpawnPlayer
  ;[1 1 1] Compare your playerInt to all Player Starts
  (bind _outactors (Actor|GetAllActorsOfClass "/Script/Engine.PlayerStart"))
  (for _array_element _outactors
    (if (Utilities|Name|Equal(Name) (Variables|/Script/Engine.PlayerStart|GetPlayerStartTag _array_element) (Utilities|String|StringToName (Utilities|String|Append "player" (Utilities|String|ToString(Integer) (Variables|Default|GetPlayerInt)))))
      ;[1 1 1] Move Spawn Location and your Transform to the Player Start tagged with your player index
      (bind _output_get (Variables|Default|SetSpawnLocation (Transformation|GetActorTransform _array_element)))
      (Transformation|SetActorTransform _output_get false true))))

(fn CreateUI
  (bind _returnvalue (UserInterface|CreateWidget "/Game/Blueprints/Player0HealthBar.Player0HealthBar_C"))
  (bind _output_get (Variables|Default|SetHealthBarReferrence _returnvalue))
  (UserInterface|Viewport|AddtoViewport _output_get 0)
  (bind _returnvalue_2 (UserInterface|CreateWidget "/Game/Blueprints/Player0StaminaBar.Player0StaminaBar_C"))
  (bind _output_get_2 (Variables|Default|SetStaminaBarReference _returnvalue_2))
  (UserInterface|Viewport|AddtoViewport _output_get_2 0))