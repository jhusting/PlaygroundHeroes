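; Base enemy Blueprint that gives each enemy a health bar widget for two local players.
; On BeginPlay it creates one widget each for player controllers 0 and 1, passing itself as EnemyBP, and adds it to that player's screen.
; Initial viewport position is the actor's world X/Y used directly, without screen projection.
; Tick, overlap and construction script are empty.
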(event EventBeginPlay
  (bind _self self)
  (bind _returnvalue (Transformation|GetActorLocation _self))
  (bind _returnvalue_2 (Math|Conversions|ToVector2D(Vector) _returnvalue))
  (bind _returnvalue_3 (UserInterface|CreateWidget "/Game/Blueprints/UI/EnemyHealthBar.EnemyHealthBar_C" (Game|GetPlayerController 0) _self))
  (Class|UserWidget|SetPositioninViewport _returnvalue_3 _returnvalue_2 true)
  (UserInterface|Viewport|AddtoPlayerScreen _returnvalue_3)
  (bind _returnvalue_4 (UserInterface|CreateWidget "/Game/Blueprints/UI/EnemyHealthBar.EnemyHealthBar_C" (Game|GetPlayerController 1) _self))
  (Class|UserWidget|SetPositioninViewport _returnvalue_4 _returnvalue_2 true)
  (UserInterface|Viewport|AddtoPlayerScreen _returnvalue_4))

(event Collision|EventActorBeginOverlap
  (params (OtherActor :type Actor%20Object%20Reference)))

(event EventTick
  (params (DeltaSeconds :type Float%20%28single-precision%29)))

(fn ConstructionScript)