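; SkeletonExplosion is an explosion actor that plays a rumble sound, expands, and kills the first JHero it overlaps while CanDamage is set.
; Tick grows the root's scale vector by GrowthRate per second, keeping its proportions.
; A hit starts GrowthTimeline, whose update and finish handlers are meant to drive GrowthRate and destroy the actor.
; A BeginPlay timer also destroys it after LifeTime.
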(event EventBeginPlay
  (Audio|Components|Audio|Play (Variables|Default|GetEXPLOSION_Medium_Bright_Impact_Rumble_Long_Tail_stereo) 0.0)
  (Utilities|Time|SetTimerbyFunctionName 0 "DestroySelf" (Variables|Default|GetLifeTime)))

(event Collision|EventActorBeginOverlap
  (params (OtherActor :type Actor%20Object%20Reference))
  (if (Variables|Default|GetcanDamage)
    (bind _asjhero (Utilities|Casting|CastToJHero OtherActor))
    (Audio|Components|Audio|Play (Variables|Default|GetGrowthTimeline))
    (Variables|/Script/PlaygroundHeroes.JHero|SetHealth _asjhero 0.0)
    (Class|JHero|Die _asjhero)
    (Variables|Default|SetcanDamage false)))

(event EventTick
  (params (DeltaSeconds :type Float%20%28single-precision%29))
  (Transformation|SetWorldScale3D (Variables|Default|GetDefaultSceneRoot) (* (Math|Vector|Normalize (Transformation|GetWorldScale (Variables|Default|GetDefaultSceneRoot))) (+ (Math|Float|Sqrt (Math|Vector|VectorLengthSquared (Transformation|GetWorldScale (Variables|Default|GetDefaultSceneRoot)))) (* (Variables|Default|GetGrowthRate) DeltaSeconds)))))

(fn ConstructionScript)

(fn DestroySelf
  (Actor|DestroyActor))