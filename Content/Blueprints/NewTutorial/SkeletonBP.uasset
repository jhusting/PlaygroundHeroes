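; Skeleton melee enemy that hunts JHero players, with its AI run directly on Tick.
; When no montage plays, it picks a standing hero by distance and facing angle, turns instantly and holds near 80% of attack range.
; In range, it plays one of two random attack montages, with a timer re-arming attacks.
; Axe overlaps damage each hero once until the hit list clears; Explode spawns an explosion and kills the skeleton.
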(event OnComponentBeginOverlap(AxeCollider)
  (params (OverlappedComponent :type Primitive%20Component%20Object%20Reference) (OtherActor :type Actor%20Object%20Reference) (OtherComp :type Primitive%20Component%20Object%20Reference) (OtherBodyIndex :type Integer) (bFromSweep :type Boolean) (SweepResult :type Hit%20Result%20Structure%20%28by%20ref%29))
  (bind _heroeshit (Variables|Default|GetHeroesHit))
  (if (Variables|Default|GetCanDamage)
    (bind _asjhero (Utilities|Casting|CastToJHero OtherActor))
    (if (== -1 (Utilities|Array|FindItem _heroeshit _asjhero))
      (Utilities|Array|Add _heroeshit _asjhero)
      (Class|JHero|AddHealth _asjhero (* (Variables|Default|GetMeleeDamage) -1.0) 0.2))))

(event EventBeginPlay
  (|CallParentFunction)
  (Variables|Default|SetAnimInstance (Components|SkeletalMesh|GetAnimInstance (Variables|Character|GetMesh)))
  (Utilities|FlowControl|Delay 0.2)
  (bind _outactors (Actor|GetAllActorsOfClass "/Script/PlaygroundHeroes.JHero"))
  (Variables|Default|SetPlayers _outactors))

(event Collision|EventActorBeginOverlap
  (params (OtherActor :type Actor%20Object%20Reference))
  (|CallParentFunction OtherActor) ; This node is disabled and will not be called.\nDrag off pins to build functionality.
)

(event EventTick
  (params (DeltaSeconds :type Float%20%28single-precision%29))
  (bind _animinstance (Variables|Default|GetAnimInstance))
  (|CallParentFunction DeltaSeconds)
  (if (not (Class|AnimInstance|IsAnyMontagePlaying (Variables|Default|GetAnimInstance)))
    (bind _closest (CallFunction|GetClosestPlayer))
    (CallFunction|MoveTowardsPlayer _closest)
    (if (and (Variables|Default|GetIWantToAttack) (< (Transformation|GetDistanceTo _closest) (Variables|Default|GetRange)))
      (Utilities|FlowControl|Sequence
        (:then_0
          (Variables|Default|SetIWantToAttack false)
          (if (< (Math|Random|RandomFloatinRange 0.0 1.0) 0.5)
            (Animation|Montage|MontagePlay _animinstance "/Game/TutorialAssets/TempSkeleton/Animations/bruteAttackMontage.bruteAttackMontage" 1.0 "MontageLength" 0.0 true)
            (else
              (Animation|Montage|MontagePlay _animinstance "/Game/TutorialAssets/TempSkeleton/Animations/bruteAttackMontage2.bruteAttackMontage2" 1.0 "MontageLength" 0.0 true))))
        (:then_1
          (goto _label Reset)))
      (else
        (Utilities|FlowControl|DoOnce false :!label _label
          (:Completed
            (bind _returnvalue (Utilities|Time|SetTimerbyFunctionName 0 "DoAttack" (Variables|Default|GetAttackSpeed)))
            (Variables|Default|SetAttackTimer _returnvalue)))))))

(fn ConstructionScript
  (|CallParentFunction))

(fn GetClosestPlayer
  (for _array_element (Variables|Default|GetPlayers)
    (LocalVariables|Setcurr _array_element)
    ;[1 1 1] Figure out if the current player is the closest player
    (if (and (<= (Transformation|GetDistanceTo (LocalVariables|Getcurr)) (LocalVariables|GetClosestDistance)) (not (Variables|/Script/PlaygroundHeroes.JHero|GetbHasFallen (LocalVariables|Getcurr))))
      (LocalVariables|SetClosestPlayer (LocalVariables|Getcurr))
      (LocalVariables|SetClosestDistance (Transformation|GetDistanceTo (LocalVariables|Getcurr)))
      ;[1 1 1] If any player is out of zorrander's range, we only care about how far they are so we'll ignore the second part of seeing the delta angle
      (if (< (Transformation|GetDistanceTo (LocalVariables|Getcurr)) (Variables|Default|GetRange))
        (LocalVariables|SetBothInRange false)
        (elif (<= (.Yaw (Math|Rotator|BreakRotator (Math|Rotator|Delta(Rotator) (Transformation|GetActorRotation) (Math|Rotator|FindLookatRotation (Transformation|GetActorLocation) (Transformation|GetActorLocation (LocalVariables|Getcurr)))))) (LocalVariables|GetLowestAngleDiff))
          (LocalVariables|SetLowestAnglePlayer (LocalVariables|Getcurr))
          (LocalVariables|SetLowestAngleDiff (.Yaw (Math|Rotator|BreakRotator (Math|Rotator|Delta(Rotator) (Transformation|GetActorRotation) (Math|Rotator|FindLookatRotation (Transformation|GetActorLocation) (Transformation|GetActorLocation (LocalVariables|Getcurr)))))))
          (else
            ;[1 1 1] If they are both in front of zorrander, we only care about the closest player
            (if (> (.Yaw (Math|Rotator|BreakRotator (Math|Rotator|Delta(Rotator) (Transformation|GetActorRotation) (Math|Rotator|FindLookatRotation (Transformation|GetActorLocation) (Transformation|GetActorLocation (LocalVariables|Getcurr)))))) 15.0)
              (LocalVariables|SetBothLessThan15 false)))))))
  (if (LocalVariables|GetBothInRange)
    (return (LocalVariables|GetClosestPlayer))
    (elif (LocalVariables|GetBothLessThan15)
      (return (LocalVariables|GetClosestPlayer))
      (else
        (LocalVariables|SetClosestPlayer (LocalVariables|GetLowestAnglePlayer))))))

(fn MoveTowardsPlayer
  (params (Victim :type J%20Hero%20Object%20Reference))
  (if (Utilities|IsValid Victim)
    (LocalVariables|SetPlayer Victim)
    (LocalVariables|SetDiff (- (Transformation|GetActorLocation Victim) (Transformation|GetActorLocation)))
    (LocalVariables|SetSweetSpotRange (* 0.8 (Variables|Default|GetRange)))
    (CallFunction|RotateTowardsTarget (Utilities|Time|GetWorldDeltaSeconds) (LocalVariables|GetPlayer) true)
    (if (not (<= (Math|Float|Absolute(Float) (- (Math|Vector|VectorLength (LocalVariables|GetDiff)) (LocalVariables|GetSweetSpotRange))) 25.0))
      (if (< (Math|Vector|VectorLength (LocalVariables|GetDiff)) (LocalVariables|GetSweetSpotRange))
        (Class|PawnMovementComponent|AddInputVector (Variables|Character|GetCharacterMovement) (* (Math|Vector|Normalize (LocalVariables|GetDiff)) -0.2) false)
        (else
          (Class|PawnMovementComponent|AddInputVector (Variables|Character|GetCharacterMovement) (* (Math|Vector|Normalize (LocalVariables|GetDiff)) 0.2) false))))))

(fn DoAttack
  (Variables|Default|SetIWantToAttack true))

(fn ClearHeroesHit
  (Utilities|Array|Clear (Variables|Default|GetHeroesHit)))

(fn Explode
  (Game|SpawnActorfromClass "/Game/Blueprints/NewTutorial/SkeletonExplosion.SkeletonExplosion_C" (Transformation|GetWorldTransform (Variables|Default|GetExplosionLocation)) "Undefined" 0 0)
  (Class|JEnemy|AddHealth -1e+04 "EXPLOSION"))