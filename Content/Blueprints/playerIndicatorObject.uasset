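; Player indicator actor that follows its owning hero by snapping to that hero's location every Tick, which also prints a "Hello" debug string.
; The construction script gathers all JHero actors into a Warriors list and derives the other player's index from the owning hero's index.
; Logic to show the Cone only to the owning player's controller exists but is unconnected, and the computed other-player index is unused.
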(event EventBeginPlay)

(event Collision|EventActorBeginOverlap
  (params (OtherActor :type Actor%20Object%20Reference)))

(event EventTick
  (params (DeltaSeconds :type Float%20%28single-precision%29))
  (Development|PrintString "Hello")
  (Transformation|SetActorLocation (Transformation|GetActorLocation (Variables|Default|GetowningHero)) false false))

(fn ConstructionScript
  (Utilities|Array|AddUnique (Variables|Default|GetWarriors) (Variables|Default|GetowningHero))
  (bind _outactors (Actor|GetAllActorsOfClass "/Script/PlaygroundHeroes.JHero"))
  (for _array_element _outactors
    (Utilities|Array|AddUnique (Variables|Default|GetWarriors) _array_element))
  (if (== (Variables|Default|GetowningHeroIndex) 0)
    (Variables|Default|SetotherPlayerIndex 1)
    (else
      (Variables|Default|SetotherPlayerIndex 0))))