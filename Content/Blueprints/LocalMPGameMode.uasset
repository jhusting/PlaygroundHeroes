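; Game mode that sets up two-player local multiplayer when play begins.
; SpawnPlayers creates a second local player without a pawn, then spawns a JHero and a Player1 actor at a fixed elevated location.
; Controller 0 possesses the JHero, while controller 1's Possess call has no pawn connected.
; An unconnected alternative creates a configurable number of players using one shared actor type, with no class set.
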(event EventBeginPlay
  (CallFunction|SpawnPlayers))

(event EventTick
  (params (DeltaSeconds :type Float%20%28single-precision%29)))

(fn ConstructionScript)

(fn SpawnPlayers
  ;[1 1 1] Create 2 different actors
  (Class|GameplayStatics|CreatePlayer 1 false) ; Make other player
  ;;[1 1 1] Spawn Actor Player0 and Connect to Unreal's Player[0]
  (bind _returnvalue (Game|SpawnActorfromClass "/Game/Blueprints/JHero.JHero_C" (Math|Transform|MakeTransform "0, 0,2000.000000") "Undefined" 0 0 47.790989 1e+02 5e+01 1e+02 0))
  (Pawn|Possess (Game|GetPlayerController 0) _returnvalue)
  ;;[1 1 1] Spawn Actor Player1 and Connect to Unreal's Player[1]
  (Game|SpawnActorfromClass "/Game/Player1.Player1_C" (Math|Transform|MakeTransform "0, 0,2000.000000") "Undefined" 0 1 0)
  (Pawn|Possess (Game|GetPlayerController 1)))