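; Actor that stages a timed transition from a "younger" character mesh to an Archer.
; On BeginPlay, a one-shot timer waits a few seconds, then plays the Standing Draw Arrow montage on the SkeletalMesh.
; A Delay matching the active montage's length then hides the SkeletalMesh and shows the Archer, propagating visibility to their child components.
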(event Custom|PlayDrawArrow
  (bind _skeletalmesh (Variables|Default|GetSkeletalMesh))
  (bind _returnvalue (Components|SkeletalMesh|GetAnimInstance _skeletalmesh))
  (Animation|Montage|MontagePlay _returnvalue "/Game/CharacterAssets/Younger/New/Anim/Standing_Draw_Arrow_Montage.Standing_Draw_Arrow_Montage" 1.0 "MontageLength" 0.0 true)
  (bind _returnvalue_2 (Animation|GetPlayLength (Animation|Montage|GetCurrentActiveMontage _returnvalue)))
  (Utilities|FlowControl|Delay _returnvalue_2)
  (CallFunction|SetYoungerInvisible)
  (CallFunction|SetArcherVisible))

(event EventBeginPlay
  (Utilities|Time|SetTimerbyEvent (delegate Custom|PlayDrawArrow) 6.0))

(event Collision|EventActorBeginOverlap
  (params (OtherActor :type Actor%20Object%20Reference)))

(event EventTick
  (params (DeltaSeconds :type Float%20%28single-precision%29)))

(fn ConstructionScript)

(fn NewFunction0)

(fn SetArcherVisible
  (Rendering|SetVisibility (Variables|Default|GetArcher) true true))

(fn SetYoungerInvisible
  (Rendering|SetVisibility (Variables|Default|GetSkeletalMesh) false true))