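; OlderTransitionBP is an actor that stages a visual transition from an older character to a knight.
; Three seconds after BeginPlay, a timer plays a draw-sword montage on the older character's skeletal mesh.
; After a delay equal to the active montage's length, it hides that mesh and reveals the KnightHidden component, swapping visibility with propagation to children.
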(event Custom|Play%20Draw%20Sword
  (bind _skeletalmesh (Variables|Default|GetSkeletalMesh))
  (bind _returnvalue (Components|SkeletalMesh|GetAnimInstance _skeletalmesh))
  (Animation|Montage|MontagePlay _returnvalue "/Game/CharacterAssets/Older/New/Anim/Draw_Sword_2_AnimBP.Draw_Sword_2_AnimBP" 1.0 "MontageLength" 0.0 true)
  (bind _returnvalue_2 (Animation|GetPlayLength (Animation|Montage|GetCurrentActiveMontage _returnvalue)))
  (Utilities|FlowControl|Delay _returnvalue_2)
  (CallFunction|SetOlderInvisible)
  (CallFunction|SetKnightVisible))

(event EventBeginPlay
  (Utilities|Time|SetTimerbyEvent (delegate Custom|Play%20Draw%20Sword) 3.0))

(event Collision|EventActorBeginOverlap
  (params (OtherActor :type Actor%20Object%20Reference)))

(event EventTick
  (params (DeltaSeconds :type Float%20%28single-precision%29)))

(fn ConstructionScript)

(fn SetKnightVisible
  (Rendering|SetVisibility (Variables|Default|GetKnight%20%28Hidden%29) true true))

(fn SetOlderInvisible
  (Rendering|SetVisibility (Variables|Default|GetSkeletalMesh) false true))