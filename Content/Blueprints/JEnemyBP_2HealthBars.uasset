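; Enemy Blueprint with a two-layer health bar, passive health regeneration and death at zero health.
; BeginPlay hands itself to the DoubleLayerEnemyHealthBar widget as EnemyBP.
; Tick updates HealthPercent, destroys the actor at exactly zero, otherwise adds frame-rate-dependent regen capped at MaxHealth.
; A Delay in Tick periodically refreshes OldHealthPercent, so the lower bar trails the current one.
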(event EventBeginPlay
  (bind _asdouble_layer_enemy_health_bar (Utilities|Casting|CastToDoubleLayerEnemyHealthBar (UserInterface|GetUserWidgetObject (Variables|Default|GetHealthBarWidget))))
  (Variables|/Game/Blueprints/UI/DoubleLayerEnemyHealthBar.DoubleLayerEnemyHealthBar_C|SetEnemyBP _asdouble_layer_enemy_health_bar self))

(event Collision|EventActorBeginOverlap
  (params (OtherActor :type Actor%20Object%20Reference)))

(event EventTick
  (params (DeltaSeconds :type Float%20%28single-precision%29))
  ;[1 1 1] Update Health Percentage (thus updatingHealth Bar)
  (bind _asjenemy (Utilities|Casting|CastToJEnemy self))
  (bind _output_get (Variables|/Script/PlaygroundHeroes.JEnemy|SetHealthPercent _asjenemy (/ (Variables|/Script/PlaygroundHeroes.JEnemy|GetHealth _asjenemy) (Variables|/Script/PlaygroundHeroes.JEnemy|GetmaxHealth _asjenemy))))
  ;[1 1 1] <DEATH>: If 0.0%, destroy parent
  (if (== _output_get 0.0)
    (Actor|DestroyActor)
    (else
      ;[1 1 1] <REGEN> Add N% every tick
      (Variables|/Script/PlaygroundHeroes.JEnemy|SetHealth _asjenemy (+ (Variables|/Script/PlaygroundHeroes.JEnemy|GetHealth _asjenemy) (/ (Variables|Default|GetHealthRegenSpeed) 1e+02)))
      ;[1 1 1] If Health>Max Health: Health = Max Health
      (if (> (Variables|/Script/PlaygroundHeroes.JEnemy|GetHealth _asjenemy) (Variables|/Script/PlaygroundHeroes.JEnemy|GetmaxHealth _asjenemy))
        (Variables|/Script/PlaygroundHeroes.JEnemy|SetHealth _asjenemy (Variables|/Script/PlaygroundHeroes.JEnemy|GetmaxHealth _asjenemy)))
      ;[1 1 1] Update Health Old Healt Percentage (thus updating the lower Health Bar)
      (Utilities|FlowControl|Delay (Variables|Default|GetOldHealthBarUpdateDelay))
      (Variables|Default|SetOldHealthPercent (/ (Variables|/Script/PlaygroundHeroes.JEnemy|GetHealth _asjenemy) (Variables|/Script/PlaygroundHeroes.JEnemy|GetmaxHealth _asjenemy))))))

(fn ConstructionScript)