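; Tree boss smash-arm attack actor that shows a growing warning shadow and damages heroes it overlaps while Attack is set.
; Tick shows the Cylinder shadow when Attack is on, scales it quadratically over time, then hides and resets it after a fixed duration.
; Overlaps damage each JHero only once via HeroesHit, which is never cleared here.
; MakeShadowPosition computes a fixed-height transform ahead of the arm, but nothing here calls it.
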(event EventBeginPlay
  (|CallParentFunction) ; This node is disabled and will not be called.\nDrag off pins to build functionality.
)

(event EventTick
  (params (DeltaSeconds :type Float%20%28single-precision%29))
  (|CallParentFunction DeltaSeconds)
  (if (Variables|Default|GetshadowIsActive)
    (CallFunction|UpdateWarningShadow DeltaSeconds)
    (elif (Variables|Default|GetAttack)
      (Variables|Default|SetshadowIsActive true)
      (Rendering|SetVisibility (Variables|Default|GetCylinder) true false))))

(event Collision|EventActorBeginOverlap
  (params (OtherActor :type Actor%20Object%20Reference))
  (bind _heroeshit (Variables|Default|GetHeroesHit))
  (if (Variables|Default|GetAttack)
    (bind _asjhero (Utilities|Casting|CastToJHero OtherActor))
    (if (== -1 (Utilities|Array|FindItem _heroeshit OtherActor))
      (Utilities|Array|Add _heroeshit OtherActor)
      (Class|JHero|AddHealth _asjhero (* (Variables|Default|GetAttackDamage) -1.0)))))

(fn ConstructionScript
  (|CallParentFunction)
  (Variables|Default|SetbaseScale (Transformation|GetWorldScale (Variables|Default|GetCylinder))))

(fn UpdateWarningShadow
  (params (deltaSeconds :type Float%20%28single-precision%29))
  (bind _cylinder (Variables|Default|GetCylinder))
  ;[1 1 1] x^2
  (bind _output_get (Variables|Default|SettimeTrack (+ deltaSeconds (Variables|Default|GettimeTrack))))
  (if (>= (Variables|Default|GettimeTrack) 6.0)
    (Transformation|SetWorldScale3D _cylinder (Variables|Default|GetbaseScale))
    (Variables|Default|SettimeTrack 0.0)
    (Variables|Default|SetshadowIsActive false)
    (Rendering|SetVisibility _cylinder false false)
    (else
      (Transformation|SetWorldScale3D (Variables|Default|GetCylinder) (* (Variables|Default|GetBaseScale) (* (* (Math|Float|Power _output_get 2.0) 0.25) (Variables|Default|GetshadowGrowthRate)))))))

(fn MakeShadowPosition
  (bind _returnvalue (Transformation|GetActorTransform))
  (bind (_location _rotation _scale) (Math|Transform|BreakTransform _returnvalue))
  (bind (_x _y) (Math|Vector|BreakVector _location))
  (return (Math|Transform|MakeTransform (+ (Math|Vector|MakeVector _x _y -136.399994) (* (Transformation|GetActorForwardVector) (* (.X (Math|Vector|BreakVector _scale)) (Variables|Default|GetshadowSpawnDistance)))) "0, 0, 0" (Transformation|GetActorScale3D))))