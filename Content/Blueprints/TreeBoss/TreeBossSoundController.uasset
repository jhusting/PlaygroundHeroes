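; TreeBossSoundController handles music and random battle sound effects for the tree boss fight.
; BeginPlay lowers the music track's pitch and starts a looping timer that plays a random sound from RandomBattleSFX.
; Tick looks up the BossController every frame and raises the music pitch once, when the boss leaves its first phase.
; Pitch and volume randomization for the effects is present but disconnected.
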(event EventBeginPlay
  (Audio|Components|Audio|SetPitchMultiplier (Variables|Default|GetPlayground_Heros_Track_1_Cue%20Lower%20Pitch) 0.8)
  (Utilities|Time|SetTimerbyFunctionName 0 "PlayRandomSFX" (Variables|Default|GetPlayRandomSFXInterval) true))

(event Collision|EventActorBeginOverlap
  (params (OtherActor :type Actor%20Object%20Reference)))

(event EventTick
  (params (DeltaSeconds :type Float%20%28single-precision%29))
  (bind _outactors (Actor|GetAllActorsOfClass "/Game/Blueprints/TreeBoss/BossController.BossController_C"))
  (if (not (Utilities|Enum|Equal(Enum) (Variables|/Game/Blueprints/TreeBoss/BossController.BossController_C|GetCurrentPhase (Utilities|Array|Get(acopy) _outactors)) "NewEnumerator0"))
    (Utilities|FlowControl|DoOnce false
      (:Completed
        (Audio|Components|Audio|SetPitchMultiplier (Variables|Default|GetPlayground_Heros_Track_1_Cue%20Lower%20Pitch) 1.8)))))

(fn ConstructionScript)

(fn PlayRandomSFX
  (bind _randombattlesfx (Variables|Default|GetRandomBattleSFX))
  (bind _randosfxtrack (Variables|Default|GetRandoSFXTrack))
  (Audio|Components|Audio|SetSound _randosfxtrack (Utilities|Array|Get(acopy) _randombattlesfx (Math|Random|RandomIntegerinRange 0 (Utilities|Array|Length _randombattlesfx))))
  (Audio|Components|Audio|Play _randosfxtrack 0.0))