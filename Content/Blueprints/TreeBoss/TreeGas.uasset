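; TreeGas is a gas hazard in the TreeBoss folder that damages heroes standing inside its cone.
; While Active, Tick stretches the actor's Z scale from MinScale to MaxScale over LifeTime, holding at the maximum.
; Cone1 overlap events maintain the HeroesInSmoke list.
; A looping timer started at BeginPlay damages each listed hero that has not fallen every TickSpeed seconds, without checking Active.
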(event OnComponentBeginOverlap(Cone1)
  (params (OverlappedComponent :type Primitive%20Component%20Object%20Reference) (OtherActor :type Actor%20Object%20Reference) (OtherComp :type Primitive%20Component%20Object%20Reference) (OtherBodyIndex :type Integer) (bFromSweep :type Boolean) (SweepResult :type Hit%20Result%20Structure%20%28by%20ref%29))
  (bind _asjhero (Utilities|Casting|CastToJHero OtherActor))
  (Utilities|Array|AddUnique (Variables|Default|GetHeroesInSmoke) _asjhero))

(event OnComponentEndOverlap(Cone1)
  (params (OverlappedComponent :type Primitive%20Component%20Object%20Reference) (OtherActor :type Actor%20Object%20Reference) (OtherComp :type Primitive%20Component%20Object%20Reference) (OtherBodyIndex :type Integer))
  (bind _asjhero (Utilities|Casting|CastToJHero OtherActor))
  (Utilities|Array|RemoveItem (Variables|Default|GetHeroesInSmoke) _asjhero))

(event EventBeginPlay
  (Utilities|Time|SetTimerbyFunctionName 0 "DoDamage" (Variables|Default|GetTickSpeed) true))

(event Collision|EventActorBeginOverlap
  (params (OtherActor :type Actor%20Object%20Reference)))

(event EventTick
  (params (DeltaSeconds :type Float%20%28single-precision%29))
  (bind _returnvalue (Transformation|GetActorScale3D))
  (bind (_x _y) (Math|Vector|BreakVector _returnvalue))
  (if (Variables|Default|GetbActive)
    (Variables|Default|SetCurrLife (Math|Float|Clamp(Float) (+ DeltaSeconds (Variables|Default|GetCurrLife)) 0.0 (Variables|Default|GetLifeTime)))
    (Transformation|SetActorScale3D (Math|Vector|MakeVector _x _y (Math|Float|Lerp (Variables|Default|GetMinScale) (Variables|Default|GetMaxScale) (/ (Variables|Default|GetCurrLife) (Variables|Default|GetLifeTime)))))))

(fn ConstructionScript)

(fn DoDamage
  (for _array_element (Variables|Default|GetHeroesInSmoke)
    (if (not (Variables|/Script/PlaygroundHeroes.JHero|GetbHasFallen _array_element))
      (Class|JHero|AddHealth _array_element (* (Variables|Default|GetDamage) -1.0) 0.0))))