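; JWeakPoint1 is a tree boss weak point Blueprint that shows whether it is alive or burnt.
; Each Tick runs the parent Tick, then ChangeMaterialOnDeath sets BurningCylinder to the hit spot material while Health is above zero, otherwise to the burnt tree material.
; The material is reapplied every frame by polling Health, which this graph only reads.
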(event EventBeginPlay
  (|CallParentFunction) ; This node is disabled and will not be called.\nDrag off pins to build functionality.
)

(event Collision|EventActorBeginOverlap
  (params (OtherActor :type Actor%20Object%20Reference))
  (|CallParentFunction OtherActor) ; This node is disabled and will not be called.\nDrag off pins to build functionality.
)

(event EventTick
  (params (DeltaSeconds :type Float%20%28single-precision%29))
  (|CallParentFunction DeltaSeconds)
  (CallFunction|ChangeMaterialonDeath))

(fn ConstructionScript
  (|CallParentFunction))

(fn ChangeMaterialonDeath
  (bind _burningcylinder (Variables|Default|GetBurningCylinder))
  (if (> (Variables|Default|GetHealth) 0.0)
    (Rendering|Material|SetMaterial _burningcylinder 0 "/Game/TreeBossAssets/Hit_Spot.Hit_Spot")
    (else
      (Rendering|Material|SetMaterial _burningcylinder 0 "/Game/TreeBossAssets/BurntTreeMaterial.BurntTreeMaterial"))))