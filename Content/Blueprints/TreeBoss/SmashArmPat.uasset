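; Tree boss smash-arm attack actor that damages heroes and casts a ground warning shadow while its Attack flag is set.
; Each attacking Tick spawns a new ShadowCaster with a set growth rate, placed at fixed height ahead of the arm by a scale-adjusted distance and matching its rotation.
; Overlaps during an attack subtract AttackDamage from JHero health, using the HeroesHit list to prevent repeat hits.
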(event EventBeginPlay
  (|CallParentFunction) ; This node is disabled and will not be called.\nDrag off pins to build functionality.
)

(event EventTick
  (params (DeltaSeconds :type Float%20%28single-precision%29))
  (bind _warningshadow (Variables|Default|GetwarningShadow))
  (|CallParentFunction DeltaSeconds)
  (if (Variables|Default|GetAttack)
    (CallFunction|SpawnWarningShadow)
    (Utilities|IsValid _warningshadow
      (:Is%20Valid
        (bind _shadowtransform (CallFunction|MakeShadowPosition))
        (Transformation|SetActorTransform _warningshadow _shadowtransform false true)
        (Transformation|SetActorRotation _warningshadow (Transformation|GetActorRotation) true)))))

(event Collision|EventActorBeginOverlap
  (params (OtherActor :type Actor%20Object%20Reference))
  (bind _heroeshit (Variables|Default|GetHeroesHit))
  (if (Variables|Default|GetAttack)
    (bind _asjhero (Utilities|Casting|CastToJHero OtherActor))
    (if (== -1 (Utilities|Array|FindItem _heroeshit OtherActor))
      (Utilities|Array|Add _heroeshit OtherActor)
      (Class|JHero|AddHealth _asjhero (* (Variables|Default|GetAttackDamage) -1.0)))))

(fn ConstructionScript
  (|CallParentFunction))

(fn SpawnWarningShadow
  (bind _shadowtransform (CallFunction|MakeShadowPosition))
  (bind _returnvalue (Game|SpawnActorfromClass "/Game/Blueprints/shadowCaster.shadowCaster_C" _shadowtransform "Undefined" 0 (Variables|Default|GetshadowGrowthRate) (Transformation|GetActorRotation) 0))
  (Variables|Default|SetwarningShadow _returnvalue))

(fn MakeShadowPosition
  (bind _returnvalue (Transformation|GetActorTransform))
  (bind (_location _rotation _scale) (Math|Transform|BreakTransform _returnvalue))
  (bind (_x _y) (Math|Vector|BreakVector _location))
  (return (Math|Transform|MakeTransform (+ (Math|Vector|MakeVector _x _y -136.399994) (* (Transformation|GetActorForwardVector) (* (.X (Math|Vector|BreakVector _scale)) (Variables|Default|GetshadowSpawnDistance)))) "0, 0, 0" (Transformation|GetActorScale3D))))