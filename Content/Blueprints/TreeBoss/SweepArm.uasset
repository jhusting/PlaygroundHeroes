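; SweepArm is a tree boss arm actor that damages heroes it touches during an attack.
; While the Attack flag is set, an overlap with a JHero applies AttackDamage as negative health.
; A HeroesHit array records each victim so a hero is hit only once; this graph never clears that list or sets the flag.
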(event EventBeginPlay
  (|CallParentFunction) ; This node is disabled and will not be called.\nDrag off pins to build functionality.
)

(event EventTick
  (params (DeltaSeconds :type Float%20%28single-precision%29))
  (|CallParentFunction DeltaSeconds) ; This node is disabled and will not be called.\nDrag off pins to build functionality.
)

(event Collision|EventActorBeginOverlap
  (params (OtherActor :type Actor%20Object%20Reference))
  (bind _heroeshit (Variables|Default|GetHeroesHit))
  (if (Variables|Default|GetAttack)
    (bind _asjhero (Utilities|Casting|CastToJHero OtherActor))
    (if (== -1 (Utilities|Array|FindItem _heroeshit OtherActor))
      (Utilities|Array|Add _heroeshit OtherActor)
      (Class|JHero|AddHealth _asjhero (* (Variables|Default|GetAttackDamage) -1.0)))))

(fn ConstructionScript
  (|CallParentFunction))