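; Tree boss smash arm that shows a growing warning shadow and damages heroes it overlaps while attacking.
; When the Attack flag turns on, a DoOnce activates the shadow, which Tick scales along a clamped, accelerating time curve until its display time expires.
; Overlaps during an attack subtract health from each JHero, using a HeroesHit list, never cleared here, to prevent repeat hits.
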(event EventBeginPlay
  (|CallParentFunction) ; This node is disabled and will not be called.\nDrag off pins to build functionality.
)

(event EventTick
  (params (DeltaSeconds :type Float%20%28single-precision%29))
  (|CallParentFunction DeltaSeconds)
  (if (Variables|Shadow|GetshadowIsActive)
    (CallFunction|IsShadowDone)
    (CallFunction|UpdateWarningShadow DeltaSeconds)
    (elif (Variables|Default|GetAttack)
      (Utilities|FlowControl|DoOnce false :!label _label
        (:Completed
          (Variables|Shadow|SetshadowIsActive true)))
      (else
        (goto _label Reset)))))

(event Collision|EventActorBeginOverlap
  (params (OtherActor :type Actor%20Object%20Reference))
  (bind _heroeshit (Variables|Default|GetHeroesHit))
  (if (Variables|Default|GetAttack)
    (bind _asjhero (Utilities|Casting|CastToJHero OtherActor))
    (if (== -1 (Utilities|Array|FindItem _heroeshit OtherActor))
      (Utilities|Array|Add _heroeshit OtherActor)
      (Class|JHero|AddHealth _asjhero (* (Variables|Default|GetAttackDamage) -1.0)))))

(fn ConstructionScript
  (|CallParentFunction)
  (Variables|Shadow|SetbaseScale (Transformation|GetWorldScale (Variables|Default|Getshadow))))

(fn UpdateWarningShadow
  (params (deltaSeconds :type Float%20%28single-precision%29))
  (bind _basescale (Variables|Default|GetBaseScale))
  (bind (_x _y _z) (Math|Vector|BreakVector _basescale))
  ;[1 1 1] Function for calculating Shadow Growth: .0003x^2x + 0.4x +.5
  (bind _output_get (Variables|Shadow|SettimeTrack (+ deltaSeconds (Variables|Shadow|GettimeTrack))))
  (Transformation|SetWorldScale3D (Variables|Default|Getshadow) (Math|Vector|MakeVector 5e+01 (* _y (Math|Float|Clamp(Float) (+ (+ (* (Math|Float|Power _output_get (* (Variables|Shadow|GettimeTrack) 3.0)) 0.0003) (* (Variables|Shadow|GettimeTrack) 0.4)) 0.1) 0.0 (Variables|Shadow|GetmaxScale))) (* _z (Math|Float|Clamp(Float) (+ (+ (* (Math|Float|Power _output_get (* (Variables|Shadow|GettimeTrack) 3.0)) 0.0003) (* (Variables|Shadow|GettimeTrack) 0.4)) 0.1) 0.0 (Variables|Shadow|GetmaxScale)))))
  (Rendering|SetVisibility (Variables|Default|Getshadow) true false))

(fn IsShadowDone
  (bind _shadow (Variables|Default|Getshadow))
  (if (>= (Variables|Shadow|GettimeTrack) (Variables|Shadow|GetmaxShadowDisplayTime))
    (Rendering|SetVisibility _shadow false false)
    (Variables|Shadow|SetshadowIsActive false)
    (Variables|Shadow|SettimeTrack -0.2)
    (Transformation|SetWorldScale3D _shadow (Math|Vector|MakeVector 0.0 0.0 0.0))))