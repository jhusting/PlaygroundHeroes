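; Tree boss weak point actor that launches sap and shows a burnt look once its health runs out.
; FireSap spawns a Sap actor ahead of and above the weak point, with randomized speed and pitch and a random yaw biased to one side of forward.
; Tick calls ChangeMaterialOnDeath, which sets BurningCylinder to the hit-spot or burnt-tree material every frame based on Health.
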(event EventBeginPlay
  (|CallParentFunction) ; This node is disabled and will not be called.\nDrag off pins to build functionality.
)

(event Collision|EventActorBeginOverlap
  (params (OtherActor :type Actor%20Object%20Reference))
  (|CallParentFunction OtherActor) ; This node is disabled and will not be called.\nDrag off pins to build functionality.
)

(event EventTick
  (params (DeltaSeconds :type Float%20%28single-precision%29))
  (|CallParentFunction DeltaSeconds)
  (CallFunction|ChangeMaterialonDeath))

(event EventFireSap
  (Game|SpawnActorfromClass "/Game/Blueprints/TreeBoss/Sap.Sap_C" (Math|Transform|MakeTransform (+ (* (Transformation|GetActorForwardVector) 200) (Transformation|GetActorLocation) (Math|Vector|MakeVector 0.0 0.0 1.5e+02)) (Transformation|GetActorRotation)) "Undefined" 0 (Math|Vector|RotateVector (Transformation|GetActorForwardVector) (Math|Rotator|MakeRotator 0.0 (Math|Random|RandomFloatinRange -45.0 2e+01) (Math|Random|RandomFloatinRange -5.0 -35.0))) (Math|Random|RandomFloatinRange 3.5e+02 1.3e+03) 0))

(fn ConstructionScript
  (|CallParentFunction))

(fn ChangeMaterialonDeath
  (bind _burningcylinder (Variables|Default|GetBurningCylinder))
  (if (> (Variables|Default|GetHealth) 0.0)
    (Rendering|Material|SetMaterial _burningcylinder 0 "/Game/TreeBossAssets/Hit_Spot.Hit_Spot")
    (else
      (Rendering|Material|SetMaterial _burningcylinder 0 "/Game/TreeBossAssets/BurntTreeMaterial.BurntTreeMaterial"))))