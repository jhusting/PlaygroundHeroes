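; SapThrower is a tree boss emitter actor that periodically launches Sap projectiles from its own transform.
; Tick counts FireRate down by delta time and, when it reaches zero, resets it to three seconds and spawns a Sap.
; CreateFiringProperties supplies each Sap with a random upward-biased direction vector and a random initial speed, passed in as spawn parameters.
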(event EventBeginPlay)

(event Collision|EventActorBeginOverlap
  (params (OtherActor :type Actor%20Object%20Reference)))

(event EventTick
  (params (DeltaSeconds :type Float%20%28single-precision%29))
  (bind _output_get (Variables|Default|SetfireRate (- (Variables|Default|GetfireRate) DeltaSeconds)))
  (if (<= _output_get 0.0)
    (Variables|Default|SetfireRate 3.0)
    (bind (_directionvector _speed) (CallFunction|CreateFiringProperties))
    (Game|SpawnActorfromClass "/Game/Blueprints/TreeBoss/Sap.Sap_C" (Transformation|GetActorTransform) "Undefined" 0 _directionvector _speed 0)))

(fn ConstructionScript)

(fn CreateFiringProperties
  (return (Math|Vector|MakeVector (Math|Random|RandomFloatinRange -1e+01 1e+01) (Math|Random|RandomFloatinRange -1e+01 1e+01) 1e+01) (Math|Random|RandomFloatinRange 3.5e+02 8e+02)))