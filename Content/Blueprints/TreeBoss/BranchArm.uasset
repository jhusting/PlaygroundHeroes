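; BranchArm is a tree boss arm actor that turns to face one of two players and exposes attack state.
; Shortly after BeginPlay it picks player 0 or 1 at random and starts tracking.
; Tick yaws it toward that target along the shortest angle at constant RotationSpeed, with a small dead zone.
; DoAttack raises the Attack flag and clears HeroesHit, while ResetAttackBools clears both Attack and Tracking.
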(event EventBeginPlay
  (|CallParentFunction)
  (Utilities|FlowControl|Delay 0.2)
  (CallFunction|PickRandomPlayer)
  (Variables|Default|SetTracking true))

(event Collision|EventActorBeginOverlap
  (params (OtherActor :type Actor%20Object%20Reference))
  (|CallParentFunction OtherActor) ; This node is disabled and will not be called.\nDrag off pins to build functionality.
)

(event EventTick
  (params (DeltaSeconds :type Float%20%28single-precision%29))
  (|CallParentFunction DeltaSeconds)
  (if (Variables|Default|GetTracking)
    (CallFunction|RotateTowardsTarget DeltaSeconds (Variables|Default|GetTarget))))

(fn ConstructionScript
  (|CallParentFunction))

(fn ResetAttackBools
  (Variables|Default|SetAttack false)
  (Variables|Default|SetTracking false))

(fn RotateTowardsTarget
  (params (DeltaTime :type Float%20%28single-precision%29) (Focus :type Actor%20Object%20Reference))
  (bind _returnvalue (Transformation|GetActorLocation Focus))
  (bind _returnvalue_2 (Transformation|GetActorLocation))
  (bind _returnvalue_3 (Transformation|GetActorRotation))
  (bind _returnvalue_4 (Math|Rotator|FindLookatRotation _returnvalue_2 _returnvalue))
  (bind _yaw (Math|Rotator|BreakRotator _returnvalue_3))
  (bind _yaw_2 (Math|Rotator|BreakRotator _returnvalue_4))
  (bind _returnvalue_5 (- _yaw_2 _yaw))
  ;[1 1 1] If the Difference is Small, Dont Do Anything
  (if (not (<= (Math|Float|Absolute(Float) _returnvalue_5) 1.0))
    ;[1 1 1] If the difference is greator than 180, rotate left instead of right
    (if (> _returnvalue_5 1.8e+02)
      (LocalVariables|SetRotationChange (- _returnvalue_5 3.6e+02))
      (else
        ;[1 1 1] If the difference is less than 180, rotate right instead of left
        (if (< _returnvalue_5 -1.8e+02)
          (LocalVariables|SetRotationChange (+ _returnvalue_5 3.6e+02))
          (else
            ;[1 1 1] If its between 180 and -180, then we found the shortest angle
            (LocalVariables|SetRotationChange _returnvalue_5)))))
    (if (> (LocalVariables|GetRotationChange) 0.0)
      ;[1 1 1] If we are rotating right, rotate at rotation speed * 1 (positive)
      (LocalVariables|SetRotationChange (Variables|Default|GetRotationSpeed))
      (else
        ;[1 1 1] If we are rotating left, rotate at rotation speed * -1 (negative)
        (LocalVariables|SetRotationChange (* (Variables|Default|GetRotationSpeed) -1.0))))
    (Transformation|AddActorLocalRotation (Math|Rotator|MakeRotator 0.0 0.0 (* DeltaTime (LocalVariables|GetRotationChange))) false false)))

(fn PickRandomPlayer
  (if (<= (Math|Random|RandomFloatinRange 0.0 1e+02) 5e+01)
    (Variables|Default|SetTarget (Game|GetPlayerCharacter 1))
    (else
      (Variables|Default|SetTarget (Game|GetPlayerCharacter 0)))))

(fn DoAttack
  (Variables|Default|SetAttack true)
  (Utilities|Array|Clear (Variables|Default|GetHeroesHit)))