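; Sap is a tree boss projectile that affects JHero characters and can leave a ground hazard on impact.
; Its construction script sets projectile velocity from Angle and applies InitialSpeed.
; Capsule overlaps apply Damage through AddHealth, using a Targets array and a delay to throttle repeat hits.
; Sphere hits ignore heroes; anything else destroys it, with static mesh actors first spawning a FirePatch below the sphere, offset by its scale.
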(event OnComponentBeginOverlap(Capsule)
  (params (OverlappedComponent :type Primitive%20Component%20Object%20Reference) (OtherActor :type Actor%20Object%20Reference) (OtherComp :type Primitive%20Component%20Object%20Reference) (OtherBodyIndex :type Integer) (bFromSweep :type Boolean) (SweepResult :type Hit%20Result%20Structure%20%28by%20ref%29))
  (bind _targets (Variables|Default|Gettargets))
  (bind _asjhero (Utilities|Casting|CastToJHero OtherActor))
  (bind _returnvalue (Utilities|Array|AddUnique _targets _asjhero))
  (if (!= _returnvalue -1)
    (Class|JHero|AddHealth _asjhero (Variables|combat|Getdamage))
    (Utilities|FlowControl|Delay (Variables|combat|GetreAttackDelay))
    (Utilities|Array|RemoveItem _targets _asjhero)))

(event OnComponentHit(Sphere)
  (params (HitComponent :type Primitive%20Component%20Object%20Reference) (OtherActor :type Actor%20Object%20Reference) (OtherComp :type Primitive%20Component%20Object%20Reference) (NormalImpulse :type Vector :default "0, 0, 0") (Hit :type Hit%20Result%20Structure%20%28by%20ref%29))
  (Utilities|Casting|CastToJHero OtherActor
    (:CastFailed
      (Utilities|Casting|CastToStaticMeshActor OtherActor
        (:then
          (Game|SpawnActorfromClass "/Game/Blueprints/TreeBoss/FirePatch.FirePatch_C" (Math|Conversions|ToTransform(Vector) (- (Transformation|GetWorldLocation HitComponent) (Math|Vector|MakeVector 0.0 0.0 (* (.Z (Math|Vector|BreakVector (Transformation|GetWorldScale (Variables|Default|GetSphere)))) 2e+01)))) "Undefined" 0 0))
        (:CastFailed
          _))
      (Actor|DestroyActor))))

(event EventBeginPlay)

(event Collision|EventActorBeginOverlap
  (params (OtherActor :type Actor%20Object%20Reference)))

(event EventTick
  (params (DeltaSeconds :type Float%20%28single-precision%29)))

(fn ConstructionScript
  (bind _projectilemovement (Variables|Default|GetProjectileMovement))
  (Variables|/Script/Engine.MovementComponent|SetVelocity _projectilemovement (Variables|Projectile|GetAngle))
  (Variables|/Script/Engine.ProjectileMovementComponent|SetInitialSpeed _projectilemovement (Variables|Projectile|GetInitialSpeed)))