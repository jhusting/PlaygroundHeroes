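; Fire patch hazard, filed under TreeBoss, that slows and damages JHero characters standing inside its box.
; Overlap adds heroes to a target list, disabling dodge and cutting movement, while Tick applies Damage per second through AddHealth.
; Leaving restores both and spawns a LingeringDamage actor on the hero at half damage.
; When Expires is set, both a BeginPlay delay and a Tick countdown on LifeTime can destroy the patch.
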(event OnComponentBeginOverlap(Box)
  (params (OverlappedComponent :type Primitive%20Component%20Object%20Reference) (OtherActor :type Actor%20Object%20Reference) (OtherComp :type Primitive%20Component%20Object%20Reference) (OtherBodyIndex :type Integer) (bFromSweep :type Boolean) (SweepResult :type Hit%20Result%20Structure%20%28by%20ref%29))
  (bind _asjhero (Utilities|Casting|CastToJHero OtherActor))
  (bind _returnvalue (Utilities|Array|AddUnique (Variables|Default|Gettargets) _asjhero))
  (if (!= _returnvalue -1)
    (Variables|/Script/PlaygroundHeroes.JHero|SetbCanDodge _asjhero false)
    (Variables|/Script/PlaygroundHeroes.JHero|SetMovementModifier _asjhero 0.25)))

(event OnComponentEndOverlap(Box)
  (params (OverlappedComponent :type Primitive%20Component%20Object%20Reference) (OtherActor :type Actor%20Object%20Reference) (OtherComp :type Primitive%20Component%20Object%20Reference) (OtherBodyIndex :type Integer))
  (bind _asjhero (Utilities|Casting|CastToJHero OtherActor))
  (bind _returnvalue (Utilities|Array|RemoveItem (Variables|Default|Gettargets) _asjhero))
  (if _returnvalue
    (Variables|/Script/PlaygroundHeroes.JHero|SetbCanDodge _asjhero true)
    (Variables|/Script/PlaygroundHeroes.JHero|SetMovementModifier _asjhero 1.0)
    (Game|SpawnActorfromClass "/Game/Blueprints/TreeBoss/LingeringDamage.LingeringDamage_C" (Transformation|GetActorTransform _asjhero) "Undefined" 0 (Variables|Default|GetlingerTime) _asjhero (/ (Variables|Default|Getdamage) 2.0) 0)))

(event EventBeginPlay
  (if (Variables|Default|Getexpires)
    (Utilities|FlowControl|Delay (Variables|Default|GetlifeTime))
    (Actor|DestroyActor)))

(event Collision|EventActorBeginOverlap
  (params (OtherActor :type Actor%20Object%20Reference)))

(event EventTick
  (params (DeltaSeconds :type Float%20%28single-precision%29))
  (if (Variables|Default|Getexpires)
    (CallFunction|LifeTimer DeltaSeconds))
  (for _array_element (Variables|Default|GetTargets)
    (CallFunction|DoDamage _array_element DeltaSeconds)))

(fn ConstructionScript)

(fn LifeTimer
  (params (deltaSeconds :type Float%20%28single-precision%29))
  (bind _output_get (Variables|Default|SetlifeTime (- (Variables|Default|GetlifeTime) deltaSeconds)))
  (if (>= 0.0 _output_get)
    (Actor|DestroyActor)))

(fn DoDamage
  (params (Character :type J%20Hero%20Object%20Reference) (deltaSeconds :type Float%20%28single-precision%29))
  (Class|JHero|AddHealth Character (* deltaSeconds (Variables|Default|Getdamage))))