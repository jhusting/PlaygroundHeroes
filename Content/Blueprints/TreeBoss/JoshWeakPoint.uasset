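; Tree boss weak point that starts spraying Sap projectiles in random forward arcs once damaged, if its health is above 20.
; Tick starts the looping FireSap timer once, and Die pauses it.
; A second timer for a sweeping fan of archer-homing sap is created paused.
; Its distance-based toggle, CheckArcherDistance, is disconnected in the event graph, so nothing here unpauses the fan.
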(event EventBeginPlay
  (|CallParentFunction)
  (bind _returnvalue (Utilities|Time|SetTimerbyFunctionName 0 "Homing Sap Fan" (Variables|Default|GetFanAttackFireRate) true))
  (bind _output_get (Variables|Default|SetHomingFanTimer _returnvalue))
  (Utilities|Time|PauseTimerbyHandle _output_get))

(event Collision|EventActorBeginOverlap
  (params (OtherActor :type Actor%20Object%20Reference)))

(event EventTick
  (params (DeltaSeconds :type Float%20%28single-precision%29))
  (|CallParentFunction DeltaSeconds)
  (if (< (Variables|Default|GetHealth) (Variables|Default|GetmaxHealth))
    (if (not (<= (Variables|Default|GetHealth) 2e+01))
      (Utilities|FlowControl|DoOnce false
        (:Completed
          (bind _returnvalue (Utilities|Time|SetTimerbyFunctionName 0 "FireSap" (Variables|Default|GetfireRate) true))
          (Variables|Default|SetFireTimer _returnvalue)
          (Variables|Default|SetFiring true))))))

(event EventDie
  (Variables|Default|SetFiring false)
  (Utilities|Time|PauseTimerbyHandle (Variables|Default|GetFireTimer)))

(fn ConstructionScript)

(fn FireSap
  (Utilities|FlowControl|Sequence
    (:then_0
      (Game|SpawnActorfromClass "/Game/Blueprints/TreeBoss/Sap.Sap_C" (Math|Transform|MakeTransform (+ (* (Transformation|GetActorForwardVector) 75) (Transformation|GetActorLocation) (Math|Vector|MakeVector 0.0 0.0 1e+02)) (Transformation|GetActorRotation)) "Undefined" 0 (Math|Vector|RotateVector (Transformation|GetActorForwardVector) (Math|Rotator|MakeRotator 0.0 (Math|Random|RandomFloatinRange -45.0 15.0) (Math|Random|RandomFloatinRange -35.0 35.0))) (Math|Random|RandomFloatinRange 3.5e+02 1.3e+03) 0))))

(fn HomingSapFan
  (for _index (range 0 (Variables|Default|GetHomingFanShots))
    (bind (_directionvector _speed) (CallFunction|Phase2FiringProperties))
    (Game|SpawnActorfromClass "/Game/Blueprints/TreeBoss/Sap_Homing_Archer.Sap_Homing_Archer_C" (Math|Transform|MakeTransform (+ (* (Transformation|GetActorForwardVector) 75) (Transformation|GetActorLocation) (Math|Vector|MakeVector 0.0 0.0 4e+02)) (Transformation|GetActorRotation)) "Undefined" 0 1.0 3.5e+02 _directionvector (* _speed 1e+01) 0)
    (Development|PrintString "Hello")))

(fn CheckArcherDistance
  (bind _homingfantimer (Variables|Default|GetHomingFanTimer))
  (bind _outactors (Actor|GetAllActorsOfClass "/Game/Blueprints/Warriors/JArcherBP.JArcherBP_C"))
  (if (< (Variables|Default|GetMinDistanceForFanAttack) (Transformation|GetDistanceTo self (Utilities|Array|Get(acopy) _outactors)))
    (Utilities|FlowControl|Sequence
      (:then_0
        (Utilities|FlowControl|DoOnce false :!label _label
          (:Completed
            (Utilities|Time|UnpauseTimerbyHandle _homingfantimer))))
      (:then_1
        (goto _label_2 Reset)))
    (else
      (Utilities|FlowControl|Sequence
        (:then_0
          (Utilities|FlowControl|DoOnce false :!label _label_2
            (:Completed
              (Utilities|Time|PauseTimerbyHandle _homingfantimer))))
        (:then_1
          (goto _label Reset))))))

(fn Phase2FiringProperties
  (if (Variables|Default|GetgoingUp)
    (if (>= (Variables|Default|GetLastPhase2YValue) 4)
      (Variables|Default|SetgoingUp false))
    (Variables|Default|SetLastPhase2YValue (+ (Variables|Default|GetLastPhase2YValue) 1))
    (else
      (if (<= (Variables|Default|GetLastPhase2YValue) -4)
        (Variables|Default|SetgoingUp true))
      (Variables|Default|SetLastPhase2YValue (+ (Variables|Default|GetLastPhase2YValue) -1))))
  (return (Math|Vector|MakeVector 0.0 (Math|Conversions|ToFloat(Integer) (Variables|Default|GetLastPhase2YValue)) 5.0) 1e+03))