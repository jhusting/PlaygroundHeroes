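; Trigger actor that plays the story dialogue between Leila and Abigail before the Tree boss fight.
; On BeginPlay it caches the first JDialogueHandler found in the level.
; When a JHero overlaps its Box, it sends the hardcoded lines, a duration and per-speaker font indices to that handler, using a DialogueSent flag to fire only once.
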(event OnComponentBeginOverlap(Box)
  (params (OverlappedComponent :type Primitive%20Component%20Object%20Reference) (OtherActor :type Actor%20Object%20Reference) (OtherComp :type Primitive%20Component%20Object%20Reference) (OtherBodyIndex :type Integer) (bFromSweep :type Boolean) (SweepResult :type Hit%20Result%20Structure%20%28by%20ref%29))
  (Utilities|Casting|CastToJHero OtherActor)
  (if (not (Variables|Default|GetDialogueSent))
    (Class|DialogueHandler|SendNewdialogueSequence (Variables|Default|GetdialogueHandler) (Utilities|Array|MakeArray "LEILA: Wow look at that tree... It seems so out of place in this clearing, almost like it’s guarding this place. " "LEILA: Abigail do you think it’s one of the monsters Zorrander sent after us?" "ABIGAIL: It must be! But... it looks so sad. It’s crumbling apart and it’s all alone here. " "ABIGAIL: Do you think it’s sick?" "LEILA: Sick? What do you mean?" "ABIGAIL: Look, the trunk is split in the middle and the inside is black. " "ABIGAL: It must be where Zorrander put the piece of his heart. The evil in his heart spread throughout the tree, " "ABIGAIL: stealing its life and beauty.... " "ABIGAIL: slowly killing it until only its burnt body was left. " "ABIGAIL: Now Zorrander’s heart can control the tree like a puppet!" "LEILA: If Zorrander releases his curse the whole kingdom will end up like this tree." "LEILA: C’mon we have to destroy this tree to weaken Zorrander!") (Utilities|Array|MakeArray 4.0) (Utilities|Array|MakeArray 1 1 2 2 1 2 2 2 2 2 1 1))
    (Variables|Default|SetDialogueSent true)))

(event EventBeginPlay
  (bind _outactors (Actor|GetAllActorsOfClass "/Game/Blueprints/UI/JDialogueHandler.JDialogueHandler_C"))
  (Variables|Default|SetdialogueHandler (Utilities|Array|Get(acopy) _outactors)))

(event Collision|EventActorBeginOverlap
  (params (OtherActor :type Actor%20Object%20Reference)))

(event EventTick
  (params (DeltaSeconds :type Float%20%28single-precision%29)))

(fn ConstructionScript)