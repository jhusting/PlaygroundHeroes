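; RootBase is a tree boss root with health and an up/down state flag that flips when its health runs out.
; Tick watches HealthPercent and, at zero or below, calls MoveRoot, which toggles IsUp and refills Health to MaxHealth.
; A three-second timer then calls MoveRoot again to flip the state back.
; The graph only sets the flag and contains no movement logic.
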(event EventBeginPlay
  (|CallParentFunction) ; This node is disabled and will not be called.\nDrag off pins to build functionality.
)

(event Collision|EventActorBeginOverlap
  (params (OtherActor :type Actor%20Object%20Reference))
  (|CallParentFunction OtherActor) ; This node is disabled and will not be called.\nDrag off pins to build functionality.
)

(event EventTick
  (params (DeltaSeconds :type Float%20%28single-precision%29))
  (|CallParentFunction DeltaSeconds)
  (if (<= (Variables|Default|GetHealthPercent) 0.0)
    (CallFunction|MoveRoot)
    (Utilities|Time|SetTimerbyFunctionName 0 "MoveRoot" 3.0)))

(fn ConstructionScript
  (|CallParentFunction))

(fn MoveRoot
  (Variables|Default|SetbIsUp (not (Variables|Default|GetbIsUp)))
  (Variables|Default|SetHealth (Variables|Default|GetmaxHealth)))