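; Controller for the tree boss fight, which finds the arms, weak points and roots, creates the health bar and plays voiced dialogue.
; Tick polls a phase switcher: a firing weak point moves the roots and starts looping smash-arm attacks on random players.
; An empty weak-point list ends the attacks, disables gas, plays victory dialogue and reloads the return map.
; Sweep-arm and attack-sequence functions exist but are not called here.
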(event EventBeginPlay
  (bind _audio (Variables|Default|GetAudio))
  (bind _asplayground_game_instance (Utilities|Casting|CastToPlaygroundGameInstance (Game|GetGameInstance)))
  (Development|PrintString (Variables|/Game/Blueprints/PlaygroundGameInstance.PlaygroundGameInstance_C|GetReturnMap _asplayground_game_instance))
  (bind _outactors (Actor|GetAllActorsOfClass "/Game/Blueprints/TreeBoss/SmashArm.SmashArm_C"))
  (if (Utilities|Array|IsValidIndex _outactors)
    (Variables|Default|SetSmashArm (Utilities|Array|Get(acopy) _outactors)))
  (bind _outactors_2 (Actor|GetAllActorsOfClass "/Game/Blueprints/TreeBoss/SweepArm.SweepArm_C"))
  (if (Utilities|Array|IsValidIndex _outactors_2)
    (Variables|Default|SetSweepArm (Utilities|Array|Get(acopy) _outactors_2)))
  (bind _outactors_3 (Actor|GetAllActorsOfClass "/Game/Blueprints/TreeBoss/JoshWeakPoint.JoshWeakPoint_C"))
  (Variables|Default|SetWeakPoints _outactors_3)
  (bind _outactors_4 (Actor|GetAllActorsOfClass "/Game/Blueprints/TreeBoss/RootBase.RootBase_C"))
  (Variables|Default|SetRoots _outactors_4)
  (bind _returnvalue (UserInterface|CreateWidget "/Game/Blueprints/UI/TreeBoss3HealthBar.TreeBoss3HealthBar_C" (Game|GetPlayerController 0)))
  (Variables|/Game/Blueprints/UI/TreeBoss3HealthBar.TreeBoss3HealthBar_C|SetRootWeakpoints _returnvalue (Variables|Default|GetWeakPoints))
  (UserInterface|Viewport|AddtoViewport _returnvalue 0)
  (bind _outactors_5 (Actor|GetAllActorsOfClass "/Game/Blueprints/UI/JDialogueHandler.JDialogueHandler_C"))
  (Variables|Default|SetDialogueHandler (Utilities|Array|Get(acopy) _outactors_5))
  (Class|DialogueHandler|SendNewdialogueSequence (Variables|Default|GetDialogueHandler) (Utilities|Array|MakeArray "This tree is too strong, we have to find weak spots!") (Utilities|Array|MakeArray 4.2) (Utilities|Array|MakeArray 0) (Utilities|Array|MakeArray "LEILA"))
  (Audio|Components|Audio|SetSound _audio "/Game/Audio/Dialog/Leila_Single_Lines/L__This_tree_is_to_strong____have_to_find_the_weak_spots.L__This_tree_is_to_strong____have_to_find_the_weak_spots")
  (Audio|Components|Audio|Play _audio 0.0)
  (bind _asplayground_game_instance_2 (Utilities|Casting|CastToPlaygroundGameInstance (Game|GetGameInstance)))
  (Variables|/Game/Blueprints/PlaygroundGameInstance.PlaygroundGameInstance_C|SetTreeBossChallenged _asplayground_game_instance_2 true))

(event Collision|EventActorBeginOverlap
  (params (OtherActor :type Actor%20Object%20Reference)))

(event EventTick
  (params (DeltaSeconds :type Float%20%28single-precision%29))
  (bind _audio (Variables|Default|GetAudio))
  (CallFunction|FirstWeakPointKillDialogue)
  (CallFunction|PhaseSwitcher)
  (if (Utilities|Enum|Equal(Enum) (Variables|Default|GetCurrentPhase) "NewEnumerator1")
    (if (not (Utilities|Time|IsTimerActivebyHandle (Variables|Default|GetAttackTimer)))
      (bind _returnvalue (Utilities|Time|SetTimerbyFunctionName 0 "AttackSmashArm" (Variables|Default|GetPhase2AttackSpeed) true))
      (Variables|Default|SetAttackTimer _returnvalue)
      (CallFunction|AttackSmashArm))
    (elif (Utilities|Enum|Equal(Enum) (Variables|Default|GetCurrentPhase) "NewEnumerator2")
      (Utilities|FlowControl|DoOnce false
        (:Completed
          (bind _outactors (Actor|GetAllActorsOfClass "/Game/Blueprints/TreeBoss/TreeGas.TreeGas_C"))
          (for _array_element _outactors
            (Variables|/Game/Blueprints/TreeBoss/TreeGas.TreeGas_C|SetbActive _array_element false))
          (Class|DialogueHandler|SendNewdialogueSequence (Variables|Default|GetDialogueHandler) (Utilities|Array|MakeArray "We did it! We destroyed Zorrander’s monster!" "… but we still have to be careful. Zorrander is weaker, but we still don’t know how powerful he is." "Well let’s go finish him off!" "Okay, are you sure you’re feeling up to it? You’re not too… tired are you?" "I’m fine, hurry up let’s go Leila!") (Utilities|Array|MakeArray 4.0 6.0 2.0 5.5 3.0) (Utilities|Array|MakeArray 0 0 0 0 0) (Utilities|Array|MakeArray "ABIGAIL" "LEILA" "ABIGAIL" "LEILA" "ABIGAIL"))
          (Audio|Components|Audio|SetSound _audio "/Game/Audio/Dialog/Cinematics/FULL_SCENES-_One_cuts/Post_Tree_Fight.Post_Tree_Fight")
          (Audio|Components|Audio|Play _audio 0.0)
          (Utilities|Time|SetTimerbyFunctionName 0 "BackToWorld" 22.0)
          (bind _foundwidgets (Widget|GetAllWidgetsOfClass "/Game/Blueprints/UI/TreeBoss3HealthBar.TreeBoss3HealthBar_C" true))
          (for _array_element_2 _foundwidgets
            (Widget|RemovefromParent _array_element_2)))))))

(fn ConstructionScript)

(fn PhaseSwitcher
  (if (Utilities|Enum|Equal(Enum) (Variables|Default|GetCurrentPhase) "NewEnumerator0")
    (for _array_element (Variables|Default|GetWeakPoints)
      (if (Variables|/Game/Blueprints/TreeBoss/JoshWeakPoint.JoshWeakPoint_C|GetFiring _array_element)
        (Utilities|FlowControl|DoOnce false
          (:Completed
            (Variables|Default|SetCurrentPhase "NewEnumerator1")
            (Variables|Default|SetcurrentAttackSpeed (Variables|Default|GetPhase1AttackSpeed))
            (CallFunction|MoveRoots)))))
    (elif (and (Utilities|Enum|Equal(Enum) (Variables|Default|GetCurrentPhase) "NewEnumerator1") (== (Utilities|Array|Length (Variables|Default|GetWeakPoints)) 0))
      (Variables|Default|SetCurrentPhase "NewEnumerator2")
      (Variables|Default|SetcurrentAttackSpeed (Variables|Default|GetPhase2AttackSpeed))
      (Utilities|Time|ClearandInvalidateTimerbyHandle (Variables|Default|GetAttackTimer))
      (CallFunction|MoveRoots)
      (elif (Utilities|Enum|Equal(Enum) (Variables|Default|GetCurrentPhase) "NewEnumerator2")
        (Utilities|FlowControl|DoOnce false
          (:Completed
            (Variables|Default|SetCurrentPhase "NewEnumerator4")))
        (elif (Utilities|Enum|Equal(Enum) (Variables|Default|GetCurrentPhase) "NewEnumerator4")
          _)))))

(fn AttackSmashArm
  (bind _smasharm (Variables|Default|GetSmashArm))
  (if (Utilities|IsValid _smasharm)
    (Default|PickRandomPlayer _smasharm)
    (Default|DoAttack _smasharm)))

(fn MoveRoots
  (for _array_element (Variables|Default|GetRoots)
    (Default|MoveRoot _array_element)))

(fn FirstWeakPointKillDialogue
  (bind _weakpoints (Variables|Default|GetWeakPoints))
  (bind _returnvalue (Utilities|Array|Length _weakpoints))
  (if (and (not (Variables|Default|GetfirstWeakPointKilled)) (== _returnvalue (- _returnvalue 1)))
    (Class|DialogueHandler|SendNewdialogueSequence (Variables|Default|GetDialogueHandler) (Utilities|Array|MakeArray "Nice job!" "Now we gotta get through to the other roots to take them down!") (Utilities|Array|MakeArray 3.0 4.0) (Utilities|Array|MakeArray 1 1) (Utilities|Array|MakeArray "LEILA" "LEILA"))
    (Variables|Default|SetfirstWeakPointKilled true)))

(fn BacktoWorld
  (bind _asplayground_game_instance (Utilities|Casting|CastToPlaygroundGameInstance (Game|GetGameInstance)))
  (bind _returnvalue (UserInterface|CreateWidget "/Game/Blueprints/UI/LoadSplash.LoadSplash_C"))
  (UserInterface|Viewport|AddtoViewport _returnvalue 0)
  (Game|OpenLevel(byName) (Utilities|String|StringToName (Variables|/Game/Blueprints/PlaygroundGameInstance.PlaygroundGameInstance_C|GetReturnMap _asplayground_game_instance))))

(fn AttackSweepArm
  (bind _sweeparm (Variables|Default|GetSweepArm))
  (if (Utilities|IsValid _sweeparm)
    (Default|PickRandomPlayer _sweeparm)
    (Default|DoAttack _sweeparm)))

(fn MakeAttackSequences
  (Variables|Default|SetAttackSequences (Utilities|Array|MakeArray (Utilities|Struct|MakeAttackSequence (Utilities|Array|MakeArray "AttackSmashArm") (Utilities|Array|MakeArray (Variables|Default|GetcurrentAttackSpeed)))))
  (return false))

(fn GetNewAttackSequence
  (bind _attacksequences (Variables|Default|GetAttackSequences))
  (Variables|Default|SetcurrentAttackSequence (Utilities|Array|Get(acopy) _attacksequences (Math|Random|RandomInteger (Utilities|Array|Length _attacksequences))))
  (Variables|Default|SetAttackSequenceProgress 0))

(fn NextAttackinSequence
  (bind _currentattacksequence (Variables|Default|GetcurrentAttackSequence))
  (Utilities|Time|ClearandInvalidateTimerbyHandle (Variables|Default|GetAttackTimer))
  (if (>= (Variables|Default|GetAttackSequenceProgress) (Utilities|Array|Length (.attacknames _currentattacksequence)))
    (Variables|Default|SetAttackSequenceProgress -1)
    (else
      (bind _returnvalue (Utilities|Time|SetTimerbyFunctionName 0 (Utilities|Array|Get(acopy) (.attacknames _currentattacksequence) (Variables|Default|GetAttackSequenceProgress)) (Utilities|Array|Get(acopy) (.delays _currentattacksequence) (Variables|Default|GetAttackSequenceProgress))))
      (Variables|Default|SetAttackTimer _returnvalue)
      (Math|Integer|IncrementInt (Variables|Default|GetAttackSequenceProgress)))))

(fn PlaySliceRootAudio
  (bind _audio (Variables|Default|GetAudio))
  (if (not (Variables|Default|GetSliceAudioPlayed))
    (Class|DialogueHandler|SendNewdialogueSequence (Variables|Default|GetdialogueHandler) (Utilities|Array|MakeArray "Nice job! Now let's slice this root down to get to the other weak spot" "") (Utilities|Array|MakeArray 5.0 0.0) (Utilities|Array|MakeArray 0 0) (Utilities|Array|MakeArray "ABIGAIL" ""))
    (Audio|Components|Audio|SetSound _audio "/Game/Audio/Dialog/Abigail_Single_lines/A__Nice_Job____Now_Lets_slice.A__Nice_Job____Now_Lets_slice")
    (Audio|Components|Audio|Play _audio 0.0)
    (Variables|Default|SetSliceAudioPlayed true)))