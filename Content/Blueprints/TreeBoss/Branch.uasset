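; Branch actor for the tree boss that temporarily moves out of position when its health is depleted, then recovers.
; Tick polls HealthPercent and, through a DoOnce gate, instantly shifts the actor by MoveOffset with a swept move.
; After the UpTime delay it moves back by the same offset, restores Health to MaxHealth and resets the gate for the next cycle.
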(event EventBeginPlay
  (|CallParentFunction) ; This node is disabled and will not be called.\nDrag off pins to build functionality.
)

(event Collision|EventActorBeginOverlap
  (params (OtherActor :type Actor%20Object%20Reference))
  (|CallParentFunction OtherActor) ; This node is disabled and will not be called.\nDrag off pins to build functionality.
)

(event EventTick
  (params (DeltaSeconds :type Float%20%28single-precision%29))
  (bind _self self)
  (bind _moveoffset (Variables|Default|GetMoveOffset))
  (bind _returnvalue (Transformation|GetActorLocation _self))
  (|CallParentFunction DeltaSeconds)
  (if (<= (Variables|Default|GetHealthPercent) 0.0)
    (Utilities|FlowControl|DoOnce false :!label _label
      (:Completed
        ;[1 1 1] Move up to location
        (Transformation|SetActorLocation (+ _returnvalue _moveoffset) true false)
        (Utilities|FlowControl|Delay (Variables|Default|GetUpTime))
        ;[1 1 1] Move back down
        (Transformation|SetActorLocation (- _returnvalue _moveoffset) true false)
        (Variables|Default|SetHealth (Variables|Default|GetmaxHealth))
        (goto _label Reset)))))

(fn ConstructionScript
  (|CallParentFunction))