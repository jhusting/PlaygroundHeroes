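; Trigger-box actor that plays a Level Sequence cutscene with dialogue for the two kid players, Younger and Older.
; Tick polls overlapping kids, showing split-screen ready prompts until one or both hold A as configured, or auto-starts after a delay.
; Starting saves return locations to the GameInstance, removes player two and switches to the sequence camera.
; AfterEndSequence either loads another level or respawns player two and restores control.
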(event OnComponentBeginOverlap(Box)
  (params (OverlappedComponent :type Primitive%20Component%20Object%20Reference) (OtherActor :type Actor%20Object%20Reference) (OtherComp :type Primitive%20Component%20Object%20Reference) (OtherBodyIndex :type Integer) (bFromSweep :type Boolean) (SweepResult :type Hit%20Result%20Structure%20%28by%20ref%29))
  (bind _warriors (Variables|Default|GetWarriors))
  ;[1 1 1] If Not All Needed Components Are Valid, Print An Error
  (if (Variables|Default|GetComponentsValid)
    (bind _asjkid (Utilities|Casting|CastToJKid OtherActor))
    (Utilities|Array|AddUnique _warriors _asjkid)
    (if (== (Utilities|Array|Length _warriors) 1) ; if first player entered
      (Class|DialogueHandler|SaveDialogue (Variables|Default|GetDialogHandler)))
    (else
      (CallFunction|PrintOutLogsOfBadComponents)
      (Development|PrintString (Utilities|String|Append (Utilities|GetDisplayName self) ": PlayCutsceneChildren: (ERROR) Cannot Play Sequence: Not All Needed Components are Defined/Valid. ") true true "(R=0.812500,G=0.000000,B=0.115263,A=1.000000)" 5.0))))

(event OnComponentEndOverlap(Box)
  (params (OverlappedComponent :type Primitive%20Component%20Object%20Reference) (OtherActor :type Actor%20Object%20Reference) (OtherComp :type Primitive%20Component%20Object%20Reference) (OtherBodyIndex :type Integer))
  (bind _warriors (Variables|Default|GetWarriors))
  (bind _asjkid (Utilities|Casting|CastToJKid OtherActor))
  (Utilities|Array|RemoveItem _warriors _asjkid)
  (if (== (Utilities|Array|Length _warriors) 0)
    ;[1 1 1] If last person inside left, clear out text
    (CallFunction|PrintDialog (Utilities|Array|MakeArray (Utilities|String|MakeLiteralString)) (Utilities|Array|MakeArray 0.0) (Utilities|Array|MakeArray 1) (Utilities|Array|MakeArray "") false true)
    (Class|DialogueHandler|LoadSavedDialogue (Variables|Default|GetDialogHandler))))

(event EventBeginPlay
  (if (Variables|Default|GetGlobalEnabled)
    (bind _outactors (Actor|GetAllActorsOfClass "/Script/PlaygroundHeroes.DialogueHandler"))
    (Variables|Default|SetDialogHandler (Utilities|Array|Get(acopy) _outactors))
    (CallFunction|CheckforRequiredComponents)
    ;[1 1 1] If Not All Needed Components Are Valid, Print An Error
    (if (not (Variables|Default|GetComponentsValid))
      (CallFunction|PrintOutLogsOfBadComponents)
      (Development|PrintString (Utilities|String|Append (Utilities|GetDisplayName self) ": PlayCutsceneChildren: (ERROR) Cannot Play Sequence: Not All Needed Components are Defined/Valid. ") true true "(R=0.812500,G=0.000000,B=0.115263,A=1.000000)" 5.0))))

(event Collision|EventActorBeginOverlap
  (params (OtherActor :type Actor%20Object%20Reference)))

(event EventTick
  (params (DeltaSeconds :type Float%20%28single-precision%29))
  (bind _warriors (Variables|Default|GetWarriors))
  (bind _returnvalue (Utilities|Array|Length _warriors))
  (if (Variables|Default|GetGlobalEnabled)
    (if (or (Variables|Default|GetIsBoss) (not (Variables|Default|GetSequenceAlreadyPlayed)))
      (if true
        (if (Variables|AutoStartAfterDelay|GetPlayOnStart)
          (Utilities|FlowControl|Delay (Variables|AutoStartAfterDelay|GetDelayOfStart))
          (Utilities|FlowControl|DoOnce false
            (:Completed
              (SequenceRelated|InitiateSequence)))
          (elif (Variables|Default|GetOnlyOneCharacterNeeded)
            ;[1 1 1] If Either Presses 'A' Button and OnlyOneCharacterNeeded is TRUE
            (for _array_element (Collision|GetOverlappingActors "/Script/PlaygroundHeroes.JKid" :!class /Script/Engine.Actor)
              (bind _asjkid (Utilities|Casting|CastToJKid _array_element))
              (CallFunction|OnlyOneNeeded _asjkid))
            (elif (== _returnvalue 2)
              (CallFunction|BothPresent)
              (elif (== 1 _returnvalue)
                (CallFunction|OnlyOnePresent)))))))))

(event Input|GamepadEvents|GamepadFaceButtonBottom
  (params (Key :type Key%20Structure)))

(fn ConstructionScript)

(fn PrintDialog
  (params (Lines :type Array%20of%20Strings) (Durations :type Array%20of%20Floats%20%28single-precision%29) (FOnts :type Array%20of%20Integers) (characters :type Array%20of%20Strings) (Split :type Boolean) (PauseAfter :type Boolean))
  (bind _dialoghandler (Variables|Default|GetDialogHandler))
  (Class|DialogueHandler|ToggleSplitMode _dialoghandler Split)
  (Class|DialogueHandler|SendNewdialogueSequence _dialoghandler Lines Durations FOnts characters)
  (if PauseAfter
    (Class|DialogueHandler|Pause _dialoghandler)))

(fn BothPresent
  (bind _warriors (Variables|Default|GetWarriors))
  (bind _temparray (Variables|Default|GetTempArray))
  (bind _output (Utilities|Array|Get(acopy) _warriors))
  (bind _output_2 (Utilities|Array|Get(acopy) _warriors 1))
  (bind _interacting (Variables|/Script/PlaygroundHeroes.JKid|Getinteracting _output_2))
  (bind _interacting_2 (Variables|/Script/PlaygroundHeroes.JKid|Getinteracting _output))
  ;[1 1 1] We want our array to be ordered Archer, Knight
  ;;[1 1 1] If the array order is Archer, Knight
  (bind _asyounger (Utilities|Casting|CastToYounger _output)
    (:then
      (Utilities|Array|AddUnique _temparray _asyounger)
      (bind _asolder (Utilities|Casting|CastToOlder _output_2))
      (Utilities|Array|AddUnique _temparray _asolder))
    (:CastFailed
      ;;[1 1 1] If array order is Knight, Archer
      (bind _asyounger_2 (Utilities|Casting|CastToYounger _output_2))
      (Utilities|Array|AddUnique (Variables|Default|GetTempArray) _asyounger_2)
      (Utilities|Casting|CastToOlder _output)))
  ;[1 1 1] Both pressing A
  (if (and _interacting_2 _interacting)
    (SequenceRelated|InitiateSequence)
    (else
      ;[1 1 1] Don't show prompt when sequence is playing
      (if (not (Audio|Components|Audio|IsPlaying (Variables|/Script/LevelSequence.LevelSequenceActor|GetSequencePlayer (Variables|Sequence|GetSequenceToPlay))))
        ;[1 1 1] A pressing A, B in
        (if (and (not _interacting_2) _interacting)
          (CallFunction|PrintDialog (Utilities|Array|MakeArray "Readied" (Utilities|String|Append "Hold A to inspect " (Variables|Default|GetObjectNameDisplayed))) (Utilities|Array|MakeArray 0.0 0.0) (Utilities|Array|MakeArray 1 2) (Utilities|Array|MakeArray "") true true)
          (else
            ;[1 1 1] A In, B pressing A
            (if (and _interacting_2 (not _interacting))
              (CallFunction|PrintDialog (Utilities|Array|MakeArray (Utilities|String|Append "Hold A to inspect " (Variables|Default|GetObjectNameDisplayed)) "Readied") (Utilities|Array|MakeArray 0.0 0.0) (Utilities|Array|MakeArray 1 2) (Utilities|Array|MakeArray "") true true)
              (else
                ;[1 1 1] Neither is pressing A
                (CallFunction|PrintDialog (Utilities|Array|MakeArray "Hold A to Ready Up" "") (Utilities|Array|MakeArray 0.0 0.0) (Utilities|Array|MakeArray 1 1) (Utilities|Array|MakeArray "") false true)))))))))

(fn OnlyOnePresent
  (bind _warriors (Variables|Default|GetWarriors))
  (bind _output (Utilities|Array|Get(acopy) _warriors))
  ;[1 1 1] Is the one actor an archer?
  (Utilities|Casting|CastToYounger _output
    (:then
      ;[1 1 1] Is the Archer present pressing A?
      (if (Variables|/Script/PlaygroundHeroes.JKid|Getinteracting _output)
        (CallFunction|PrintDialog (Utilities|Array|MakeArray "Readied" (Utilities|String|Append "Abigail: Come over here, lets look at " (Variables|Default|GetObjectNameDisplayed))) (Utilities|Array|MakeArray 0.0 0.0) (Utilities|Array|MakeArray 1 2) (Utilities|Array|MakeArray "") true true)
        (else
          (CallFunction|PrintDialog (Utilities|Array|MakeArray "Hold A to ready up" "") (Utilities|Array|MakeArray 0.0 0.0) (Utilities|Array|MakeArray 1 1) (Utilities|Array|MakeArray "") true true))))
    (:CastFailed
      ;[1 1 1] Is the Knight presing A?
      (if (Variables|/Script/PlaygroundHeroes.JKid|Getinteracting _output)
        (CallFunction|PrintDialog (Utilities|Array|MakeArray (Utilities|String|Append "Leila: Come over here, lets look at " (Variables|Default|GetObjectNameDisplayed)) "Readied") (Utilities|Array|MakeArray 0.0 0.0) (Utilities|Array|MakeArray 1 2) (Utilities|Array|MakeArray "") true true)
        (else
          (CallFunction|PrintDialog (Utilities|Array|MakeArray "" "Hold A to ready up") (Utilities|Array|MakeArray 0.0 0.0) (Utilities|Array|MakeArray 1 2) (Utilities|Array|MakeArray "") true true))))))

(fn SetKidReturnLocationsOfGameInstance
  (bind _asplayground_game_instance (Utilities|Casting|CastToPlaygroundGameInstance (Game|GetGameInstance)))
  (Utilities|IsValid _asplayground_game_instance
    (:Is%20Valid
      ;[1 1 1] Set Next Level and Keep Track of This Level (So we can return back)
      (Variables|/Game/Blueprints/PlaygroundGameInstance.PlaygroundGameInstance_C|SetDesiredMap _asplayground_game_instance (Variables|LevelChange|GetDesiredLevel))
      (bind _returnvalue (Game|GetCurrentLevelName true))
      (Variables|/Game/Blueprints/PlaygroundGameInstance.PlaygroundGameInstance_C|SetReturnMap _asplayground_game_instance _returnvalue)
      ;[1 1 1] Store Abigail Position
      (bind _outactors (Actor|GetAllActorsOfClass "/Game/Blueprints/Children/Younger.Younger_C"))
      (Variables|/Game/Blueprints/PlaygroundGameInstance.PlaygroundGameInstance_C|SetPlayer%200%20Vector%203 _asplayground_game_instance (Math|Vector|MakeVector (.X (Math|Vector|BreakVector (Transformation|GetActorLocation (Utilities|Array|Get(acopy) _outactors)))) (.Y (Math|Vector|BreakVector (Transformation|GetActorLocation (Utilities|Array|Get(acopy) _outactors)))) (+ (.Z (Math|Vector|BreakVector (Transformation|GetActorLocation (Utilities|Array|Get(acopy) _outactors)))) 25.0)))
      (Variables|/Game/Blueprints/PlaygroundGameInstance.PlaygroundGameInstance_C|SetPlayer%200%20Boolean _asplayground_game_instance true)
      ;[1 1 1] Store Leila's Position
      (bind _outactors_2 (Actor|GetAllActorsOfClass "/Game/Blueprints/Children/Older.Older_C"))
      (Variables|/Game/Blueprints/PlaygroundGameInstance.PlaygroundGameInstance_C|SetPlayer%201%20Vector%203 _asplayground_game_instance (Math|Vector|MakeVector (.X (Math|Vector|BreakVector (Transformation|GetActorLocation (Utilities|Array|Get(acopy) _outactors_2)))) (.Y (Math|Vector|BreakVector (Transformation|GetActorLocation (Utilities|Array|Get(acopy) _outactors_2)))) (+ (.Z (Math|Vector|BreakVector (Transformation|GetActorLocation (Utilities|Array|Get(acopy) _outactors_2)))) 25.0)))
      (Variables|/Game/Blueprints/PlaygroundGameInstance.PlaygroundGameInstance_C|SetPlayer%201%20Boolean _asplayground_game_instance true))
    (:Is%20Not%20Valid
      (Development|PrintString "Hello"))))

(fn InitiateSequence
  (bind _sequencetoplay (Variables|Sequence|GetSequenceToPlay))
  (bind _sequenceplayer (Variables|/Script/LevelSequence.LevelSequenceActor|GetSequencePlayer _sequencetoplay))
  (CallFunction|SetKidReturnLocationsOfGameInstance)
  (Utilities|Time|SetTimerbyFunctionName 0 "SpawnParticleAtTime" (Variables|ParticleSystem|GetDelayBeforeParticleSpawn))
  ;[1 1 1] Move Box Up So it Stops Generating Overlap Events
  (Transformation|AddLocalOffset (Variables|Default|GetBox) "0, 0,1000.000000" false false)
  ;[1 1 1] Disable Player Control and Remove Player 2 (Disable SplitScreen)
  (bind _outactors (Actor|GetAllActorsOfClass "/Game/Blueprints/Children/Younger.Younger_C"))
  (bind _outactors_2 (Actor|GetAllActorsOfClass "/Game/Blueprints/Children/Older.Older_C"))
  (Rendering|SetVisibility (Variables|/Script/Engine.Character|GetMesh (Utilities|Array|Get(acopy) _outactors)) false false)
  (Variables|/Script/PlaygroundHeroes.JKid|Setinteracting (Utilities|Array|Get(acopy) _outactors) false)
  (Variables|/Script/PlaygroundHeroes.JKid|Setinteracting (Utilities|Array|Get(acopy) _outactors_2) false)
  (Input|DisableInput (Utilities|Array|Get(acopy) _outactors) (Game|GetPlayerController 0))
  (Variables|Default|SetYoungerTransform (Transformation|GetActorTransform (Utilities|Array|Get(acopy) _outactors)))
  (Variables|Default|SetOlderTransform (Transformation|GetActorTransform (Utilities|Array|Get(acopy) _outactors_2)))
  (Class|GameplayStatics|RemovePlayer (Game|GetPlayerController 1) true)
  (Game|Player|SetViewTargetwithBlend (Game|GetPlayerController 0) (Variables|Sequence|GetSequenceCamera) 0.0 "VTBlend_Linear" 0.0 false)
  (Sequencer|Player|Play _sequenceplayer :!class /Script/MovieScene.MovieSceneSequencePlayer)
  (Development|PrintString "Hello")
  (PlayDialogs|PlayDialog1)
  (EventDispatchers|BindEventtoOnFinished _sequenceplayer (EventDispatchers|CreateEvent :!event AfterEndSequence)))

(fn OnlyOneNeeded
  (params (Kid :type J%20Kid%20Object%20Reference))
  (bind _array (Utilities|Array|MakeArray ""))
  (bind _array_2 (Utilities|Array|MakeArray 0.0 0.0))
  (bind _array_3 (Utilities|Array|MakeArray 1 2))
  ;[1 1 1] Is the one actor the Younger?
  (Utilities|Casting|CastToYounger Kid
    (:then
      ;[1 1 1] Is the Archer present pressing A?
      (if (Variables|/Script/PlaygroundHeroes.JKid|Getinteracting Kid)
        (SequenceRelated|InitiateSequence :!label _label)
        (else
          ;[1 1 1] Don't show prompt when sequence is playing
          (if (Audio|Components|Audio|IsPlaying (Variables|/Script/LevelSequence.LevelSequenceActor|GetSequencePlayer (Variables|Sequence|GetSequenceToPlay)))
            ;[1 1 1] Blank
            (CallFunction|PrintDialog (Utilities|Array|MakeArray "") _array_2 _array_3 _array false false)
            (else
              (CallFunction|PrintDialog (Utilities|Array|MakeArray (Utilities|String|Append "Hold A to inspect to " (Variables|Default|GetObjectNameDisplayed)) "") _array_2 _array_3 _array true true))))))
    (:CastFailed
      ;[1 1 1] Is the Knight presing A?
      (if (Variables|/Script/PlaygroundHeroes.JKid|Getinteracting Kid)
        (goto _label)
        (else
          ;[1 1 1] Don't show prompt when sequence is playing
          (if (not (Audio|Components|Audio|IsPlaying (Variables|/Script/LevelSequence.LevelSequenceActor|GetSequencePlayer (Variables|Sequence|GetSequenceToPlay))))
            (CallFunction|PrintDialog (Utilities|Array|MakeArray "" (Utilities|String|Append "Hold A to inspect to " (Variables|Default|GetObjectNameDisplayed))) (Utilities|Array|MakeArray 0.0 0.0) (Utilities|Array|MakeArray 1 2) (Utilities|Array|MakeArray "") true true)))))))

(fn PlayDialog1
  (Default|Dialog1 (Variables|Default|GetLinesHolder)))

(fn PlayDialog2
  (Default|Dialog2 (Variables|Default|GetLinesHolder)))

(fn AfterEndSequence
  (bind _returnvalue (Game|GetPlayerController 0))
  (Variables|Default|SetSequenceAlreadyPlayed true)
  (if (Variables|LevelChange|GetChangeLevel?)
    ;[1 1 1] Load Different Level
    (bind _returnvalue_2 (UserInterface|CreateWidget "/Game/Blueprints/UI/LoadSplash.LoadSplash_C"))
    (UserInterface|Viewport|AddtoViewport _returnvalue_2 0)
    (Game|OpenLevel(byName) (Utilities|String|StringToName (Variables|LevelChange|GetDesiredLevel)))
    (else
      ;[1 1 1] Return Control Back to Player 1
      (bind _outactors (Actor|GetAllActorsOfClass "/Game/Blueprints/Children/Younger.Younger_C"))
      (Input|EnableInput (Utilities|Array|Get(acopy) _outactors) _returnvalue)
      (Rendering|SetVisibility (Variables|/Script/Engine.Character|GetMesh (Utilities|Array|Get(acopy) _outactors)) true false)
      (Game|Player|SetViewTargetwithBlend _returnvalue (Utilities|Array|Get(acopy) _outactors) 0.0 "VTBlend_Linear" 0.0 false)
      ;[1 1 1] Respawn Player 2 and Give Control Back
      (bind _returnvalue_3 (Game|SpawnActorfromClass "/Game/Blueprints/Children/Older.Older_C" (Variables|Default|GetOlderTransform) "Undefined" 0 0))
      (bind _returnvalue_4 (Class|GameplayStatics|CreatePlayer 1))
      (Pawn|Possess _returnvalue_4 _returnvalue_3)
      (Game|Player|SetViewTargetwithBlend _returnvalue_4 _returnvalue_3 0.0 "VTBlend_Linear" 0.0 false)
      ;[1 1 1] Move Overlap Box Back to Base Location
      (Variables|Default|SetcanPlaySequence true)
      (Transformation|AddLocalOffset (Variables|Default|GetBox) "0, 0,-1000.000000" false false))))

(fn CheckforRequiredComponents
  ;[1 1 1] Check if each needed component is valid and outputs a warning if it isn't
  (Utilities|IsValid (Variables|Default|GetDialogHandler)
    (:Is%20Valid
      _)
    (:Is%20Not%20Valid
      (Development|PrintString (Utilities|String|Append (Utilities|GetDisplayName self) ": PlayCutsceneChildren: (WARNING) Invalid Dialog Handler") true true "(R=1.000000,G=0.769224,B=0.000000,A=1.000000)" 5.0)))
  (Utilities|IsValid (Variables|Default|GetLinesHolder)
    (:Is%20Valid
      _)
    (:Is%20Not%20Valid
      (Development|PrintString (Utilities|String|Append (Utilities|GetDisplayName self) ": PlayCutsceneChildren: (WARNING) Invalid Dialog Lines Holder") true true "(R=1.000000,G=0.769224,B=0.000000,A=1.000000)" 5.0)))
  (Utilities|IsValid (Variables|Sequence|GetSequenceToPlay)
    (:Is%20Valid
      _)
    (:Is%20Not%20Valid
      (Development|PrintString (Utilities|String|Append (Utilities|GetDisplayName self) ": PlayCutsceneChildren: (WARNING) Invalid or Undefined Sequence") true true "(R=1.000000,G=0.769224,B=0.000000,A=1.000000)" 5.0)))
  (Utilities|IsValid (Variables|Sequence|GetSequenceCamera)
    (:Is%20Valid
      _)
    (:Is%20Not%20Valid
      (Development|PrintString (Utilities|String|Append (Utilities|GetDisplayName self) ": PlayCutsceneChildren: (WARNING) Invalid or Undefined Camera Actor") true true "(R=1.000000,G=0.769224,B=0.000000,A=1.000000)" 5.0)))
  ;[1 1 1] Determine if all components are Valid
  (Variables|Default|SetComponentsValid (Math|Boolean|ANDBoolean (Utilities|IsValid (Variables|Default|GetDialogHandler)) (Utilities|IsValid (Variables|Default|GetLinesHolder)) (Utilities|IsValid (Variables|Sequence|GetSequenceToPlay)) (Utilities|IsValid (Variables|Sequence|GetSequenceCamera)))))

(fn PrintOutLogsOfBadComponents
  (Utilities|IsValid (Variables|Default|GetDialogHandler)
    (:Is%20Valid
      _)
    (:Is%20Not%20Valid
      (Development|PrintString "---Bad Dialog Handler" true true "(R=1.000000,G=0.000000,B=0.021375,A=1.000000)" 5.0)))
  (Utilities|IsValid (Variables|Default|GetLinesHolder)
    (:Is%20Valid
      _)
    (:Is%20Not%20Valid
      (Development|PrintString "---Bad Lines Holder" true true "(R=1.000000,G=0.000000,B=0.021375,A=1.000000)" 5.0)))
  (Utilities|IsValid (Variables|Sequence|GetSequenceToPlay)
    (:Is%20Valid
      _)
    (:Is%20Not%20Valid
      (Development|PrintString "---Bad Sequence To Play" true true "(R=1.000000,G=0.000000,B=0.021375,A=1.000000)" 5.0)))
  (Utilities|IsValid (Variables|Sequence|GetSequenceCamera)
    (:Is%20Not%20Valid
      (Development|PrintString "---Bad Sequence Camera" true true "(R=1.000000,G=0.000000,B=0.021375,A=1.000000)" 5.0))))

(fn PlayDialog3
  (Default|Dialog3 (Variables|Default|GetLinesHolder)))

(fn PlayDialog4
  (Default|Dialog4 (Variables|Default|GetLinesHolder)))

(fn PlayDialog5
  (Default|Dialog5 (Variables|Default|GetLinesHolder)))

(fn PlayDialog0
  (Default|Dialog0 (Variables|Default|GetLinesHolder)))

(fn SpawnParticleatTime
  (Effects|SpawnEmitteratLocation (Variables|ParticleSystem|GetParticleToSpawn) (Transformation|GetActorLocation)))