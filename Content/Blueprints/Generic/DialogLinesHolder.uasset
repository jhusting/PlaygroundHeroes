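; Actor that holds up to five dialogue sequences plus one-liners and sends their lines, durations, fonts and characters to the scene's DialogueHandler, found at BeginPlay.
; Each DialogN function can derive line durations from voice clip lengths, sets split mode, then starts its voice playback.
; PlayVoiceN chains clips on its own AudioComponent through OnAudioFinished, sharing one VoiceLineNumber index.
; Custom one-liners send text only, as OneLinerVoice is an empty stub.
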(event Custom|OneLinerVoice
  (params (VoiceLines :type Array%20of%20Sound%20Wave%20Object%20References))
  ;[1 1 1] Play Voice Dialog Events
  ;;[1 1 1] Play One Line Of Voice Dialog From One Liner Lines Array
)

(event Custom|PlayVoice2
  (params (VoiceLines :type Array%20of%20Sound%20Wave%20Object%20References))
  (bind _audiocomponent2 (Variables|Default|GetAudioComponent2))
  ;[1 1 1] Play Voice Dialog Events
  ;;[1 1 1] Comment
  ;;[1 1 1] Avoid playing a out of bounds null sound wave. (Don't play arr[len+1])
  (if (>= (Utilities|Array|Length VoiceLines) (Variables|Default|GetVoiceLineNumber))
    ;;[1 1 1] Play Sound At Given Index
    (Audio|Components|Audio|SetSound _audiocomponent2 (Utilities|Array|Get(acopy) VoiceLines (Variables|Default|GetVoiceLineNumber)))
    (Audio|Components|Audio|Play _audiocomponent2 0.0)
    ;;[1 1 1] Play Next Track On Finish
    (EventDispatchers|AssignOnAudioFinished _audiocomponent2 (delegate Custom|PlayNextTrack2))
    (else
      (Variables|Default|SetVoiceLineNumber 0))))

(event Custom|PlayNextTrack2
  (bind _audiocomponent2 (Variables|Default|GetAudioComponent2))
  ;[1 1 1] Play Voice Dialog Events
  ;;[1 1 1] Avoid playing a out of bounds null sound wave. (Don't play arr[len+1])
  (if (>= (Utilities|Array|Length (stale Custom|PlayVoice2 VoiceLines)) (Variables|Default|GetVoiceLineNumber))
    ;;[1 1 1] Move To Next Sound
    (Math|Integer|IncrementInt (Variables|Default|GetVoiceLineNumber)
      (:%20%20
        ;;[1 1 1] Play Sound At Given Index
        (Audio|Components|Audio|SetSound _audiocomponent2 (Utilities|Array|Get(acopy) (stale Custom|PlayVoice2 VoiceLines) (Variables|Default|GetVoiceLineNumber)))
        (Audio|Components|Audio|Play _audiocomponent2 0.0)
        ;;[1 1 1] Play Next Track On Finish
        (EventDispatchers|AssignOnAudioFinished _audiocomponent2 (delegate Custom|PlayNextTrack2))))
    (else
      (Variables|Default|SetVoiceLineNumber 0))))

(event Custom|PlayVoice3
  (params (VoiceLines :type Array%20of%20Sound%20Wave%20Object%20References))
  (bind _audiocomponent3 (Variables|Default|GetAudioComponent3))
  ;[1 1 1] Play Voice Dialog Events
  ;;[1 1 1] Avoid playing a out of bounds null sound wave. (Don't play arr[len+1])
  (if (>= (Utilities|Array|Length VoiceLines) (Variables|Default|GetVoiceLineNumber))
    ;;[1 1 1] Play Sound At Given Index
    (Audio|Components|Audio|SetSound _audiocomponent3 (Utilities|Array|Get(acopy) VoiceLines (Variables|Default|GetVoiceLineNumber)))
    (Audio|Components|Audio|Play _audiocomponent3 0.0)
    ;;[1 1 1] Play Next Track On Finish
    (EventDispatchers|AssignOnAudioFinished _audiocomponent3 (delegate Custom|PlayNextTrack3))
    (else
      (Variables|Default|SetVoiceLineNumber 0))))

(event Custom|PlayNextTrack3
  (bind _audiocomponent3 (Variables|Default|GetAudioComponent3))
  ;[1 1 1] Play Voice Dialog Events
  ;;[1 1 1] Avoid playing a out of bounds null sound wave. (Don't play arr[len+1])
  (if (>= (Utilities|Array|Length (stale Custom|PlayVoice3 VoiceLines)) (Variables|Default|GetVoiceLineNumber))
    ;;[1 1 1] Move To Next Sound
    (Math|Integer|IncrementInt (Variables|Default|GetVoiceLineNumber)
      (:%20%20
        ;;[1 1 1] Play Sound At Given Index
        (Audio|Components|Audio|SetSound _audiocomponent3 (Utilities|Array|Get(acopy) (stale Custom|PlayVoice3 VoiceLines) (Variables|Default|GetVoiceLineNumber)))
        (Audio|Components|Audio|Play _audiocomponent3 0.0)
        ;;[1 1 1] Play Next Track On Finish
        (EventDispatchers|AssignOnAudioFinished _audiocomponent3 (delegate Custom|PlayNextTrack3))))
    (else
      (Variables|Default|SetVoiceLineNumber 0))))

(event Custom|PlayVoice1
  (params (VoiceLines :type Array%20of%20Sound%20Wave%20Object%20References))
  (bind _audiocomponent1 (Variables|Default|GetAudioComponent1))
  ;[1 1 1] Play Voice Dialog Events
  ;;[1 1 1] Avoid playing a out of bounds null sound wave. (Don't play arr[len+1])
  (if (>= (Utilities|Array|Length VoiceLines) (Variables|Default|GetVoiceLineNumber))
    ;;[1 1 1] Play Sound At Given Index
    (Audio|Components|Audio|SetSound _audiocomponent1 (Utilities|Array|Get(acopy) VoiceLines (Variables|Default|GetVoiceLineNumber)))
    (Audio|Components|Audio|Play _audiocomponent1 0.0)
    ;;[1 1 1] Play Next Track On Finish
    (EventDispatchers|AssignOnAudioFinished _audiocomponent1 (delegate Custom|PlayNextTrack1))
    (else
      (Variables|Default|SetVoiceLineNumber 0))))

(event Custom|PlayVoice4
  (params (VoiceLines :type Array%20of%20Sound%20Wave%20Object%20References))
  (bind _audiocomponent4 (Variables|Default|GetAudioComponent4))
  ;[1 1 1] Play Voice Dialog Events
  ;;[1 1 1] Avoid playing a out of bounds null sound wave. (Don't play arr[len+1])
  (if (>= (Utilities|Array|Length VoiceLines) (Variables|Default|GetVoiceLineNumber))
    ;;[1 1 1] Play Sound At Given Index
    (Audio|Components|Audio|SetSound _audiocomponent4 (Utilities|Array|Get(acopy) VoiceLines (Variables|Default|GetVoiceLineNumber)))
    (Audio|Components|Audio|Play _audiocomponent4 0.0)
    ;;[1 1 1] Play Next Track On Finish
    (EventDispatchers|AssignOnAudioFinished _audiocomponent4 (delegate Custom|PlayNextTrack4))
    (else
      (Variables|Default|SetVoiceLineNumber 0))))

(event Custom|PlayNextTrack4
  (bind _audiocomponent4 (Variables|Default|GetAudioComponent4))
  ;[1 1 1] Play Voice Dialog Events
  ;;[1 1 1] Avoid playing a out of bounds null sound wave. (Don't play arr[len+1])
  (if (>= (Utilities|Array|Length (stale Custom|PlayVoice4 VoiceLines)) (Variables|Default|GetVoiceLineNumber))
    ;;[1 1 1] Move To Next Sound
    (Math|Integer|IncrementInt (Variables|Default|GetVoiceLineNumber)
      (:%20%20
        ;;[1 1 1] Play Sound At Given Index
        (Audio|Components|Audio|SetSound _audiocomponent4 (Utilities|Array|Get(acopy) (stale Custom|PlayVoice4 VoiceLines) (Variables|Default|GetVoiceLineNumber)))
        (Audio|Components|Audio|Play _audiocomponent4 0.0)
        ;;[1 1 1] Play Next Track On Finish
        (EventDispatchers|AssignOnAudioFinished _audiocomponent4 (delegate Custom|PlayNextTrack4))))
    (else
      (Variables|Default|SetVoiceLineNumber 0))))

(event Custom|PlayVoice5
  (params (VoiceLines :type Array%20of%20Sound%20Wave%20Object%20References))
  (bind _audiocomponent5 (Variables|Default|GetAudioComponent5))
  ;[1 1 1] Play Voice Dialog Events
  ;;[1 1 1] Avoid playing a out of bounds null sound wave. (Don't play arr[len+1])
  (if (>= (Utilities|Array|Length VoiceLines) (Variables|Default|GetVoiceLineNumber))
    ;;[1 1 1] Play Sound At Given Index
    (Audio|Components|Audio|SetSound _audiocomponent5 (Utilities|Array|Get(acopy) VoiceLines (Variables|Default|GetVoiceLineNumber)))
    (Audio|Components|Audio|Play _audiocomponent5 0.0)
    ;;[1 1 1] Play Next Track On Finish
    (EventDispatchers|AssignOnAudioFinished _audiocomponent5 (delegate Custom|PlayNextTrack5))
    (else
      (Variables|Default|SetVoiceLineNumber 0))))

(event Custom|PlayNextTrack5
  (bind _audiocomponent5 (Variables|Default|GetAudioComponent5))
  ;[1 1 1] Play Voice Dialog Events
  ;;[1 1 1] Avoid playing a out of bounds null sound wave. (Don't play arr[len+1])
  (if (>= (Utilities|Array|Length (stale Custom|PlayVoice5 VoiceLines)) (Variables|Default|GetVoiceLineNumber))
    ;;[1 1 1] Move To Next Sound
    (Math|Integer|IncrementInt (Variables|Default|GetVoiceLineNumber)
      (:%20%20
        ;;[1 1 1] Play Sound At Given Index
        (Audio|Components|Audio|SetSound _audiocomponent5 (Utilities|Array|Get(acopy) (stale Custom|PlayVoice5 VoiceLines) (Variables|Default|GetVoiceLineNumber)))
        (Audio|Components|Audio|Play _audiocomponent5 0.0)
        ;;[1 1 1] Play Next Track On Finish
        (EventDispatchers|AssignOnAudioFinished _audiocomponent5 (delegate Custom|PlayNextTrack5))))
    (else
      (Variables|Default|SetVoiceLineNumber 0))))

(event Custom|PlayNextTrack1
  (bind _audiocomponent1 (Variables|Default|GetAudioComponent1))
  ;[1 1 1] Play Voice Dialog Events
  ;;[1 1 1] Avoid playing a out of bounds null sound wave. (Don't play arr[len+1])
  (if (>= (Utilities|Array|Length (stale Custom|PlayVoice1 VoiceLines)) (Variables|Default|GetVoiceLineNumber))
    ;;[1 1 1] Move To Next Sound
    (Math|Integer|IncrementInt (Variables|Default|GetVoiceLineNumber)
      (:%20%20
        ;;[1 1 1] Play Sound At Given Index
        (Audio|Components|Audio|SetSound _audiocomponent1 (Utilities|Array|Get(acopy) (stale Custom|PlayVoice1 VoiceLines) (Variables|Default|GetVoiceLineNumber)))
        (Audio|Components|Audio|Play _audiocomponent1 0.0)
        ;;[1 1 1] Play Next Track On Finish
        (EventDispatchers|AssignOnAudioFinished _audiocomponent1 (delegate Custom|PlayNextTrack1))))
    (else
      (Variables|Default|SetVoiceLineNumber 0))))

(event EventBeginPlay
  (bind _dialog1durations (Variables|Dialog1|GetDialog1Durations))
  (CallFunction|GetDialogHandlerReference)
  (Utilities|IsValid (Variables|Default|GetDialogueHandler)
    (:Is%20Valid
      _)
    (:Is%20Not%20Valid
      (Development|PrintString "JDialogueHandler missing from scene")))
  (if (Variables|OneLiners|GetOneLinerResizeDurations)
    ;[1 1 1] Set Duration[x] To VoiceLines[x].length
    (for (_ _array_index) (Variables|OneLiners|GetOneLinerDurations)
      (Utilities|Array|SetArrayElem (Variables|OneLiners|GetOneLinerDurations) _array_index (Variables|/Script/Engine.SoundBase|GetDuration (Utilities|Array|Get(acopy) (Variables|OneLiners|GetOneLinerVoiceLines) _array_index)) true))
    (else
      (for (_ _array_index_2) _dialog1durations
        (Utilities|Array|SetArrayElem _dialog1durations _array_index_2 (Variables|/Script/Engine.SoundBase|GetDuration (Utilities|Array|Get(acopy) (Variables|Dialog1|GetDialog1VoiceLines) _array_index_2)))
        (Variables|Default|SetTotalTime (+ (Variables|/Script/Engine.SoundBase|GetDuration (Utilities|Array|Get(acopy) (Variables|Dialog1|GetDialog1VoiceLines) _array_index_2)) (Variables|Default|GetTotalTime)))))))

(event Collision|EventActorBeginOverlap
  (params (OtherActor :type Actor%20Object%20Reference)))

(event EventTick
  (params (DeltaSeconds :type Float%20%28single-precision%29)))

(fn ConstructionScript)

(fn Dialog1
  (bind _dialoguehandler (Variables|Default|GetDialogueHandler))
  (bind _dialog1voicelines (Variables|Dialog1|GetDialog1VoiceLines))
  ;[1 1 1] Set Duration[x] To VoiceLines[x].length
  (if (Variables|Dialog1|GetDialog1ResizeDurations)
    (for (_ _array_index) (Variables|Dialog1|GetDialog1Durations)
      (Utilities|Array|SetArrayElem (Variables|Dialog1|GetDialog1Durations) _array_index (Variables|/Script/Engine.SoundBase|GetDuration (Utilities|Array|Get(acopy) (Variables|Dialog1|GetDialog1VoiceLines) _array_index)) true)))
  (Class|DialogueHandler|ToggleSplitMode _dialoguehandler (Variables|Dialog1|GetDialog1Split))
  (Class|DialogueHandler|SendNewdialogueSequence _dialoguehandler (Variables|Dialog1|GetDialog1Lines) (Variables|Dialog1|GetDialog1Durations) (Variables|Dialog1|GetDialog1Fonts) (Variables|Dialog1|GetDialog1Characters))
  (if (> (Utilities|Array|Length _dialog1voicelines) 0)
    (CallFunction|PlayVoice1 _dialog1voicelines)))

(fn Dialog2
  (bind _dialoguehandler (Variables|Default|GetDialogueHandler))
  (bind _dialog2voicelines (Variables|Dialog2|GetDialog2VoiceLines))
  (if (Variables|Dialog2|GetDialog2ResizeDurations)
    ;[1 1 1] Set Duration[x] To VoiceLines[x].length
    (for (_ _array_index) (Variables|Dialog2|GetDialog2Durations)
      (Utilities|Array|SetArrayElem (Variables|Dialog2|GetDialog2Durations) _array_index (Variables|/Script/Engine.SoundBase|GetDuration (Utilities|Array|Get(acopy) (Variables|Dialog2|GetDialog2VoiceLines) _array_index)) true)))
  (Class|DialogueHandler|ToggleSplitMode _dialoguehandler (Variables|Dialog2|GetDialog2Split))
  (Class|DialogueHandler|SendNewdialogueSequence _dialoguehandler (Variables|Dialog2|GetDialog2Lines) (Variables|Dialog2|GetDialog2Durations) (Variables|Dialog2|GetDialog2Fonts) (Variables|Dialog2|GetDialog2Characters))
  (if (> (Utilities|Array|Length _dialog2voicelines) 0)
    (CallFunction|PlayVoice2 _dialog2voicelines)))

(fn Dialog3
  (bind _dialoguehandler (Variables|Default|GetDialogueHandler))
  (bind _dialog3voicelines (Variables|Dialog3|GetDialog3VoiceLines))
  (if (Variables|Dialog3|GetDialog3ResizeDurations)
    ;[1 1 1] Set Duration[x] To VoiceLines[x].length
    (for (_ _array_index) (Variables|Dialog3|GetDialog3Durations)
      (Utilities|Array|SetArrayElem (Variables|Dialog3|GetDialog3Durations) _array_index (Variables|/Script/Engine.SoundBase|GetDuration (Utilities|Array|Get(acopy) (Variables|Dialog3|GetDialog3VoiceLines) _array_index)) true)))
  (Class|DialogueHandler|ToggleSplitMode _dialoguehandler (Variables|Dialog3|GetDialog3SPlit))
  (Class|DialogueHandler|SendNewdialogueSequence _dialoguehandler (Variables|Dialog3|GetDialog3Lines) (Variables|Dialog3|GetDialog3Durations) (Variables|Dialog3|GetDialog3Fonts) (Variables|Dialog3|GetDialog3Characters))
  (if (> (Utilities|Array|Length _dialog3voicelines) 0)
    (CallFunction|PlayVoice3 _dialog3voicelines)))

(fn Dialog4
  (bind _dialoguehandler (Variables|Default|GetDialogueHandler))
  (bind _dialog4voicelines (Variables|Dialog4|GetDialog4VoiceLines))
  (if (Variables|Dialog4|GetDialog4ResizeDurations)
    ;[1 1 1] Set Duration[x] To VoiceLines[x].length
    (for (_ _array_index) (Variables|Dialog4|GetDialog4Durations)
      (Utilities|Array|SetArrayElem (Variables|Dialog4|GetDialog4Durations) _array_index (Variables|/Script/Engine.SoundBase|GetDuration (Utilities|Array|Get(acopy) (Variables|Dialog4|GetDialog4VoiceLines) _array_index)) true)))
  (Class|DialogueHandler|ToggleSplitMode _dialoguehandler (Variables|Dialog4|GetDialog4Split))
  (Class|DialogueHandler|SendNewdialogueSequence _dialoguehandler (Variables|Dialog4|GetDialog4Lines) (Variables|Dialog4|GetDialog4Durations) (Variables|Dialog4|GetDialog4Fonts) (Variables|Dialog4|GetDialog4Characters))
  (if (> (Utilities|Array|Length _dialog4voicelines) 0)
    (CallFunction|PlayVoice4 _dialog4voicelines)))

(fn Dialog5
  (bind _dialoguehandler (Variables|Default|GetDialogueHandler))
  (bind _dialog5voicelines (Variables|Dialog5|GetDialog5VoiceLines))
  (if (Variables|Dialog5|GetDialog5ResizeDurations)
    ;[1 1 1] Set Duration[x] To VoiceLines[x].length
    (for (_ _array_index) (Variables|Dialog5|GetDialog5Durations)
      (Utilities|Array|SetArrayElem (Variables|Dialog5|GetDialog5Durations) _array_index (Variables|/Script/Engine.SoundBase|GetDuration (Utilities|Array|Get(acopy) (Variables|Dialog5|GetDialog5VoiceLines) _array_index)) true)))
  (Class|DialogueHandler|ToggleSplitMode _dialoguehandler (Variables|Dialog5|GetDialog5Split))
  (Class|DialogueHandler|SendNewdialogueSequence _dialoguehandler (Variables|Dialog5|GetDialog5Lines) (Variables|Dialog5|GetDialog5Durations) (Variables|Dialog5|GetDialog5Fonts) (Variables|Dialog5|GetDialog5Characters))
  (if (> (Utilities|Array|Length _dialog5voicelines) 0)
    (CallFunction|PlayVoice5 _dialog5voicelines)))

(fn GetDialogHandlerReference
  (bind _outactors (Actor|GetAllActorsOfClass "/Script/PlaygroundHeroes.DialogueHandler"))
  (Variables|Default|SetDialogueHandler (Utilities|Array|Get(acopy) _outactors)))

(fn PrintDialog
  (params (Lines :type Array%20of%20Strings) (Duration :type Array%20of%20Floats%20%28single-precision%29) (Fonts :type Array%20of%20Integers) (characters :type Array%20of%20Strings) (Split :type Boolean) (PauseAfter :type Boolean))
  (bind _dialoguehandler (Variables|Default|GetDialogueHandler))
  (Class|DialogueHandler|ToggleSplitMode _dialoguehandler Split)
  (Class|DialogueHandler|SendNewdialogueSequence _dialoguehandler Lines Duration Fonts characters)
  (if PauseAfter
    (Class|DialogueHandler|Pause _dialoguehandler)))

(fn Dialog0)

(fn PlayOneLinerSaved
  (params (IndexOfLineToPlay :type Integer))
  (bind _onelinervoicelines (Variables|OneLiners|GetOneLinerVoiceLines))
  (if (Variables|OneLiners|GetOneLinerResizeDurations)
    ;[1 1 1] Set Duration[x] To VoiceLines[x].length
    (for (_ _array_index) (Variables|OneLiners|GetOneLinerDurations)
      (Utilities|Array|SetArrayElem (Variables|OneLiners|GetOneLinerDurations) _array_index (Variables|/Script/Engine.SoundBase|GetDuration (Utilities|Array|Get(acopy) (Variables|OneLiners|GetOneLinerVoiceLines) _array_index)) true)
      (Class|DialogueHandler|SendNewdialogueSequence (Variables|Default|GetDialogueHandler) (Utilities|Array|MakeArray (Utilities|Array|Get(acopy) (Variables|OneLiners|GetOneLinerLines) IndexOfLineToPlay)) (Variables|OneLiners|GetOneLinerDurations) (Variables|OneLiners|GetOneLinerFonts) (Variables|OneLiners|GetOneLinerCharacters))
      (if (> (Utilities|Array|Length _onelinervoicelines) 0)
        (CallFunction|PlayVoice1 _onelinervoicelines)))
    (else
      (Class|DialogueHandler|SendNewdialogueSequence (Variables|Default|GetDialogueHandler) (Utilities|Array|MakeArray (Utilities|Array|Get(acopy) (Variables|OneLiners|GetOneLinerLines) IndexOfLineToPlay)) (Variables|OneLiners|GetOneLinerDurations) (Variables|OneLiners|GetOneLinerFonts) (Variables|OneLiners|GetOneLinerCharacters))
      (if (> (Utilities|Array|Length _onelinervoicelines) 0)
        (CallFunction|PlayVoice1 _onelinervoicelines)))))

(fn PlayOneLinerCustomText
  (params (Line :type String) (Duration :type Float%20%28single-precision%29) (Font :type Integer) (Character :type String) (VoiceLine :type Sound%20Wave%20Object%20Reference))
  (bind _array (Utilities|Array|MakeArray VoiceLine))
  (Class|DialogueHandler|SendNewdialogueSequence (Variables|Default|GetDialogueHandler) (Utilities|Array|MakeArray Line) (Utilities|Array|MakeArray Duration) (Utilities|Array|MakeArray Font) (Utilities|Array|MakeArray Character))
  (if (> (Utilities|Array|Length _array) 0)
    (CallFunction|OneLinerVoice _array)))