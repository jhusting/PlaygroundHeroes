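; Cutscene actor that plays a level sequence with dialog after a start delay on BeginPlay, for either kid or warrior maps.
; It validates its references, disables player 1, removes player 2 to end split-screen and switches to the sequence camera.
; It triggers the numbered dialog on LinesHolder through a timer using a built function name.
; Its end routine restores player 1 and respawns player 2 at the saved transform.
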(event EventBeginPlay
  (Utilities|FlowControl|Delay (Variables|Default|GetStartDelay))
  (bind _outactors (Actor|GetAllActorsOfClass "/Script/PlaygroundHeroes.DialogueHandler"))
  (Variables|Dialog|SetDialogHandler (Utilities|Array|Get(acopy) _outactors))
  (CallFunction|CheckforRequiredComponents)
  ;[1 1 1] If Not All Needed Components Are Valid, Print An Error
  (if (Variables|Default|GetComponentsValid)
    (CallFunction|InitiateSequence)
    (else
      (CallFunction|PrintOutLogsOfBadComponents)
      (Development|PrintString (Utilities|String|Append (Utilities|GetDisplayName self) ": PlayCutsceneChildren: (ERROR) Cannot Play Sequence: Not All Needed Components are Defined/Valid. ") true true "(R=0.812500,G=0.000000,B=0.115263,A=1.000000)" 5.0))))

(fn ConstructionScript)

(fn PrintDialog
  (params (Lines :type Array%20of%20Strings) (Durations :type Array%20of%20Floats%20%28single-precision%29) (FOnts :type Array%20of%20Integers) (characters :type Array%20of%20Strings) (Split :type Boolean) (PauseAfter :type Boolean))
  (bind _dialoghandler (Variables|Dialog|GetDialogHandler))
  (Class|DialogueHandler|ToggleSplitMode _dialoghandler Split)
  (Class|DialogueHandler|SendNewdialogueSequence _dialoghandler Lines Durations FOnts characters)
  (if PauseAfter
    (Class|DialogueHandler|Pause _dialoghandler)))

(fn SetKidLocations
  (bind _asplayground_game_instance (Utilities|Casting|CastToPlaygroundGameInstance (Game|GetGameInstance)))
  (bind _outactors (Actor|GetAllActorsOfClass "/Game/Blueprints/Children/Younger.Younger_C"))
  (Variables|/Game/Blueprints/PlaygroundGameInstance.PlaygroundGameInstance_C|SetPlayer%200%20Vector%203 _asplayground_game_instance (Math|Vector|MakeVector (.X (Math|Vector|BreakVector (Transformation|GetActorLocation (Utilities|Array|Get(acopy) _outactors)))) (.Y (Math|Vector|BreakVector (Transformation|GetActorLocation (Utilities|Array|Get(acopy) _outactors)))) (+ (.Z (Math|Vector|BreakVector (Transformation|GetActorLocation (Utilities|Array|Get(acopy) _outactors)))) 25.0)))
  (Variables|/Game/Blueprints/PlaygroundGameInstance.PlaygroundGameInstance_C|SetPlayer%200%20Boolean _asplayground_game_instance true)
  (bind _outactors_2 (Actor|GetAllActorsOfClass "/Game/Blueprints/Children/Older.Older_C"))
  (Variables|/Game/Blueprints/PlaygroundGameInstance.PlaygroundGameInstance_C|SetPlayer%201%20Vector%203 _asplayground_game_instance (Math|Vector|MakeVector (.X (Math|Vector|BreakVector (Transformation|GetActorLocation (Utilities|Array|Get(acopy) _outactors_2)))) (.Y (Math|Vector|BreakVector (Transformation|GetActorLocation (Utilities|Array|Get(acopy) _outactors_2)))) (+ (.Z (Math|Vector|BreakVector (Transformation|GetActorLocation (Utilities|Array|Get(acopy) _outactors_2)))) 25.0)))
  (Variables|/Game/Blueprints/PlaygroundGameInstance.PlaygroundGameInstance_C|SetPlayer%201%20Boolean _asplayground_game_instance true))

(fn InitiateSequence
  (bind _sequencetoplay (Variables|Sequence|GetSequenceToPlay))
  (bind _sequenceplayer (Variables|/Script/LevelSequence.LevelSequenceActor|GetSequencePlayer _sequencetoplay))
  ;[1 1 1] Does this map have warriors or children?
  (bind _outactors (Actor|GetAllActorsOfClass "/Game/Blueprints/Children/Younger.Younger_C"))
  (if (== (Utilities|Array|Length _outactors) 0)
    ;[1 1 1] WARRIORS: Disable Player Control and Remove Player 2 (Disable SplitScreen)
    (bind _outactors_2 (Actor|GetAllActorsOfClass "/Game/Blueprints/Warriors/JArcherBP.JArcherBP_C"))
    (bind _outactors_3 (Actor|GetAllActorsOfClass "/Game/Blueprints/Warriors/JKnightBP.JKnightBP_C"))
    (Rendering|SetVisibility (Variables|/Script/Engine.Character|GetMesh (Utilities|Array|Get(acopy) _outactors_2)) false false)
    (Rendering|SetVisibility (Variables|/Game/Blueprints/Warriors/JArcherBP.JArcherBP_C|GetBow (Utilities|Array|Get(acopy) _outactors_2)) false false)
    (Input|DisableInput (Utilities|Array|Get(acopy) _outactors_2) (Game|GetPlayerController 0))
    (Variables|Default|SetYounger+ArcherTransform (Transformation|GetActorTransform (Utilities|Array|Get(acopy) _outactors_2)))
    (Variables|Default|SetOlder+KnightTransform (Transformation|GetActorTransform (Utilities|Array|Get(acopy) _outactors_3)))
    (Class|GameplayStatics|RemovePlayer (Game|GetPlayerController 1) true)
    (else
      ;[1 1 1] KIDS: Disable Player Control and Remove Player 2 (Disable SplitScreen)
      (bind _outactors_4 (Actor|GetAllActorsOfClass "/Game/Blueprints/Children/Younger.Younger_C"))
      (bind _outactors_5 (Actor|GetAllActorsOfClass "/Game/Blueprints/Children/Older.Older_C"))
      (Rendering|SetVisibility (Variables|/Script/Engine.Character|GetMesh (Utilities|Array|Get(acopy) _outactors_4)) false false)
      (Input|DisableInput (Utilities|Array|Get(acopy) _outactors_4) (Game|GetPlayerController 0))
      (Variables|Default|SetYounger+ArcherTransform (Transformation|GetActorTransform (Utilities|Array|Get(acopy) _outactors_4)))
      (Variables|Default|SetOlder+KnightTransform (Transformation|GetActorTransform (Utilities|Array|Get(acopy) _outactors_5)))
      (Class|GameplayStatics|RemovePlayer (Game|GetPlayerController 1) true)))
  (Game|Player|SetViewTargetwithBlend (Game|GetPlayerController 0) (Variables|Sequence|GetSequenceCamera) 0.0 "VTBlend_Linear" 0.0 false)
  (Sequencer|Player|Play _sequenceplayer :!class /Script/MovieScene.MovieSceneSequencePlayer)
  ;[1 1 1] Call PlayDialog# Function During Sequencer
  (Utilities|Time|SetTimerbyFunctionName (Variables|Dialog|GetLinesHolder) (Utilities|String|Append (Utilities|String|MakeLiteralString "Dialog ") (Utilities|String|ToString(Integer) (Variables|Dialog|GetDialogNumberToPlay))) 0.0)
  (EventDispatchers|BindEventtoOnFinished _sequenceplayer (EventDispatchers|CreateEvent :!event EndSequenceandRetoreControl)))

(fn PlayDialog1
  (Default|Dialog1 (Variables|Dialog|GetLinesHolder)))

(fn PlayDialog2
  (Default|Dialog2 (Variables|Dialog|GetLinesHolder)))

(fn EndSequenceandRetoreControl
  (bind _returnvalue (Game|GetPlayerController 0))
  (bind _returnvalue_2 (Game|GetPlayerController 0))
  ;[1 1 1] Does this map have warriors or children?
  (bind _outactors (Actor|GetAllActorsOfClass "/Game/Blueprints/Children/Younger.Younger_C"))
  (if (== (Utilities|Array|Length _outactors) 0)
    ;[1 1 1] WARRIORS: Return Control Back to Player 1
    (bind _outactors_2 (Actor|GetAllActorsOfClass "/Game/Blueprints/Warriors/JArcherBP.JArcherBP_C"))
    (Input|EnableInput (Utilities|Array|Get(acopy) _outactors_2) _returnvalue)
    (Rendering|SetVisibility (Variables|/Game/Blueprints/Warriors/JArcherBP.JArcherBP_C|GetBow (Utilities|Array|Get(acopy) _outactors_2)) true true)
    (Rendering|SetVisibility (Variables|/Script/Engine.Character|GetMesh (Utilities|Array|Get(acopy) _outactors_2)) true true)
    (Game|Player|SetViewTargetwithBlend _returnvalue (Utilities|Array|Get(acopy) _outactors_2) 0.0 "VTBlend_Linear" 0.0 false)
    ;[1 1 1] Respawn Player 2 and Give Control Back
    (bind _returnvalue_3 (Game|SpawnActorfromClass "/Game/Blueprints/Warriors/JKnightBP.JKnightBP_C" (Variables|Default|GetOlder+KnightTransform) "Undefined" 0 0))
    (bind _returnvalue_4 (Class|GameplayStatics|CreatePlayer 1))
    (Pawn|Possess _returnvalue_4 _returnvalue_3)
    (Game|Player|SetViewTargetwithBlend _returnvalue_4 _returnvalue_3 0.0 "VTBlend_Linear" 0.0 false)
    (else
      ;[1 1 1] KIDS: Return Control Back to Player 1
      (bind _outactors_3 (Actor|GetAllActorsOfClass "/Game/Blueprints/Children/Younger.Younger_C"))
      (Input|EnableInput (Utilities|Array|Get(acopy) _outactors_3) _returnvalue_2)
      (Game|Player|SetViewTargetwithBlend _returnvalue_2 (Utilities|Array|Get(acopy) _outactors_3) 0.0 "VTBlend_Linear" 0.0 false)
      ;[1 1 1] Respawn Player 2 and Give Control Back
      (bind _returnvalue_5 (Game|SpawnActorfromClass "/Game/Blueprints/Children/Older.Older_C" (Variables|Default|GetOlder+KnightTransform) "Undefined" 0 0))
      (bind _returnvalue_6 (Class|GameplayStatics|CreatePlayer 1))
      (Pawn|Possess _returnvalue_6 _returnvalue_5)
      (Game|Player|SetViewTargetwithBlend _returnvalue_6 _returnvalue_5 0.0 "VTBlend_Linear" 0.0 false))))

(fn CheckforRequiredComponents
  ;[1 1 1] Check if each needed component is valid and outputs a warning if it isn't
  (Utilities|IsValid (Variables|Dialog|GetDialogHandler)
    (:Is%20Valid
      _)
    (:Is%20Not%20Valid
      (Development|PrintString (Utilities|String|Append (Utilities|GetDisplayName self) ": PlayCutsceneChildren: (WARNING) Invalid Dialog Handler") true true "(R=1.000000,G=0.769224,B=0.000000,A=1.000000)" 5.0)))
  (Utilities|IsValid (Variables|Dialog|GetLinesHolder)
    (:Is%20Valid
      _)
    (:Is%20Not%20Valid
      (Development|PrintString (Utilities|String|Append (Utilities|GetDisplayName self) ": PlayCutsceneChildren: (WARNING) Invalid Dialog Lines Holder") true true "(R=1.000000,G=0.769224,B=0.000000,A=1.000000)" 5.0)))
  (Utilities|IsValid (Variables|Sequence|GetSequenceToPlay)
    (:Is%20Valid
      _)
    (:Is%20Not%20Valid
      (Development|PrintString (Utilities|String|Append (Utilities|GetDisplayName self) ": PlayCutsceneChildren: (WARNING) Invalid or Undefined Sequence") true true "(R=1.000000,G=0.769224,B=0.000000,A=1.000000)" 5.0)))
  (Utilities|IsValid (Variables|Sequence|GetSequenceCamera)
    (:Is%20Valid
      _)
    (:Is%20Not%20Valid
      (Development|PrintString (Utilities|String|Append (Utilities|GetDisplayName self) ": PlayCutsceneChildren: (WARNING) Invalid or Undefined Camera Actor") true true "(R=1.000000,G=0.769224,B=0.000000,A=1.000000)" 5.0)))
  ;[1 1 1] Determine if all components are Valid
  (Variables|Default|SetComponentsValid (Math|Boolean|ANDBoolean (Utilities|IsValid (Variables|Dialog|GetDialogHandler)) (Utilities|IsValid (Variables|Dialog|GetLinesHolder)) (Utilities|IsValid (Variables|Sequence|GetSequenceToPlay)) (Utilities|IsValid (Variables|Sequence|GetSequenceCamera)))))

(fn PrintOutLogsOfBadComponents
  (Utilities|IsValid (Variables|Dialog|GetDialogHandler)
    (:Is%20Valid
      _)
    (:Is%20Not%20Valid
      (Development|PrintString "---Bad Dialog Handler" true true "(R=1.000000,G=0.000000,B=0.021375,A=1.000000)" 5.0)))
  (Utilities|IsValid (Variables|Dialog|GetLinesHolder)
    (:Is%20Valid
      _)
    (:Is%20Not%20Valid
      (Development|PrintString "---Bad Lines Holder" true true "(R=1.000000,G=0.000000,B=0.021375,A=1.000000)" 5.0)))
  (Utilities|IsValid (Variables|Sequence|GetSequenceToPlay)
    (:Is%20Valid
      _)
    (:Is%20Not%20Valid
      (Development|PrintString "---Bad Sequence To Play" true true "(R=1.000000,G=0.000000,B=0.021375,A=1.000000)" 5.0)))
  (Utilities|IsValid (Variables|Sequence|GetSequenceCamera)
    (:Is%20Not%20Valid
      (Development|PrintString "---Bad Sequence Camera" true true "(R=1.000000,G=0.000000,B=0.021375,A=1.000000)" 5.0))))

(fn PlayDialog0
  (Default|Dialog0 (Variables|Dialog|GetLinesHolder)))

(fn PlayDialog4
  (Default|Dialog4 (Variables|Dialog|GetLinesHolder)))

(fn PlayDialog5
  (Default|Dialog5 (Variables|Dialog|GetLinesHolder)))

(fn PlayDialog3
  (Default|Dialog3 (Variables|Dialog|GetLinesHolder)))