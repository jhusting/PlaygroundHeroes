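; Level-change trigger with a spinning visual that opens LevelToGoTo when heroes inside hold Interacting.
; Tick accepts any overlapping hero if OnlyOneCharacterNeeded; otherwise both box-tracked Warriors must be ready together.
; In two-player mode, the level's DialogueHandler shows ready-up prompts, split for Archer and Knight.
; The first hero entering saves the current dialogue; the last leaving clears the prompt and restores it.
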(event OnComponentBeginOverlap(Box)
  (params (OverlappedComponent :type Primitive%20Component%20Object%20Reference) (OtherActor :type Actor%20Object%20Reference) (OtherComp :type Primitive%20Component%20Object%20Reference) (OtherBodyIndex :type Integer) (bFromSweep :type Boolean) (SweepResult :type Hit%20Result%20Structure%20%28by%20ref%29))
  (bind _warriors (Variables|Default|GetWarriors))
  (bind _asjhero (Utilities|Casting|CastToJHero OtherActor))
  (Utilities|Array|AddUnique _warriors _asjhero)
  (if (== (Utilities|Array|Length _warriors) 1) ; if first player entered
    (Class|DialogueHandler|SaveDialogue (Variables|Default|GetDialogHandler))))

(event OnComponentEndOverlap(Box)
  (params (OverlappedComponent :type Primitive%20Component%20Object%20Reference) (OtherActor :type Actor%20Object%20Reference) (OtherComp :type Primitive%20Component%20Object%20Reference) (OtherBodyIndex :type Integer))
  (bind _warriors (Variables|Default|GetWarriors))
  (bind _asjhero (Utilities|Casting|CastToJHero OtherActor))
  (Utilities|Array|RemoveItem _warriors _asjhero)
  (if (== (Utilities|Array|Length _warriors) 0)
    ;[1 1 1] If last person inside left, clear out text
    (CallFunction|PrintDialog (Utilities|Array|MakeArray (Utilities|String|MakeLiteralString)) (Utilities|Array|MakeArray 0.0) (Utilities|Array|MakeArray 1) false true)
    (Class|DialogueHandler|LoadSavedDialogue (Variables|Default|GetDialogHandler))))

(event EventBeginPlay
  (bind _outactors (Actor|GetAllActorsOfClass "/Script/PlaygroundHeroes.DialogueHandler"))
  (Variables|Default|SetDialogHandler (Utilities|Array|Get(acopy) _outactors)))

(event Collision|EventActorBeginOverlap
  (params (OtherActor :type Actor%20Object%20Reference)))

(event EventTick
  (params (DeltaSeconds :type Float%20%28single-precision%29))
  (bind _warriors (Variables|Default|GetWarriors))
  (bind _returnvalue (Utilities|Array|Length _warriors))
  (CallFunction|RotateVisual)
  (if (Variables|Default|GetOnlyOneCharacterNeeded)
    ;[1 1 1] If Either Presses 'A' Button and OnlyOneCharacterNeeded is TRUE
    (for _array_element (Collision|GetOverlappingActors "/Script/PlaygroundHeroes.JHero" :!class /Script/Engine.Actor)
      (bind _asjhero (Utilities|Casting|CastToJHero _array_element))
      (if (Variables|/Script/PlaygroundHeroes.JHero|Getinteracting _asjhero)
        (Game|OpenLevel(byName) (Variables|Default|GetLevelToGoTo))))
    (elif (== _returnvalue 2)
      (CallFunction|BothPresent)
      (elif (== _returnvalue 1)
        (CallFunction|OnlyOnePresent)))))

(fn ConstructionScript)

(fn PrintDialog
  (params (Lines :type Array%20of%20Strings) (Durations :type Array%20of%20Floats%20%28single-precision%29) (FOnts :type Array%20of%20Integers) (Split :type Boolean) (PauseAfter :type Boolean))
  (bind _dialoghandler (Variables|Default|GetDialogHandler))
  (Class|DialogueHandler|ToggleSplitMode _dialoghandler Split)
  (Class|DialogueHandler|SendNewdialogueSequence _dialoghandler Lines Durations FOnts)
  (if PauseAfter
    (Class|DialogueHandler|Pause _dialoghandler)))

(fn BothPresent
  (bind _warriors (Variables|Default|GetWarriors))
  (bind _temparray (Variables|Default|GetTempArray))
  (bind _output (Utilities|Array|Get(acopy) _warriors))
  (bind _output_2 (Utilities|Array|Get(acopy) _warriors 1))
  (bind _interacting (Variables|/Script/PlaygroundHeroes.JHero|Getinteracting _output))
  (bind _interacting_2 (Variables|/Script/PlaygroundHeroes.JHero|Getinteracting _output_2))
  ;[1 1 1] We want our array to be ordered Archer, Knight
  ;;[1 1 1] If the array order is Archer, Knight
  (bind _asjarcher (Utilities|Casting|CastToJArcher _output)
    (:then
      (Utilities|Array|AddUnique _temparray _asjarcher)
      (bind _asjknight (Utilities|Casting|CastToJKnight _output_2))
      (Utilities|Array|AddUnique _temparray _asjknight))
    (:CastFailed
      ;;[1 1 1] If array order is Knight, Archer
      (bind _asjarcher_2 (Utilities|Casting|CastToJArcher _output_2))
      (Utilities|Array|AddUnique (Variables|Default|GetTempArray) _asjarcher_2)
      (Utilities|Casting|CastToJKnight _output)))
  ;[1 1 1] Both pressing A
  (if (and _interacting _interacting_2)
    (Game|OpenLevel(byName) (Variables|Default|GetLevelToGoTo))
    (else
      ;[1 1 1] A pressing A, B in
      (if (and (not _interacting) _interacting_2)
        (CallFunction|PrintDialog (Utilities|Array|MakeArray "Readied" (Utilities|String|Append "Press A to move to " (Utilities|String|ToString(Name) (Variables|Default|GetLevelToGoTo)))) (Utilities|Array|MakeArray 0.0 0.0) (Utilities|Array|MakeArray 1 2) true true)
        (else
          ;[1 1 1] A In, B pressing A
          (if (and _interacting (not _interacting_2))
            (CallFunction|PrintDialog (Utilities|Array|MakeArray (Utilities|String|Append "Press A to move to " (Utilities|String|ToString(Name) (Variables|Default|GetLevelToGoTo))) "Readied") (Utilities|Array|MakeArray 0.0 0.0) (Utilities|Array|MakeArray 1 2) true true)
            (else
              ;[1 1 1] Neither is pressing A
              (CallFunction|PrintDialog (Utilities|Array|MakeArray "Press A to Ready Up" "") (Utilities|Array|MakeArray 0.0 0.0) (Utilities|Array|MakeArray 1 1) false true))))))))

(fn OnlyOnePresent
  (bind _warriors (Variables|Default|GetWarriors))
  (bind _output (Utilities|Array|Get(acopy) _warriors))
  ;[1 1 1] Is the one actor an archer?
  (Utilities|Casting|CastToJArcher _output
    (:then
      ;[1 1 1] Is the Archer present pressing A?
      (if (Variables|/Script/PlaygroundHeroes.JHero|Getinteracting _output)
        (CallFunction|PrintDialog (Utilities|Array|MakeArray "Readied" (Utilities|String|Append "Abigail: Come over here, lets go to " (Utilities|String|ToString(Name) (Variables|Default|GetLevelToGoTo)))) (Utilities|Array|MakeArray 0.0 0.0) (Utilities|Array|MakeArray 1 2) true true)
        (else
          (CallFunction|PrintDialog (Utilities|Array|MakeArray "Press A to ready" "") (Utilities|Array|MakeArray 0.0 0.0) (Utilities|Array|MakeArray 1 1) true true))))
    (:CastFailed
      ;[1 1 1] Is the Knight presing A?
      (if (Variables|/Script/PlaygroundHeroes.JHero|Getinteracting _output)
        (CallFunction|PrintDialog (Utilities|Array|MakeArray (Utilities|String|Append "Leila: Come over here, lets go to " (Utilities|String|ToString(Name) (Variables|Default|GetLevelToGoTo))) "Readied") (Utilities|Array|MakeArray 0.0 0.0) (Utilities|Array|MakeArray 1 2) true true)
        (else
          (CallFunction|PrintDialog (Utilities|Array|MakeArray "" "Press A to ready") (Utilities|Array|MakeArray 0.0 0.0) (Utilities|Array|MakeArray 1 2) true true))))))

(fn RotateVisual
  (bind _visual (Variables|Default|GetVisual))
  (bind _returnvalue (Transformation|GetWorldRotation _visual))
  (bind (_roll _pitch _yaw) (Math|Rotator|BreakRotator _returnvalue))
  (Transformation|SetWorldRotation _visual (Math|Rotator|MakeRotator _roll _pitch (+ _yaw 1.0)) false false))