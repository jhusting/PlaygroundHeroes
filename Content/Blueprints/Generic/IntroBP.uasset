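; IntroBP is a level actor that stages the intro by suspending normal two-player split-screen play.
; On BeginPlay it finds the Younger and Older actors, hides Younger's mesh and clears the Interacting flag on both.
; It then disables Younger's input, removes player two with its pawn to drop split-screen, and blends player one's view to its Camera.
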(event EventBeginPlay
  ;[1 1 1] Disable Player Control and Remove Player 2 (Disable SplitScreen)
  (bind _outactors (Actor|GetAllActorsOfClass "/Game/Blueprints/Children/Younger.Younger_C"))
  (bind _outactors_2 (Actor|GetAllActorsOfClass "/Game/Blueprints/Children/Older.Older_C"))
  (Rendering|SetVisibility (Variables|/Script/Engine.Character|GetMesh (Utilities|Array|Get(acopy) _outactors)) false false)
  (Variables|/Script/PlaygroundHeroes.JKid|Setinteracting (Utilities|Array|Get(acopy) _outactors) false)
  (Variables|/Script/PlaygroundHeroes.JKid|Setinteracting (Utilities|Array|Get(acopy) _outactors_2) false)
  (Input|DisableInput (Utilities|Array|Get(acopy) _outactors) (Game|GetPlayerController 0))
  (Class|GameplayStatics|RemovePlayer (Game|GetPlayerController 1) true)
  (Game|Player|SetViewTargetwithBlend (Game|GetPlayerController 0) (Variables|Default|GetCamera) 0.0 "VTBlend_Linear" 0.0 false))

(event Collision|EventActorBeginOverlap
  (params (OtherActor :type Actor%20Object%20Reference)))

(event EventTick
  (params (DeltaSeconds :type Float%20%28single-precision%29)))

(fn ConstructionScript)