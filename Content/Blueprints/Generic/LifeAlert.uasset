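; LifeAlert is the downed-player actor for two-player co-op, handling revival of its owning fallen JHero.
; It hides the hero, possesses an immobilized child stand-in (Younger or Older) and follows it, prompting through DialogueHandler outside tutorials.
; An overlapping partner holding Interact fills the ReviveBar, which drains twice as fast on release; completion restores and revives the hero.
; A second simultaneous LifeAlert triggers a restart prompt or previous-level return.
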(event EventBeginPlay
  (CallFunction|TransformtoChildren)
  (bind _outactors (Actor|GetAllActorsOfClass "LifeAlert_C"))
  (if (== (Utilities|Array|Length _outactors) 2) ; If there is already a life alert, then both are dead
    (if (Variables|Default|GetGivenChanceToRestartInLevel)
      (CallFunction|SpawnDeathPromptwithRestartOption)
      (else
        (CallFunction|ReturnBacktoPreviousLevel)))
    (else
      (bind _returnvalue (UserInterface|CreateWidget "/Game/Blueprints/UI/ReviveProgress.ReviveProgress_C" (Game|GetPlayerController 0) (Variables|Default|GetfallenPlayerIndex)))
      (bind _output_get (Variables|Default|SetreviveBar _returnvalue))
      (UserInterface|Viewport|AddtoViewport _output_get 0)
      (Widget|SetRenderOpacity _output_get 0.0)
      (for _array_element (Collision|GetOverlappingActors "/Script/PlaygroundHeroes.JHero" :!class /Script/Engine.Actor) ; Make sure they aren't already next to each other
        (bind _asjhero (Utilities|Casting|CastToJHero _array_element))
        (Utilities|Array|AddUnique (Variables|Default|GetWarriors) _asjhero))
      (Utilities|FlowControl|Delay 0.2)
      (if (== (Utilities|Array|Length (Variables|Default|GetWarriors)) 2)
        (CallFunction|SendRevivePrompt)
        (else
          (CallFunction|SendforHelp))))))

(event Collision|EventActorBeginOverlap
  (params (OtherActor :type Actor%20Object%20Reference))
  (bind _asjhero (Utilities|Casting|CastToJHero OtherActor))
  (bind _returnvalue (Utilities|Array|AddUnique (Variables|Default|GetWarriors) _asjhero))
  (if (!= _returnvalue -1)
    (CallFunction|SendRevivePrompt)))

(event EventTick
  (params (DeltaSeconds :type Float%20%28single-precision%29))
  (bind _revivebar (Variables|Default|GetreviveBar))
  (bind _warriors (Variables|Default|GetWarriors))
  (bind _revivebar_2 (Variables|Default|GetreviveBar))
  (CallFunction|UpdatePosition)
  (if (== (Utilities|Array|Length _warriors) 2) ; If both are in range
    (if (Variables|/Script/PlaygroundHeroes.JHero|Getinteracting (Utilities|Array|Get(acopy) _warriors 1)) ; If other player is holding A increase progress, else decrease
      ;[1 1 1] Increase Revival Progress Bar
      (Variables|Default|SetprogressCount (+ DeltaSeconds (Variables|Default|GetprogressCount)))
      (Utilities|IsValid _revivebar
        (:Is%20Valid
          (Widget|SetRenderOpacity _revivebar 1.0)
          (Variables|/Game/Blueprints/UI/ReviveProgress.ReviveProgress_C|Setpercentage _revivebar (/ (Variables|Default|GetprogressCount) (Variables|Default|GetreviveTime)))
          ;[1 1 1] Revive Fallen Player
          (if (>= (Variables|Default|GetprogressCount) (Variables|Default|GetreviveTime))
            (Class|DialogueHandler|Clear (Variables|Default|GetDialogueHandler))
            (CallFunction|TransformtoHeroes)
            (Class|JHero|Revive (Utilities|Array|Get(acopy) (Variables|Default|GetWarriors))))))
      (else
        ;[1 1 1] descrese Progress if not reviving
        (Variables|Default|SetprogressCount (Math|Float|Clamp(Float) (- (Variables|Default|GetprogressCount) (* DeltaSeconds 2.0)) 0.0 (Variables|Default|GetreviveTime)))
        (Utilities|IsValid _revivebar_2
          (:Is%20Valid
            (Variables|/Game/Blueprints/UI/ReviveProgress.ReviveProgress_C|Setpercentage _revivebar_2 (/ (Variables|Default|GetprogressCount) (Variables|Default|GetreviveTime)))
            (if (== (Variables|Default|GetprogressCount) 0.0)
              (Widget|SetRenderOpacity _revivebar_2 0.0))))))))

(event Collision|EventActorEndOverlap
  (params (OtherActor :type Actor%20Object%20Reference))
  (bind _revivebar (Variables|Default|GetreviveBar))
  (bind _asjhero (Utilities|Casting|CastToJHero OtherActor))
  (Utilities|Array|RemoveItem (Variables|Default|GetWarriors) _asjhero)
  (Variables|Default|SetprogressCount 0.0)
  (Utilities|IsValid _revivebar
    (:Is%20Valid
      (Widget|SetRenderOpacity _revivebar 0.0)
      (Class|DialogueHandler|Clear (Variables|Default|GetDialogueHandler)))))

(fn ConstructionScript
  (bind _warriors (Variables|Default|GetWarriors))
  (bind _outactors (Actor|GetAllActorsOfClass "/Game/Blueprints/UI/JDialogueHandler.JDialogueHandler_C"))
  (Variables|Default|SetDialogueHandler (Utilities|Array|Get(acopy) _outactors))
  (Variables|Default|SetprogressCount 0.0)
  ;[1 1 1] Get reference to Jhero that died, and get which player it was. Warrior 0 will always be fallen player
  (bind _asjhero (Utilities|Casting|CastToJHero (Components|GetOwner)))
  (Variables|Default|SetfallenController (Pawn|GetController _asjhero))
  (bind _asjarcher (Utilities|Casting|CastToJArcher _asjhero)
    (:then
      (Utilities|Array|AddUnique _warriors _asjarcher)
      (Variables|Default|SetfallenPlayerIndex 0))
    (:CastFailed
      (Utilities|Array|AddUnique _warriors _asjhero)
      (Variables|Default|SetfallenPlayerIndex 1)))
  (bind _outactors_2 (Actor|GetAllActorsOfClass "/Game/Blueprints/Generic/TutorialHandler.TutorialHandler_C"))
  (if (Utilities|IsValid (Utilities|Array|Get(acopy) _outactors_2))
    (Variables|Default|SettutorialMode true)))

(fn SendforHelp
  (bind _helpchars (LocalVariables|GethelpChars))
  (bind _helpmessage (LocalVariables|GetHelpMessage))
  (bind _helpfonts (LocalVariables|GethelpFonts))
  (if (Variables|Default|GettutorialMode)
    (Development|PrintString "not sending?")
    (else
      (if (== (Variables|Default|GetfallenPlayerIndex) 0)
        (Utilities|Array|Add _helpchars "")
        (Utilities|Array|Add _helpchars (Utilities|String|MakeLiteralString "ABIGAIL"))
        (Utilities|Array|Add _helpmessage (Utilities|String|MakeLiteralString "You have fallen"))
        (Utilities|Array|Add _helpmessage (Utilities|String|MakeLiteralString "LEILA, I'M DYING!!!"))
        (Utilities|Array|Add _helpfonts 0)
        (Utilities|Array|Add _helpfonts 2)
        (else
          (Utilities|Array|Add _helpchars (Utilities|String|MakeLiteralString "LEILA"))
          (Utilities|Array|Add _helpchars "")
          (Utilities|Array|Add _helpmessage (Utilities|String|MakeLiteralString "Help, I've fallen and I can't get up!"))
          (Utilities|Array|Add _helpmessage (Utilities|String|MakeLiteralString "You have fallen"))
          (Utilities|Array|Add _helpfonts 1)
          (Utilities|Array|Add _helpfonts 0)))
      (Class|DialogueHandler|SendInputText (Variables|Default|GetDialogueHandler) (LocalVariables|GetHelpMessage) (LocalVariables|GethelpFonts) (LocalVariables|GethelpChars)))))

(fn SendRevivePrompt
  (bind _revivemessage (LocalVariables|GetreviveMessage))
  (bind _revivefonts (LocalVariables|GetreviveFonts))
  (bind _dialoguehandler (Variables|Default|GetDialogueHandler))
  (if (not (Variables|Default|GettutorialMode))
    (if (== (Variables|Default|GetfallenPlayerIndex) 0)
      (Utilities|Array|Add _revivemessage (Utilities|String|MakeLiteralString "You have fallen"))
      (Utilities|Array|Add _revivemessage (Utilities|String|MakeLiteralString "Hold A to Revive"))
      (Utilities|Array|Add _revivefonts 0)
      (Utilities|Array|Add _revivefonts 0)
      (else
        (Utilities|Array|Add _revivemessage (Utilities|String|MakeLiteralString "Hold A to Revive"))
        (Utilities|Array|Add _revivemessage (Utilities|String|MakeLiteralString "You have fallen"))
        (Utilities|Array|Add _revivefonts 0)
        (Utilities|Array|Add _revivefonts 0)))
    (Class|DialogueHandler|ToggleSplitMode _dialoguehandler true)
    (Class|DialogueHandler|SendInputText _dialoguehandler (LocalVariables|GetreviveMessage) (LocalVariables|GetreviveFonts) (Utilities|Array|MakeArray "" ""))))

(fn UpdatePosition
  (Transformation|SetWorldLocation (Variables|Default|GetDefaultSceneRoot) (Transformation|GetWorldLocation (Variables|/Script/Engine.Actor|GetRootComponent (Variables|Default|GetcrawlingKid))) false false))

(fn ReturnBacktoPreviousLevel
  (bind _asplayground_game_instance (Utilities|Casting|CastToPlaygroundGameInstance (Game|GetGameInstance)))
  (Game|OpenLevel(byName) (Utilities|String|StringToName (Variables|/Game/Blueprints/PlaygroundGameInstance.PlaygroundGameInstance_C|GetReturnMap _asplayground_game_instance))))

(fn SpawnDeathPromptwithRestartOption
  (bind _returnvalue (UserInterface|CreateWidget "/Game/Blueprints/UI/DeathPopUp.DeathPopUp_C"))
  (Input|SetInputModeUIOnly (Game|GetPlayerController 0) _returnvalue "DoNotLock")
  (UserInterface|Viewport|AddtoViewport _returnvalue 0))

(fn TransformtoChildren
  (bind _fallencontroller (Variables|Default|GetfallenController))
  (bind _warriors (Variables|Default|GetWarriors))
  (bind _output (Utilities|Array|Get(acopy) _warriors))
  (bind _returnvalue (Transformation|GetActorTransform _output))
  (Utilities|FlowControl|Sequence
    (:then_0
      (Rendering|SetVisibility (Variables|/Script/Engine.Character|GetMesh _output) false true)
      (Collision|SetActorEnableCollision _output false)
      (Utilities|Casting|CastToJArcher _output
        (:then
          (bind _returnvalue_2 (Game|SpawnActorfromClass "/Game/Blueprints/Children/Younger.Younger_C" _returnvalue "Undefined" 0 0))
          (bind _output_get (Variables|Default|SetcrawlingKid _returnvalue_2))
          (Animation|Montage|MontagePlay (Components|SkeletalMesh|GetAnimInstance (Variables|/Script/Engine.Character|GetMesh _output_get)) "/Game/CharacterAssets/Younger/New/Newer/younger_DeathMontage.younger_DeathMontage" 1.0 "MontageLength" 0.0 true))
        (:CastFailed
          (bind _returnvalue_3 (Game|SpawnActorfromClass "/Game/Blueprints/Children/Older.Older_C" _returnvalue "Undefined" 0 0))
          (bind _output_get_2 (Variables|Default|SetcrawlingKid _returnvalue_3))
          (Animation|Montage|MontagePlay (Components|SkeletalMesh|GetAnimInstance (Variables|/Script/Engine.Character|GetMesh _output_get_2)) "/Game/CharacterAssets/Older/New/Newer/Older_DeathMontage.Older_DeathMontage" 1.0 "MontageLength" 0.0 true))))
    (:then_1
      (Pawn|UnPossess _fallencontroller)
      (Pawn|Possess _fallencontroller (Variables|Default|GetcrawlingKid))
      (Variables|/Script/PlaygroundHeroes.JKid|SetMovementModifier (Variables|Default|GetcrawlingKid) 0.0))))

(fn TransformtoHeroes
  (bind _fallencontroller (Variables|Default|GetfallenController))
  (bind _warriors (Variables|Default|GetWarriors))
  (bind _output (Utilities|Array|Get(acopy) _warriors))
  (Pawn|UnPossess _fallencontroller)
  (Pawn|Possess _fallencontroller _output)
  (Rendering|SetVisibility (Variables|/Script/Engine.Character|GetMesh _output) true true)
  (Collision|SetActorEnableCollision _output true)
  (Actor|DestroyActor (Variables|Default|GetcrawlingKid)))