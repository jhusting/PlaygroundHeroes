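; Firewatch tower actor that turns on custom depth rendering for its static mesh, presumably for an outline, while a JKid is nearby.
; It caches all JKid actors at BeginPlay and checks their distance to itself every Tick.
; Any kid in range enables custom depth and restarts a one-second timer, which switches it off once no kid has been in range for that long.
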(event EventBeginPlay
  (bind _outactors (Actor|GetAllActorsOfClass "/Script/PlaygroundHeroes.JKid"))
  (Variables|Default|SetKids _outactors))

(event Collision|EventActorBeginOverlap
  (params (OtherActor :type Actor%20Object%20Reference)))

(event EventTick
  (params (DeltaSeconds :type Float%20%28single-precision%29))
  (for _array_element (Variables|Default|GetKids)
    (if (<= (Transformation|GetDistanceTo _array_element) 3.75e+03)
      (Rendering|SetRenderCustomDepth (Variables|Debug|GetStaticMeshComponent) true)
      (Utilities|Time|ClearandInvalidateTimerbyHandle (Variables|Default|GetDepthTimerHandler))
      (bind _returnvalue (Utilities|Time|SetTimerbyFunctionName 0 "ResetCustomDepth" 1.0))
      (Variables|Default|SetDepthTimerHandler _returnvalue))))

(fn ConstructionScript)

(fn ResetCustomDepth
  (Rendering|SetRenderCustomDepth (Variables|Debug|GetStaticMeshComponent) false))