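; Co-op level-change trigger where the Younger and Older kids hold A to travel or start a Level Sequence.
; Box overlaps track kids present, saving DialogueHandler text on first entry and restoring it when empty.
; Tick spins the visual and polls readiness, requiring both kids or one per OnlyOneCharacterNeeded, with split-screen prompts.
; Travel stores map names and kid locations in PlaygroundGameInstance; sequences blend both players to SequenceCamera.
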(event OnComponentBeginOverlap(Box)
  (params (OverlappedComponent :type Primitive%20Component%20Object%20Reference) (OtherActor :type Actor%20Object%20Reference) (OtherComp :type Primitive%20Component%20Object%20Reference) (OtherBodyIndex :type Integer) (bFromSweep :type Boolean) (SweepResult :type Hit%20Result%20Structure%20%28by%20ref%29))
  (bind _warriors (Variables|Default|GetWarriors))
  (bind _asjkid (Utilities|Casting|CastToJKid OtherActor))
  (Utilities|Array|AddUnique _warriors _asjkid)
  (if (== (Utilities|Array|Length _warriors) 1) ; if first player entered
    (Class|DialogueHandler|SaveDialogue (Variables|Default|GetDialogHandler))))

(event OnComponentEndOverlap(Box)
  (params (OverlappedComponent :type Primitive%20Component%20Object%20Reference) (OtherActor :type Actor%20Object%20Reference) (OtherComp :type Primitive%20Component%20Object%20Reference) (OtherBodyIndex :type Integer))
  (bind _warriors (Variables|Default|GetWarriors))
  (bind _asjkid (Utilities|Casting|CastToJKid OtherActor))
  (Utilities|Array|RemoveItem _warriors _asjkid)
  (if (== (Utilities|Array|Length _warriors) 0)
    ;[1 1 1] If last person inside left, clear out text
    (CallFunction|PrintDialog (Utilities|Array|MakeArray (Utilities|String|MakeLiteralString)) (Utilities|Array|MakeArray 0.0) (Utilities|Array|MakeArray 1) false true)
    (Class|DialogueHandler|LoadSavedDialogue (Variables|Default|GetDialogHandler))))

(event EventBeginPlay
  (bind _outactors (Actor|GetAllActorsOfClass "/Script/PlaygroundHeroes.DialogueHandler"))
  (Variables|Default|SetDialogHandler (Utilities|Array|Get(acopy) _outactors)))

(event Collision|EventActorBeginOverlap
  (params (OtherActor :type Actor%20Object%20Reference)))

(event EventTick
  (params (DeltaSeconds :type Float%20%28single-precision%29))
  (bind _warriors (Variables|Default|GetWarriors))
  (bind _returnvalue (Utilities|Array|Length _warriors))
  (if (Variables|Default|GetStationaryVisual)
    _
    (else
      (CallFunction|RotateVisual)))
  (if (Variables|Default|GetOnlyOneCharacterNeeded)
    ;[1 1 1] If Either Presses 'A' Button and OnlyOneCharacterNeeded is TRUE
    (for _array_element (Collision|GetOverlappingActors "/Script/PlaygroundHeroes.JKid" :!class /Script/Engine.Actor)
      (bind _asjkid (Utilities|Casting|CastToJKid _array_element))
      (CallFunction|OnlyOneNeeded _asjkid))
    (elif (== _returnvalue 2)
      (CallFunction|BothPresent)
      (elif (== 1 _returnvalue)
        (CallFunction|OnlyOnePresent)))))

(fn ConstructionScript)

(fn PrintDialog
  (params (Lines :type Array%20of%20Strings) (Durations :type Array%20of%20Floats%20%28single-precision%29) (FOnts :type Array%20of%20Integers) (Split :type Boolean) (PauseAfter :type Boolean))
  (bind _dialoghandler (Variables|Default|GetDialogHandler))
  (Class|DialogueHandler|ToggleSplitMode _dialoghandler Split)
  (Class|DialogueHandler|SendNewdialogueSequence _dialoghandler Lines Durations FOnts)
  (if PauseAfter
    (Class|DialogueHandler|Pause _dialoghandler)))

(fn BothPresent
  (bind _warriors (Variables|Default|GetWarriors))
  (bind _temparray (Variables|Default|GetTempArray))
  (bind _output (Utilities|Array|Get(acopy) _warriors))
  (bind _output_2 (Utilities|Array|Get(acopy) _warriors 1))
  (bind _interacting (Variables|/Script/PlaygroundHeroes.JKid|Getinteracting _output_2))
  (bind _interacting_2 (Variables|/Script/PlaygroundHeroes.JKid|Getinteracting _output))
  ;[1 1 1] We want our array to be ordered Archer, Knight
  ;;[1 1 1] If the array order is Archer, Knight
  (bind _asyounger (Utilities|Casting|CastToYounger _output)
    (:then
      (Utilities|Array|AddUnique _temparray _asyounger)
      (bind _asolder (Utilities|Casting|CastToOlder _output_2))
      (Utilities|Array|AddUnique _temparray _asolder))
    (:CastFailed
      ;;[1 1 1] If array order is Knight, Archer
      (bind _asyounger_2 (Utilities|Casting|CastToYounger _output_2))
      (Utilities|Array|AddUnique (Variables|Default|GetTempArray) _asyounger_2)
      (Utilities|Casting|CastToOlder _output)))
  ;[1 1 1] Both pressing A
  (if (and _interacting_2 _interacting)
    (if (Variables|Default|GetPlaySequenceVsOpenlevel)
      (CallFunction|InitiateSequence)
      (else
        (CallFunction|MovetoLevel)))
    (else
      ;[1 1 1] A pressing A, B in
      (if (and (not _interacting_2) _interacting)
        (CallFunction|PrintDialog (Utilities|Array|MakeArray "Readied" (Utilities|String|Append "Hold A to move to " (Variables|Default|GetLevelNameDisplayed))) (Utilities|Array|MakeArray 0.0 0.0) (Utilities|Array|MakeArray 1 2) true true)
        (else
          ;[1 1 1] A In, B pressing A
          (if (and _interacting_2 (not _interacting))
            (CallFunction|PrintDialog (Utilities|Array|MakeArray (Utilities|String|Append "Hold A to move to " (Variables|Default|GetLevelNameDisplayed)) "Readied") (Utilities|Array|MakeArray 0.0 0.0) (Utilities|Array|MakeArray 1 2) true true)
            (else
              ;[1 1 1] Neither is pressing A
              (CallFunction|PrintDialog (Utilities|Array|MakeArray "Hold A to Ready Up" "") (Utilities|Array|MakeArray 0.0 0.0) (Utilities|Array|MakeArray 1 1) false true))))))))

(fn OnlyOnePresent
  (bind _warriors (Variables|Default|GetWarriors))
  (bind _output (Utilities|Array|Get(acopy) _warriors))
  ;[1 1 1] Is the one actor an archer?
  (Utilities|Casting|CastToYounger _output
    (:then
      ;[1 1 1] Is the Archer present pressing A?
      (if (Variables|/Script/PlaygroundHeroes.JKid|Getinteracting _output)
        (CallFunction|PrintDialog (Utilities|Array|MakeArray "Readied" (Utilities|String|Append "Abigail: Come over here, lets go to " (Variables|Default|GetLevelNameDisplayed))) (Utilities|Array|MakeArray 0.0 0.0) (Utilities|Array|MakeArray 1 2) true true)
        (else
          (CallFunction|PrintDialog (Utilities|Array|MakeArray "Hold A to ready up" "") (Utilities|Array|MakeArray 0.0 0.0) (Utilities|Array|MakeArray 1 1) true true))))
    (:CastFailed
      ;[1 1 1] Is the Knight presing A?
      (if (Variables|/Script/PlaygroundHeroes.JKid|Getinteracting _output)
        (CallFunction|PrintDialog (Utilities|Array|MakeArray (Utilities|String|Append "Leila: Come over here, lets go to " (Variables|Default|GetLevelNameDisplayed)) "Readied") (Utilities|Array|MakeArray 0.0 0.0) (Utilities|Array|MakeArray 1 2) true true)
        (else
          (CallFunction|PrintDialog (Utilities|Array|MakeArray "" "Hold A to ready up") (Utilities|Array|MakeArray 0.0 0.0) (Utilities|Array|MakeArray 1 2) true true))))))

(fn RotateVisual
  (bind _visual (Variables|Default|GetVisual))
  (bind _returnvalue (Transformation|GetWorldRotation _visual))
  (bind (_roll _pitch _yaw) (Math|Rotator|BreakRotator _returnvalue))
  (Transformation|SetWorldRotation _visual (Math|Rotator|MakeRotator _roll _pitch (+ _yaw 1.0)) false false))

(fn SetKidLocations
  (bind _asplayground_game_instance (Utilities|Casting|CastToPlaygroundGameInstance (Game|GetGameInstance)))
  (bind _outactors (Actor|GetAllActorsOfClass "/Game/Blueprints/Children/Younger.Younger_C"))
  (Variables|/Game/Blueprints/PlaygroundGameInstance.PlaygroundGameInstance_C|SetPlayer%200%20Vector%203 _asplayground_game_instance (Math|Vector|MakeVector (.X (Math|Vector|BreakVector (Transformation|GetActorLocation (Utilities|Array|Get(acopy) _outactors)))) (.Y (Math|Vector|BreakVector (Transformation|GetActorLocation (Utilities|Array|Get(acopy) _outactors)))) (+ (.Z (Math|Vector|BreakVector (Transformation|GetActorLocation (Utilities|Array|Get(acopy) _outactors)))) 25.0)))
  (Variables|/Game/Blueprints/PlaygroundGameInstance.PlaygroundGameInstance_C|SetPlayer%200%20Boolean _asplayground_game_instance true)
  (bind _outactors_2 (Actor|GetAllActorsOfClass "/Game/Blueprints/Children/Older.Older_C"))
  (Variables|/Game/Blueprints/PlaygroundGameInstance.PlaygroundGameInstance_C|SetPlayer%201%20Vector%203 _asplayground_game_instance (Math|Vector|MakeVector (.X (Math|Vector|BreakVector (Transformation|GetActorLocation (Utilities|Array|Get(acopy) _outactors_2)))) (.Y (Math|Vector|BreakVector (Transformation|GetActorLocation (Utilities|Array|Get(acopy) _outactors_2)))) (+ (.Z (Math|Vector|BreakVector (Transformation|GetActorLocation (Utilities|Array|Get(acopy) _outactors_2)))) 25.0)))
  (Variables|/Game/Blueprints/PlaygroundGameInstance.PlaygroundGameInstance_C|SetPlayer%201%20Boolean _asplayground_game_instance true))

(fn MovetoLevel
  (bind _asplayground_game_instance (Utilities|Casting|CastToPlaygroundGameInstance (Game|GetGameInstance)))
  (Variables|/Game/Blueprints/PlaygroundGameInstance.PlaygroundGameInstance_C|SetDesiredMap _asplayground_game_instance (Variables|Default|GetDesiredLevel))
  (bind _returnvalue (Game|GetCurrentLevelName true))
  (bind _output_get (Variables|/Game/Blueprints/PlaygroundGameInstance.PlaygroundGameInstance_C|SetReturnMap _asplayground_game_instance _returnvalue))
  (Development|PrintString _output_get)
  (Game|OpenLevel(byName) (Variables|Default|GetLevelToGoTo))
  (CallFunction|SetKidLocations))

(fn InitiateSequence
  (bind _sequencetoplay (Variables|Sequence|GetSequenceToPlay))
  (bind _sequencecamera (Variables|Sequence|GetSequenceCamera))
  (bind _sequenceplayer (Variables|/Script/LevelSequence.LevelSequenceActor|GetSequencePlayer _sequencetoplay))
  (Game|Player|SetViewTargetwithBlend (Game|GetPlayerController 0) _sequencecamera 0.0 "VTBlend_Linear" 0.0 false)
  (Game|Player|SetViewTargetwithBlend (Game|GetPlayerController 1) _sequencecamera 0.0 "VTBlend_Linear" 0.0 false)
  (Sequencer|Player|Play _sequenceplayer :!class /Script/MovieScene.MovieSceneSequencePlayer)
  (EventDispatchers|BindEventtoOnFinished _sequenceplayer (EventDispatchers|CreateEvent :!event MovetoLevel)))

(fn OnlyOneNeeded
  (params (Kid :type J%20Kid%20Object%20Reference))
  ;[1 1 1] Is the one actor the Younger?
  (Utilities|Casting|CastToYounger Kid
    (:then
      ;[1 1 1] Is the Archer present pressing A?
      (if (Variables|/Script/PlaygroundHeroes.JKid|Getinteracting Kid)
        (if (Variables|Default|GetPlaySequenceVsOpenlevel)
          (CallFunction|InitiateSequence)
          (else
            (CallFunction|MovetoLevel)))
        (else
          (CallFunction|PrintDialog (Utilities|Array|MakeArray (Utilities|String|Append "Hold A to move to " (Variables|Default|GetLevelNameDisplayed)) "") (Utilities|Array|MakeArray 0.0 0.0) (Utilities|Array|MakeArray 1 1) true true))))
    (:CastFailed
      ;[1 1 1] Is the Knight presing A?
      (if (Variables|/Script/PlaygroundHeroes.JKid|Getinteracting Kid)
        (if (Variables|Default|GetPlaySequenceVsOpenlevel)
          (CallFunction|InitiateSequence)
          (else
            (CallFunction|MovetoLevel)))
        (else
          (CallFunction|PrintDialog (Utilities|Array|MakeArray "" (Utilities|String|Append "Hold A to move to " (Variables|Default|GetLevelNameDisplayed))) (Utilities|Array|MakeArray 0.0 0.0) (Utilities|Array|MakeArray 1 2) true true))))))