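; Tutorial sequencer actor that walks the Knight and Archer through story dialogue and control prompts.
; Tick switches on DialogueStep, sending each step's lines to JDialogueHandler, then showing an input prompt once dialogue finishes.
; Every prompt step currently advances via the movement check, which Archer movement alone satisfies.
; Dodge, attack, block, revive and key-item checks, plus per-player input widgets, exist but are not wired in.
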(event EventBeginPlay
  (CallFunction|FindPlayersandHandler))

(event Collision|EventActorBeginOverlap
  (params (OtherActor :type Actor%20Object%20Reference)))

(event EventTick
  (params (DeltaSeconds :type Float%20%28single-precision%29))
  (CallFunction|DisplayText)
  (switch int (Variables|Default|GetDialogueStep)
    (:0
      (if (Variables|/Script/PlaygroundHeroes.DialogueHandler|GetdialogueFinished (Variables|Default|GetDialogHandler))
        (Variables|Default|SetDialogueStep (+ (Variables|Default|GetDialogueStep) 1))
        (Variables|Default|SetdialogueSent false)))
    (:1
      (CallFunction|CheckifDialogFinished (Utilities|Array|MakeArray "\"Use Left Stick To Move\"") true)
      (if (Variables|Default|GetinputReady)
        (ProgressChecks|HandleMovementInputCheck :!label _label)))
    (:2
      (CallFunction|CheckifDialogFinished (Utilities|Array|MakeArray "\"Press B to dodge an attack. Dodging costs Stamina\"") true)
      (if (Variables|Default|GetinputReady)
        (goto _label)))
    (:3
      (CallFunction|CheckifDialogFinished (Utilities|Array|MakeArray "\"Press RB to attack. You can string together 3 attacks to deal extra damage\"") true)
      (if (Variables|Default|GetinputReady)
        (goto _label)))
    (:4
      (CallFunction|CheckifDialogFinished (Utilities|Array|MakeArray "\"Hold and release RB to fire an arrow. A fully-charged arrow does more damage\"") true)
      (if (Variables|Default|GetinputReady)
        (goto _label)))
    (:5
      (CallFunction|CheckifDialogFinished (Utilities|Array|MakeArray "\"Hold LB to block. Blocking the moment an attack lands greatly reduces Stamina damage\"") true)
      (if (Variables|Default|GetinputReady)
        (goto _label)))
    (:6
      (CallFunction|CheckifDialogFinished (Utilities|Array|MakeArray "\"Hold A near your fallen sister to revive her!\"") true)
      (if (Variables|Default|GetinputReady)
        (goto _label)))
    (:7
      (CallFunction|CheckifDialogFinished (Utilities|Array|MakeArray "\"Get together and hold A near a key object to interact with it\"") true)
      (if (Variables|Default|GetinputReady)
        (goto _label)))))

(fn ConstructionScript)

(fn FindPlayersandHandler
  (bind _outactors (Actor|GetAllActorsOfClass "/Game/Blueprints/Warriors/JKnightBP.JKnightBP_C"))
  (bind _output_get (Variables|Default|SetKnight (Utilities|Array|Get(acopy) _outactors)))
  (Utilities|IsValid _output_get
    (:Is%20Valid
      _)
    (:Is%20Not%20Valid
      (Development|PrintString "TutorialHandler (WARNING): Knight not found")))
  (bind _outactors_2 (Actor|GetAllActorsOfClass "/Game/Blueprints/Warriors/JArcherBP.JArcherBP_C"))
  (bind _output_get_2 (Variables|Default|SetArcher (Utilities|Array|Get(acopy) _outactors_2)))
  (Utilities|IsValid _output_get_2
    (:Is%20Valid
      _)
    (:Is%20Not%20Valid
      (Development|PrintString "TutorialHandler (WARNING): Archer not found")))
  (bind _outactors_3 (Actor|GetAllActorsOfClass "/Game/Blueprints/UI/JDialogueHandler.JDialogueHandler_C"))
  (bind _output_get_3 (Variables|Default|SetDialogHandler (Utilities|Array|Get(acopy) _outactors_3)))
  (Utilities|IsValid _output_get_3
    (:Is%20Not%20Valid
      (Development|PrintString "Tutorial Handler (WARNING): Dialog Handler not found"))))

(fn DisplayText
  (if (not (Variables|Default|GetdialogueSent))
    (Variables|/Script/PlaygroundHeroes.DialogueHandler|SetsplitMode (Variables|Default|GetDialogHandler) true)
    (switch int (Variables|Default|GetDialogueStep)
      (:0
        ;[1 1 1] Case 0 == Intro Cinematic
        (CallFunction|PrintDialog (Utilities|Array|MakeArray "Intro 00" "Intro 01" "Intro 02") (Utilities|Array|MakeArray 2.0 2.0 2.0) (Utilities|Array|MakeArray 1 1 1) (Utilities|Array|MakeArray "\"A\"" "\"B\"" "\"A\"") false false))
      (:1
        (Class|DialogueHandler|SendNewdialogueSequence (Variables|Default|GetDialogHandler) (Utilities|Array|MakeArray "Zorrander must've sent him after us. C'mon this is the perfect opportunity to practice before we go on our adventure!" "Now, although we may be the strongest fighters in all the land, we still need to practice!") (Utilities|Array|MakeArray 2.0 2.0) (Utilities|Array|MakeArray 1 2) (Utilities|Array|MakeArray "LEILA" "ABIGAIL")))
      (:2
        (Class|DialogueHandler|SendNewdialogueSequence (Variables|Default|GetDialogHandler) (Utilities|Array|MakeArray "Look Out!" "") (Utilities|Array|MakeArray 2.0 2.0) (Utilities|Array|MakeArray 1 2) (Utilities|Array|MakeArray "LEILA" "")))
      (:3
        (CallFunction|PrintDialog (Utilities|Array|MakeArray "" "Show him your strength!") (Utilities|Array|MakeArray 2.0 2.0) (Utilities|Array|MakeArray 1 2) (Utilities|Array|MakeArray "" "ABIGAIL") true false))
      (:4
        (CallFunction|PrintDialog (Utilities|Array|MakeArray "Go shoot him with your arrows while I attack him!" "") (Utilities|Array|MakeArray 2.0 2.0) (Utilities|Array|MakeArray 1 2) (Utilities|Array|MakeArray "LEILA" "") true false))
      (:5
        (CallFunction|PrintDialog (Utilities|Array|MakeArray "" "Leila quick, use your shield!") (Utilities|Array|MakeArray 2.0 2.0) (Utilities|Array|MakeArray 1 2) (Utilities|Array|MakeArray "" "ABIGAIL") true false))
      (:6
        (if (Variables|/Script/PlaygroundHeroes.JHero|GetbHasFallen (Variables|Default|GetKnight))
          ;[1 1 1] Leila Down
          (CallFunction|PrintDialog (Utilities|Array|MakeArray "Abigail, come help me. I've fallen and I can't get up" "" "A-Abigail come over here!" "I'll come help you hold on!") (Utilities|Array|MakeArray 2.0 2.0 2.0 2.0) (Utilities|Array|MakeArray 1 2 1 2) (Utilities|Array|MakeArray "LEILA" "" "LEILA" "ABIGAIL") true false)
          (else
            ;[1 1 1] Abigail Down
            (CallFunction|PrintDialog (Utilities|Array|MakeArray "" "Leila help!" "Abigail I'll save you" "I'm Dyinnnnnggg") (Utilities|Array|MakeArray 2.0 2.0 2.0 2.0) (Utilities|Array|MakeArray 1 2 1 2) (Utilities|Array|MakeArray "LEILA" "ABIGAIL" "LEILA" "ABIGAIL") true false))))
      (:7
        (CallFunction|PrintDialog (Utilities|Array|MakeArray "Now we have to be careful on our journey to find Zorrander, he’s going to do everything in his power to stop us from reaching him. What do we know about him?" "Well, when he learned that the two strongest heroes were on their way to his lair, he got scared that his evil plans would be ruined! So, to protect himself he created three monsters to guard the forest." "Like that will stop us!" "Of course it won’t! But he believed that only the purest evil would be strong enough to stop us... so he created each monster using a piece of his black heart. The monsters are all a part of him." "Hmm so that must mean if we defeat the monsters Zorrander becomes weaker?" "Yes, but each monster will try their best to keep us out of the forest. They can see our deepest darkest fears and will use that to try and scare us away." "Uh...They know our deepest darkest fears…?" "Yup but that’s ok because we’re the bravest heroes!" "You’re right, they won’t scare us." "Leila, what’s your greatest fear?" "… My greatest fear is… losing you." "Losing me? That seems pretty lame. Don’t worry, we’ll always be together! Right?" "Of course silly… " "The forest is just past that big tree over there, I am ready when you are\"") (Utilities|Array|MakeArray 2.0 2.0 2.0 2.0 2.0 2.0 2.0 2.0 2.0 2.0 2.0 2.0 2.0 2.0) (Utilities|Array|MakeArray 1 2 1 2 1 2 1 2 1 2 1 2 1 2) (Utilities|Array|MakeArray "LEILA" "ABIGAIL" "LEILA" "ABIGAIL" "LEILA" "ABIGAIL" "LEILA" "ABIGAIL" "LEILA" "ABIGAIL" "LEILA" "ABIGAIL" "LEILA" "ABIGAIL") true false)))
    (Variables|Default|SetdialogueSent true)
    (Variables|Default|SetinputReady false)))

(fn SendInputText
  (params (inputLines :type Array%20of%20Strings) (inputInCenter :type Boolean))
  (bind _dialoghandler (Variables|Default|GetDialogHandler))
  (if (not (Variables|Default|GetinputSent))
    (if inputInCenter
      (Class|DialogueHandler|SendNewdialogueSequence _dialoghandler inputLines (Utilities|Array|MakeArray 0.0) (Variables|Default|GetinputFonts) (Variables|Default|GetinputChars))
      (Class|DialogueHandler|Pause _dialoghandler)
      (else
        (Class|DialogueHandler|SendInputText _dialoghandler inputLines (Variables|Default|GetinputFonts) (Variables|Default|GetinputChars))))
    (Variables|Default|SetinputSent true)))

(fn PostInput
  ;[1 1 1] Clean Up
  (Variables|Default|SetKnightDidInput false)
  (Variables|Default|SetArcherDidInput false)
  (Variables|Default|SetinputSent false)
  ;[1 1 1] Advance Dialogue to Next Step
  (Variables|Default|SetDialogueStep (+ (Variables|Default|GetDialogueStep) 1))
  (Variables|Default|SetdialogueSent false))

(fn HandleMovementInputCheck
  (bind _archer (Variables|Default|GetArcher))
  (bind _knight (Variables|Default|GetKnight))
  (bind _inputdirection (Variables|/Script/PlaygroundHeroes.JHero|GetInputDirection _knight))
  (bind _inputdirection_2 (Variables|/Script/PlaygroundHeroes.JHero|GetInputDirection _archer))
  (bind (_x _y) (Math|Vector|BreakVector _inputdirection))
  (bind (_x_2 _y_2) (Math|Vector|BreakVector _inputdirection_2))
  (if (or (!= _x_2 0.0) (!= _y_2 0.0))
    (Variables|Default|SetArcherDidInput true)
    (CallFunction|PostInput :!label _label)
    (else
      (if (or (!= _x 0.0) (!= _y 0.0))
        (Variables|Default|SetKnightDidInput true))
      (if (and (Variables|Default|GetArcherDidInput) (Variables|Default|GetKnightDidInput))
        (goto _label)))))

(fn HandleDodgeCheck
  (if (Variables|/Script/PlaygroundHeroes.JHero|GetbInputtingDodge (Variables|Default|GetArcher))
    (Variables|Default|SetArcherDidInput true))
  (if (Variables|/Script/PlaygroundHeroes.JHero|GetbInputtingDodge (Variables|Default|GetKnight))
    (Variables|Default|SetKnightDidInput false))
  (if (Variables|Default|GetArcherDidInput)
    (CallFunction|PostInput)))

(fn HandleKnightAttack
  (bind _knight (Variables|Default|GetKnight))
  (bind _currenthittype (Variables|/Script/PlaygroundHeroes.JHero|GetCurrentHitType _knight))
  (if (Utilities|Enum|Equal(Enum) _currenthittype "KnightAttack1")
    (Development|PrintString "KnightAttack1"))
  (if (Utilities|Enum|Equal(Enum) _currenthittype "KnightAttack2")
    (Development|PrintString "KnightAttack2"))
  (if (Utilities|Enum|Equal(Enum) _currenthittype "KnightAttack3")
    (Development|PrintString "KnightAttack3")
    (CallFunction|PostInput)
    (Variables|Default|SetDialogueStep (+ (Variables|Default|GetDialogueStep) 1))
    (Variables|Default|SetdialogueSent false)))

(fn HandleArcherAttack
  (if (>= (Variables|/Script/PlaygroundHeroes.JArcher|GettimeHeld (Variables|Default|GetArcher)) 2.0)
    (Development|PrintString "Archer held longer than 2 secs")
    (CallFunction|PostInput)))

(fn HandleKnightBlock
  (bind _knight (Variables|Default|GetKnight))
  (if (Components|Activation|IsActive (Variables|/Game/Blueprints/Warriors/JKnightBP.JKnightBP_C|GetBlockEmit _knight))
    (Development|PrintString "Block"))
  (if (Components|Activation|IsActive (Variables|/Game/Blueprints/Warriors/JKnightBP.JKnightBP_C|GetPerfectBlockEmit _knight))
    (Development|PrintString "PerfectBlock")
    (CallFunction|PostInput)))

(fn HandleRevive
  (if (not (and (Variables|/Script/PlaygroundHeroes.JHero|GetbHasFallen (Variables|Default|GetKnight)) (Variables|/Script/PlaygroundHeroes.JHero|GetbHasFallen (Variables|Default|GetArcher))))
    (CallFunction|PostInput)))

(fn HandleKeyItem)

(fn CheckifDialogFinished
  (params (Input%20Text%20Lines :type Array%20of%20Strings) (inputInCenter :type Boolean))
  (if (Variables|/Script/PlaygroundHeroes.DialogueHandler|GetdialogueFinished (Variables|Default|GetDialogHandler))
    (Class|DialogueHandler|ToggleSplitMode (Variables|Default|GetDialogHandler) false)
    (Variables|Default|SetinputReady true)
    (CallFunction|SendInputText Input%20Text%20Lines inputInCenter)))

(fn PrintDialog
  (params (Lines :type Array%20of%20Strings) (Durations :type Array%20of%20Floats%20%28single-precision%29) (Fonts :type Array%20of%20Integers) (Chars :type Array%20of%20Strings) (Split :type Boolean) (PauseAfter :type Boolean))
  (bind _dialoghandler (Variables|Default|GetDialogHandler))
  (Class|DialogueHandler|ToggleSplitMode _dialoghandler Split)
  (Class|DialogueHandler|SendNewdialogueSequence _dialoghandler Lines Durations Fonts Chars)
  (if PauseAfter
    (Class|DialogueHandler|Pause _dialoghandler)))

(fn AttachInputWidgets
  (bind _returnvalue (UserInterface|CreateWidget "/Game/Blueprints/UI/ArcherTutorialInputWidget.ArcherTutorialInputWidget_C" (Game|GetPlayerController 0)))
  (Variables|/Game/Blueprints/UI/ArcherTutorialInputWidget.ArcherTutorialInputWidget_C|SetArcher _returnvalue (Variables|Default|GetArcher))
  (bind _output_get (Variables|InputWidgets|SetArcherInputWidget _returnvalue))
  (UserInterface|Viewport|AddtoViewport _output_get 0)
  (bind _returnvalue_2 (UserInterface|CreateWidget "/Game/Blueprints/UI/KnightTutorialInputWidget.KnightTutorialInputWidget_C" (Game|GetPlayerController 1)))
  (Variables|/Game/Blueprints/UI/KnightTutorialInputWidget.KnightTutorialInputWidget_C|SetKnight _returnvalue_2 (Variables|Default|GetKnight))
  (bind _output_get_2 (Variables|InputWidgets|SetKnightInputWidget _returnvalue_2))
  (UserInterface|Viewport|AddtoViewport _output_get_2 0)
  (bind _returnvalue_3 (UserInterface|CreateWidget "/Game/Blueprints/UI/BothTutorialInputWidget.BothTutorialInputWidget_C" (Game|GetPlayerController 0)))
  (Variables|/Game/Blueprints/UI/BothTutorialInputWidget.BothTutorialInputWidget_C|SetArcher _returnvalue_3 (Variables|Default|GetArcher))
  (Variables|/Game/Blueprints/UI/BothTutorialInputWidget.BothTutorialInputWidget_C|SetKnight _returnvalue_3 (Variables|Default|GetKnight))
  (bind _output_get_3 (Variables|InputWidgets|SetBothInputWidget _returnvalue_3))
  (UserInterface|Viewport|AddtoViewport _output_get_3 0))

(fn DEBUGUpdateInputWidgets
  (Appearance|SetBrushfromTexture (Variables|/Game/Blueprints/UI/ArcherTutorialInputWidget.ArcherTutorialInputWidget_C|GetImage_59 (Variables|InputWidgets|GetArcherInputWidget)) "/Game/Nature/Grass/Alt_Grass/grass.grass" false)
  (Appearance|SetBrushfromTexture (Variables|/Game/Blueprints/UI/KnightTutorialInputWidget.KnightTutorialInputWidget_C|GetImage_56 (Variables|InputWidgets|GetKnightInputWidget)) "/Game/Nature/Grass/Alt_Grass/grass.grass" false)
  (Appearance|SetBrushfromTexture (Variables|/Game/Blueprints/UI/BothTutorialInputWidget.BothTutorialInputWidget_C|GetImage_74 (Variables|InputWidgets|GetBothInputWidget)) "/Game/Nature/Grass/Alt_Grass/grass.grass" false))