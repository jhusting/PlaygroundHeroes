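; Trigger-box actor that plays a dialogue sequence on overlap, optionally clearing it on exit.
; BeginPlay caches the sole JDialogueHandler, which receives either manually entered line arrays or is bypassed for a numbered DialogLines function.
; Options allow separate second-visit lines, play-once and requiring two JKid actors inside.
; With PlayOnce, AlreadyPlayed is set before the two-kid check, so a failed check still uses up the trigger.
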(event OnComponentBeginOverlap(Box)
  (params (OverlappedComponent :type Primitive%20Component%20Object%20Reference) (OtherActor :type Actor%20Object%20Reference) (OtherComp :type Primitive%20Component%20Object%20Reference) (OtherBodyIndex :type Integer) (bFromSweep :type Boolean) (SweepResult :type Hit%20Result%20Structure%20%28by%20ref%29))
  (bind _usedifflineson2ndvisit_ (Variables|DialogueInput|GetUseDiffLinesOn2ndVisit?))
  (bind _dialoglines (Variables|DialogueInput:DialogueLinesHolder|GetDialogLines))
  (bind _dialoglines_2 (Variables|DialogueInput:DialogueLinesHolder|GetDialogLines))
  (bind _shouldplay (CallFunction|DetermineifShouldShow))
  (if _shouldplay
    (if (Variables|DialogueInput|GetManualEntryOrDialogLines)
      (if _usedifflineson2ndvisit_
        (if (Variables|Default|Get_AlreadyPlayed)
          (CallFunction|PrintDialog (Variables|DialogueInput:ManualEntry2ndVisit|GetLines2ndVisit) (Variables|DialogueInput:ManualEntry2ndVisit|GetDurations2ndVisit) (Variables|DialogueInput:ManualEntry2ndVisit|GetFonts2ndVisit) (Variables|DialogueInput:ManualEntry2ndvisit|GetCharacters2ndVisit) (Variables|DialogueInput:ManualEntry2ndVisit|GetSplit2ndVisit) false)
          (else
            (CallFunction|PrintDialog (Variables|DialogueInput:ManualEntry|GetLines) (Variables|DialogueInput:ManualEntry|GetDurations) (Variables|DialogueInput:ManualEntry|GetFonts) (Variables|DialogueInput:ManualEntry|GetCharacters) (Variables|DialogueInput:ManualEntry|GetSplit) (Variables|Default|GetPause%20After) :!label _label)
            (Variables|Default|Set_AlreadyPlayed true)))
        (else
          (goto _label)))
      (elif _usedifflineson2ndvisit_
        (if (Variables|Default|Get_AlreadyPlayed)
          (switch int (Variables|DialogueInput:DialogueLinesHolder|GetDialogLinesFunctionNumber2ndVisit)
            (:1
              (Default|Dialog1 _dialoglines_2))
            (:2
              (Default|Dialog2 _dialoglines_2))
            (:3
              (Default|Dialog3 _dialoglines_2))
            (:4
              (Default|Dialog4 _dialoglines_2))
            (:5
              (Default|Dialog5 _dialoglines_2)))
          (else
            (switch int (Variables|DialogueInput:DialogueLinesHolder|GetDialogLinesFunctionNumber) :!label _label_2
              (:1
                (Default|Dialog1 _dialoglines))
              (:2
                (Default|Dialog2 _dialoglines))
              (:3
                (Default|Dialog3 _dialoglines))
              (:4
                (Default|Dialog4 _dialoglines))
              (:5
                (Default|Dialog5 _dialoglines)))
            (Variables|Default|Set_AlreadyPlayed true)))
        (else
          (goto _label_2))))))

(event OnComponentEndOverlap(Box)
  (params (OverlappedComponent :type Primitive%20Component%20Object%20Reference) (OtherActor :type Actor%20Object%20Reference) (OtherComp :type Primitive%20Component%20Object%20Reference) (OtherBodyIndex :type Integer))
  (if (Variables|Default|GetClearOnExit)
    (CallFunction|ClearDialog)))

(event EventBeginPlay
  (bind _outactors (Actor|GetAllActorsOfClass "/Game/Blueprints/UI/JDialogueHandler.JDialogueHandler_C"))
  (if (== (Utilities|Array|Length _outactors) 0)
    (Development|PrintString "PlayDialogOnEnter: ERROR - No Dialog Handler")
    (elif (>= (Utilities|Array|Length _outactors) 2)
      (Development|PrintString "PlayDialogOnEnter: WARNING - >1 Dialog Handlers")
      (else
        (Variables|Default|SetDialogHandlerRef (Utilities|Array|Get(acopy) _outactors))))))

(event Collision|EventActorBeginOverlap
  (params (OtherActor :type Actor%20Object%20Reference)))

(event EventTick
  (params (DeltaSeconds :type Float%20%28single-precision%29)))

(fn ConstructionScript)

(fn PrintDialog
  (params (Lines :type Array%20of%20Strings) (Durations :type Array%20of%20Floats%20%28single-precision%29) (Fonts :type Array%20of%20Integers) (Chars :type Array%20of%20Strings) (Split :type Boolean) (PauseAfter :type Boolean))
  (bind _dialoghandlerref (Variables|Default|GetDialogHandlerRef))
  (Class|DialogueHandler|ToggleSplitMode _dialoghandlerref Split)
  (Class|DialogueHandler|SendNewdialogueSequence _dialoghandlerref Lines Durations Fonts Chars)
  (if PauseAfter
    (Class|DialogueHandler|Pause _dialoghandlerref)))

(fn ClearDialog
  (CallFunction|PrintDialog (Utilities|Array|MakeArray "") (Utilities|Array|MakeArray 0.5) (Utilities|Array|MakeArray 0) (Utilities|Array|MakeArray "") false false))

(fn DetermineifShouldShow
  (if (Variables|Default|GetPlayOnce)
    (if (Variables|Default|Get_AlreadyPlayed)
      (return false)
      (else
        (Variables|Default|Set_AlreadyPlayed true))))
  ;[1 1 1] Both Kids Needed Logic
  (if (Variables|Default|GetBothKidsNeeded)
    (if (== (Utilities|Array|Length (Collision|GetOverlappingActors (Variables|Default|GetBox) "/Script/PlaygroundHeroes.JKid" :!class /Script/Engine.PrimitiveComponent)) 2)
      _
      (else
        (return false))))
  (return true))