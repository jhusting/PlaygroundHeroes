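; ForceMoveLevel is an actor that sends the game to a destination level with set positions for the Archer and Knight.
; While its ACTIVE flag is true, Tick writes both destinations and their flags into the InstanceBlueprint game instance, then opens the level by name.
; BeginPlay caches the Archer and Knight actors and prints warnings if missing, though the move itself does not use these references.
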(event EventBeginPlay
  (CallFunction|FindPlayers))

(event Collision|EventActorBeginOverlap
  (params (OtherActor :type Actor%20Object%20Reference)))

(event EventTick
  (params (DeltaSeconds :type Float%20%28single-precision%29))
  (if (Variables|Default|GetACTIVE)
    (CallFunction|MoveLevelSetLocation (Variables|Default|GetArcherDestinationLocation) (Variables|Default|GetKnightDestinationLocation) (Variables|Default|GetDestinationLevel))))

(event Input|KeyboardEvents|Backspace
  (params (Key :type Key%20Structure)))

(fn ConstructionScript)

(fn MoveLevelSetLocation
  (params (DesiredArcherLocation :type Vector) (DesiredKnightLocation :type Vector) (Level :type Name))
  (bind _asinstance_blueprint (Utilities|Casting|CastToInstanceBlueprint (Game|GetGameInstance)))
  (Variables|/Game/Blueprints/Generic/InstanceBlueprint.InstanceBlueprint_C|SetArcher%20Vector%203 _asinstance_blueprint DesiredArcherLocation)
  (Variables|/Game/Blueprints/Generic/InstanceBlueprint.InstanceBlueprint_C|SetArcher%20Boolean _asinstance_blueprint true)
  (Variables|/Game/Blueprints/Generic/InstanceBlueprint.InstanceBlueprint_C|SetKnight%20Vector%203 _asinstance_blueprint DesiredKnightLocation)
  (Variables|/Game/Blueprints/Generic/InstanceBlueprint.InstanceBlueprint_C|SetKnight%20Boolean _asinstance_blueprint true)
  (Game|OpenLevel(byName) Level))

(fn FindPlayers
  (bind _outactors (Actor|GetAllActorsOfClass "/Game/Blueprints/Warriors/JArcherBP.JArcherBP_C"))
  (Utilities|IsValid (Utilities|Array|Get(acopy) _outactors)
    (:Is%20Valid
      (Variables|Default|SetArcher (Utilities|Array|Get(acopy) _outactors))
      (bind _outactors_2 (Actor|GetAllActorsOfClass "/Game/Blueprints/Warriors/JKnightBP.JKnightBP_C"))
      (Utilities|IsValid (Utilities|Array|Get(acopy) _outactors_2)
        (:Is%20Valid
          (Variables|Default|SetKnight (Utilities|Array|Get(acopy) _outactors_2)))
        (:Is%20Not%20Valid
          (Development|PrintString "ForceMoveLevel: Warning: Knight not found"))))
    (:Is%20Not%20Valid
      (Development|PrintString "ForceMoveLevel: Warning: Archer not found"))))