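; Helper actor that watches Zorrander's Sweet Death attack and cuts it short.
; Every tick it checks whether the victim has fallen, Zorrander's recent-hit list holds an archer crit or the knight's third attack, or its absolute damage build-up reaches a threshold.
; Any of these blends out the Sweet Death montage on Zorrander's mesh and destroys the interruptor.
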(event EventBeginPlay)

(event Collision|EventActorBeginOverlap
  (params (OtherActor :type Actor%20Object%20Reference)))

(event EventTick
  (params (DeltaSeconds :type Float%20%28single-precision%29))
  (bind _zorreference (Variables|Default|GetZorReference))
  (bind _recentlyhitby (Variables|/Script/PlaygroundHeroes.JEnemy|GetRecentlyHitBy _zorreference))
  (if (Math|Boolean|ORBoolean (Variables|/Script/PlaygroundHeroes.JHero|GetbHasFallen (Variables|Default|Getvictim)) (Utilities|Array|ContainsItem _recentlyhitby "ArcherCrit") (Utilities|Array|ContainsItem _recentlyhitby "KnightAttack3") (>= (Math|Float|Absolute(Float) (Variables|/Game/Blueprints/Zorrander/Zorrander.Zorrander_C|GetDamageBuildUp _zorreference)) (Variables|Default|GetCumulativeDamageToInterrupt)))
    (Animation|Montage|MontageStop (Components|SkeletalMesh|GetAnimInstance (Variables|/Script/Engine.Character|GetMesh (Variables|Default|GetZorReference))) 0.3 "/Game/ZorranderAssets/Animations/Sweet_Death_Montage.Sweet_Death_Montage")
    (Actor|DestroyActor)))

(fn ConstructionScript)