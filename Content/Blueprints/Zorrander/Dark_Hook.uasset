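; Dark_Hook is Zorrander's hook actor that reaches toward a hero, stuns it and drags it in.
; Unless a victim is already set, it picks the nearer non-fallen of two JHeroes on spawn, and it blocks Zorrander's blink.
; Tick stretches and aims the beam over a countdown, then lerps the victim toward the hook.
; Coming within range clears Zorrander's casting and resumes his disappear timer; completion unstuns, restores blink and self-destructs.
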(event EventBeginPlay
  (bind _zorranderref (Variables|Default|GetZorranderRef))
  (if (Utilities|IsValid (Variables|Default|Getvictim))
    _
    (else
      (CallFunction|FindVictim)))
  (Variables|Default|SetinitReachTime (Variables|Default|GetreachTime))
  (if (Utilities|IsValid _zorranderref)
    (Variables|/Game/Blueprints/Zorrander/Zorrander.Zorrander_C|SetcanBlink _zorranderref false) ; inelegant, but functional
  ))

(event Collision|EventActorBeginOverlap
  (params (OtherActor :type Actor%20Object%20Reference)))

(event EventTick
  (params (DeltaSeconds :type Float%20%28single-precision%29))
  (bind _victim (Variables|Default|Getvictim))
  (if (Variables|Default|GetpullMode)
    (CallFunction|PullTowards DeltaSeconds)
    (CallFunction|ChangeBeamPulling)
    (if (>= (Variables|Default|GetlerpProgress) 1.0)
      (CallFunction|EndHook))
    (else
      (bind _output_get (Variables|Default|SetreachTime (- (Variables|Default|GetreachTime) DeltaSeconds)))
      (if (<= _output_get 0.0)
        (Variables|Default|SetpullMode true)
        (Class|JHero|Stun (Variables|Default|Getvictim))
        (Variables|Default|SetvictimInitialLocation (Transformation|GetActorLocation _victim))
        (Variables|Default|SetpullTime (/ (Transformation|GetDistanceTo _victim) (Variables|Default|GetpullSpeed)))
        (else
          (CallFunction|ChangeBeamReaching _output_get))))))

(fn ConstructionScript)

(fn PullTowards
  (params (deltaSeconds :type Float%20%28single-precision%29))
  (bind _zorranderref (Variables|Default|GetZorranderRef))
  (bind _output_get (Variables|Default|SettimePassed (+ deltaSeconds (Variables|Default|GettimePassed))))
  (bind _output_get_2 (Variables|Default|SetlerpProgress (/ _output_get (Variables|Default|GetpullTime))))
  (Transformation|SetActorLocation (Variables|Default|Getvictim) (Math|Vector|Lerp(Vector) (Variables|Default|GetvictimInitialLocation) (+ (Transformation|GetActorLocation) (* (Transformation|GetActorForwardVector) "100.000000,100.000000,1.000000")) _output_get_2) false false)
  (if (Utilities|IsValid _zorranderref)
    (if (< (Transformation|GetHorizontalDistanceTo (Variables|Default|Getvictim) _zorranderref) (Variables|/Game/Blueprints/Zorrander/Zorrander.Zorrander_C|GetRange _zorranderref))
      (Variables|/Game/Blueprints/Zorrander/Zorrander.Zorrander_C|SetCasting (Variables|Default|GetZorranderRef) false)
      (Utilities|Time|UnpauseTimerbyHandle (Variables|/Game/Blueprints/Zorrander/Zorrander.Zorrander_C|GetDisappearTimer (Variables|Default|GetZorranderRef))))))

(fn FindVictim
  (bind _outactors (Actor|GetAllActorsOfClass "/Script/PlaygroundHeroes.JHero"))
  (if (== (Utilities|Array|Length _outactors) 2)
    (if (< (Transformation|GetDistanceTo (Utilities|Array|Get(acopy) _outactors)) (Transformation|GetDistanceTo (Utilities|Array|Get(acopy) _outactors 1)))
      (Variables|Default|Setvictim (Utilities|Array|Get(acopy) _outactors))
      (if (Variables|/Script/PlaygroundHeroes.JHero|GetbHasFallen (Variables|Default|Getvictim))
        (Variables|Default|Setvictim (Utilities|Array|Get(acopy) _outactors 1)))
      (else
        (Variables|Default|Setvictim (Utilities|Array|Get(acopy) _outactors 1))
        (if (Variables|/Script/PlaygroundHeroes.JHero|GetbHasFallen (Variables|Default|Getvictim))
          (Variables|Default|Setvictim (Utilities|Array|Get(acopy) _outactors)))))
    (else
      (Actor|DestroyActor))))

(fn ChangeBeamPulling
  (bind _returnvalue (Transformation|GetActorLocation))
  (Transformation|SetWorldScale3D (Variables|Default|Gethook) (Math|Vector|MakeVector (/ (Transformation|GetDistanceTo (Variables|Default|Getvictim)) 1e+02) 0.5 0.5))
  (Transformation|SetWorldLocation (Variables|Default|Gethook) (+ (* (Transformation|GetActorForwardVector) (/ (Transformation|GetDistanceTo (Variables|Default|Getvictim)) 2.0)) _returnvalue) false false)
  (Transformation|SetActorRotation (Math|Rotator|FindLookatRotation _returnvalue (Transformation|GetActorLocation (Variables|Default|Getvictim)))))

(fn ChangeBeamReaching
  (params (reachTime :type Float%20%28single-precision%29))
  (bind _returnvalue (Transformation|GetActorLocation))
  (bind _initreachtime (Variables|Default|GetinitReachTime))
  (bind _returnvalue_2 (- _initreachtime reachTime))
  (bind _returnvalue_3 (/ _returnvalue_2 _initreachtime))
  (Transformation|SetWorldScale3D (Variables|Default|Gethook) (Math|Vector|MakeVector (* _returnvalue_3 (/ (Transformation|GetDistanceTo (Variables|Default|Getvictim)) 1e+02)) 0.5 0.5))
  (Transformation|SetWorldLocation (Variables|Default|Gethook) (+ (* (Transformation|GetActorForwardVector) (* (/ (Transformation|GetDistanceTo (Variables|Default|Getvictim)) 2.0) _returnvalue_3)) _returnvalue) false false)
  (Transformation|SetActorRotation (Math|Rotator|FindLookatRotation _returnvalue (Transformation|GetActorLocation (Variables|Default|Getvictim)))))

(fn EndHook
  (bind _zorranderref (Variables|Default|GetZorranderRef))
  (bind _victim (Variables|Default|Getvictim))
  (if (Variables|/Script/PlaygroundHeroes.JHero|GetbHasFallen _victim)
    _
    (else
      (Class|JHero|UnStun _victim)))
  (if (Utilities|IsValid _zorranderref)
    (Variables|/Game/Blueprints/Zorrander/Zorrander.Zorrander_C|SetcanBlink _zorranderref true))
  (Actor|DestroyActor))