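; Zorrander Jr is a child Blueprint, apparently a junior variant of the Zorrander enemy, that strips down behavior inherited from its parent.
; Parent Tick runs only while BattleReady is true, and PhaseSwitcher and StaminaDrain are empty overrides that disable phase switching and stamina drain.
; GetClosestPlayer and ChooseRandomVictim both return the JHero at the fixed TargetPlayer index, printing a warning if it is missing.
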(event EventBeginPlay
  (|CallParentFunction))

(event Collision|EventActorBeginOverlap
  (params (OtherActor :type Actor%20Object%20Reference))
  (|CallParentFunction OtherActor) ; This node is disabled and will not be called.\nDrag off pins to build functionality.
)

(event EventTick
  (params (DeltaSeconds :type Float%20%28single-precision%29))
  (if (Variables|Default|GetbattleReady)
    (|CallParentFunction DeltaSeconds)))

(event EventPhaseSwitcher)

(event EventStaminaDrain
  (params (DeltaTime :type Float%20%28single-precision%29)))

(fn ConstructionScript
  (|CallParentFunction))

(fn GetClosestPlayer
  (bind _targetplayer (Variables|Default|GettargetPlayer))
  (bind _asjhero (Utilities|Casting|CastToJHero (Game|Player|GetPlayerPawn _targetplayer))
    (:then
      (return _asjhero))
    (:CastFailed
      (Development|PrintString (Utilities|String|Append (Utilities|String|Append (Utilities|String|MakeLiteralString "Warning: Player ") (Utilities|String|ToString(Integer) _targetplayer)) " missing!")))))

(fn ChooseRandomVictim
  (bind _targetplayer (Variables|Default|GettargetPlayer))
  (bind _asjhero (Utilities|Casting|CastToJHero (Game|Player|GetPlayerPawn _targetplayer))
    (:then
      (return _asjhero))
    (:CastFailed
      (Development|PrintString (Utilities|String|Append (Utilities|String|Append (Utilities|String|MakeLiteralString "Warning: Player ") (Utilities|String|ToString(Integer) _targetplayer)) " missing!")))))