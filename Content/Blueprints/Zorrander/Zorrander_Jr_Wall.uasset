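; Zorrander Jr. Wall is a mini-boss variant that fights one assigned player and retreats through teleport points in its level zone.
; Once activated, Tick faces or chases that player, queuing attacks up close and casting long-range spells on timers otherwise.
; TeleportBack advances through points tagged by zone and index; past the last, it increments the handler's cleared count and destroys itself.
; Phase switching and stamina drain are overridden as no-ops.
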(event EventBeginPlay
  (|CallParentFunction)
  (Variables|Default|SetdamageAtLastJump (Variables|Default|GetHealth))
  (bind _outactors (Actor|GetAllActorsOfClass "/Game/Blueprints/Zorrander/teleportPoint.teleportPoint_C"))
  (for _array_element _outactors
    (if (and (Variables|/Game/Blueprints/Zorrander/teleportPoint.teleportPoint_C|GetteleportBackPoint _array_element) (Utilities|Name|Equal(Name) (Variables|/Game/Blueprints/Zorrander/teleportPoint.teleportPoint_C|GetlevelZone _array_element) (Variables|Default|GetlevelZone)))
      (Utilities|Array|Add (Variables|Default|GetteleportPoints) _array_element))))

(event Collision|EventActorBeginOverlap
  (params (OtherActor :type Actor%20Object%20Reference))
  (|CallParentFunction OtherActor) ; This node is disabled and will not be called.\nDrag off pins to build functionality.
)

(event EventTick
  (params (DeltaSeconds :type Float%20%28single-precision%29))
  (|CallParentFunction DeltaSeconds)
  (if (Variables|Default|GetbattleReady)
    (Variables|Default|SetmanualCastTimer (+ DeltaSeconds (Variables|Default|GetmanualCastTimer)))
    (bind _closest (CallFunction|GetClosestPlayer))
    (if (and (not (Variables|Default|GetCasting)) (not (Variables|Default|GetSmashing)))
      (Variables|Default|SetClosestHero _closest)
      (if (Math|Boolean|ORBoolean (Variables|Default|GetIsBlinking) (Variables|Default|GetbAttacking) (Variables|Default|GetCasting))
        (CallFunction|RotateTowardsTarget DeltaSeconds (Variables|Default|GetClosestHero) false)
        (else
          (bind _out (CallFunction|IsAnyPlayerinRange))
          (if _out
            (CallFunction|MoveTowardsPlayer (Variables|Default|GetClosestHero))
            (Variables|Default|SetSpellNames (Variables|Default|GetcloseRangeSpells))
            (if (not (Utilities|Time|IsTimerActivebyHandle (Variables|Default|GetAttackTimer)))
              (CallFunction|QueueAttack))
            (else
              (Variables|Default|SetSpellNames (Variables|Default|GetlongRangeSpells))
              (if (not (or (Utilities|Time|IsTimerActivebyHandle (Variables|Default|GetCastTimer)) (< (Variables|Default|GetmanualCastTimer) 3.0)))
                (Variables|Default|SetmanualCastTimer 0.0)
                (CallFunction|CastSpell)))))))))

(event EventPhaseSwitcher)

(event EventStaminaDrain
  (params (DeltaTime :type Float%20%28single-precision%29)))

(fn ConstructionScript
  (|CallParentFunction))

(fn GetClosestPlayer
  (bind _targetplayer (Variables|Default|GettargetPlayer))
  (bind _asjhero (Utilities|Casting|CastToJHero (Game|Player|GetPlayerPawn _targetplayer))
    (:then
      (return _asjhero))
    (:CastFailed
      (Development|PrintString (Utilities|String|Append (Utilities|String|Append (Utilities|String|MakeLiteralString "Warning: Player ") (Utilities|String|ToString(Integer) _targetplayer)) " missing!")))))

(fn ChooseRandomVictim
  (bind _targetplayer (Variables|Default|GettargetPlayer))
  (bind _asjhero (Utilities|Casting|CastToJHero (Game|Player|GetPlayerPawn _targetplayer))
    (:then
      (return _asjhero))
    (:CastFailed
      (Development|PrintString (Utilities|String|Append (Utilities|String|Append (Utilities|String|MakeLiteralString "Warning: Player ") (Utilities|String|ToString(Integer) _targetplayer)) " missing!")))))

(fn TeleportBack
  (bind _currentpoint (Variables|Default|GetcurrentPoint))
  (bind _levelzone (Variables|Default|GetlevelZone))
  (bind _teleportpoints (Variables|Default|GetteleportPoints))
  (bind _returnvalue (Utilities|String|ToString(Name) _levelzone))
  (bind _returnvalue_2 (Utilities|String|ToString(Integer) _currentpoint))
  (bind _returnvalue_3 (Utilities|String|Append _returnvalue _returnvalue_2))
  (bind _returnvalue_4 (Utilities|String|MakeLiteralString _returnvalue_3))
  (bind _result (Math|Integer|IncrementInt (Variables|Default|GetcurrentPoint))
    (:%20%20
      (if (> _result (Utilities|Array|Length _teleportpoints))
        (CallFunction|Defeated)
        (else
          (bind _array_element (Utilities|Array|ForEachLoopwithBreak _teleportpoints :!label _label)
            (:LoopBody
              (if (Actor|ActorHasTag _array_element (Utilities|String|StringToName _returnvalue_4))
                (Variables|Default|SetManualTPPoint (Transformation|GetActorLocation _array_element))
                (CallFunction|Disappear true)
                (Development|PrintString "teleportCalled")
                (goto _label Break)))
            (:Completed
              (Development|PrintString _returnvalue_4))))))))

(fn Defeated
  (Math|Integer|IncrementInt (Variables|/Game/Blueprints/Zorrander/Zorrander_Jr_Handler.Zorrander_Jr_Handler_C|GetminiZorsCleared (Variables|Default|Gethandler))
    (:%20%20
      (Actor|DestroyActor))))

(fn BattleActivate
  (bind _currentpoint (Variables|Default|GetcurrentPoint))
  (bind _levelzone (Variables|Default|GetlevelZone))
  (bind _returnvalue (Utilities|String|ToString(Name) _levelzone))
  (bind _returnvalue_2 (Utilities|String|ToString(Integer) _currentpoint))
  (bind _returnvalue_3 (Utilities|String|Append _returnvalue _returnvalue_2))
  (bind _returnvalue_4 (Utilities|String|MakeLiteralString _returnvalue_3))
  (bind _outactors (Actor|GetAllActorsOfClass "/Game/Blueprints/Zorrander/Zorrander_Jr_Handler.Zorrander_Jr_Handler_C"))
  (Variables|Default|Sethandler (Utilities|Array|Get(acopy) _outactors))
  (Variables|Default|SetbattleReady true)
  (Math|Integer|IncrementInt (Variables|Default|GetcurrentPoint)
    (:%20%20
      (bind _array_element (Utilities|Array|ForEachLoopwithBreak (Variables|Default|GetteleportPoints))
        (:LoopBody
          (if (Actor|ActorHasTag _array_element (Utilities|String|StringToName _returnvalue_4))
            (Transformation|SetActorLocation (Transformation|GetActorLocation _array_element) false true)))
        (:Completed
          (Development|PrintString _returnvalue_4))))))