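; Growing damage zone actor that deals periodic damage to overlapping JHero characters and expands in scale while occupied.
; Each entering hero gets a looping one-second timer, bound by name to an index-specific DoDamage function (only two exist), and cleared on exit.
; After an activation delay, Tick linearly increases the root's scale magnitude while any damage timer is held.
; Damage timers start on overlap regardless of activation.
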(event EventBeginPlay
  (Utilities|Time|SetTimerbyFunctionName 0 "Activate" (Variables|Default|GetActivateTime)))

(event EventTick
  (params (DeltaSeconds :type Float%20%28single-precision%29))
  (if (and (> (Utilities|Array|Length (Variables|Default|GetDamageHandles)) 0) (Variables|Default|GetbActive))
    (CallFunction|LinearGrow DeltaSeconds)))

(event Collision|EventActorBeginOverlap
  (params (OtherActor :type Actor%20Object%20Reference))
  (bind _asjhero (Utilities|Casting|CastToJHero OtherActor))
  (if (== (Utilities|Array|FindItem (Variables|Default|GetHeroes) _asjhero) -1)
    (bind _returnvalue (Utilities|Array|Add (Variables|Default|GetHeroes) _asjhero))
    (bind _returnvalue_2 (Utilities|Time|SetTimerbyFunctionName 0 (Utilities|String|Append "DoDamage" (Utilities|String|ToString(Integer) _returnvalue)) 1.0 true))
    (Utilities|Array|Insert (Variables|Default|GetDamageHandles) _returnvalue_2 _returnvalue)))

(event Collision|EventActorEndOverlap
  (params (OtherActor :type Actor%20Object%20Reference))
  (bind _asjhero (Utilities|Casting|CastToJHero OtherActor))
  (if (!= (Utilities|Array|FindItem (Variables|Default|GetHeroes) _asjhero) -1)
    (Development|PrintString (Utilities|String|ToString(Integer) (Utilities|Array|FindItem (Variables|Default|GetHeroes) _asjhero)))
    (Utilities|Time|ClearandInvalidateTimerbyHandle (Utilities|Array|Get(acopy) (Variables|Default|GetDamageHandles) (Utilities|Array|FindItem (Variables|Default|GetHeroes) _asjhero)))
    (Utilities|Array|RemoveIndex (Variables|Default|GetDamageHandles) (Utilities|Array|FindItem (Variables|Default|GetHeroes) _asjhero))
    (Utilities|Array|RemoveIndex (Variables|Default|GetHeroes) (Utilities|Array|FindItem (Variables|Default|GetHeroes) _asjhero))))

(fn ConstructionScript)

(fn DoDamage0
  (bind _heroes (Variables|Default|GetHeroes))
  (bind _output (Utilities|Array|Get(acopy) _heroes))
  (if (Utilities|IsValid _output)
    (Class|JHero|AddHealth _output (* -1.0 (Variables|Default|GetDamage)))))

(fn DoDamage1
  (bind _heroes (Variables|Default|GetHeroes))
  (bind _output (Utilities|Array|Get(acopy) _heroes 1))
  (if (Utilities|IsValid _output)
    (Class|JHero|AddHealth _output (* -1.0 (Variables|Default|GetDamage)))))

(fn LinearGrow
  (params (dTime :type Float%20%28single-precision%29))
  (Transformation|SetWorldScale3D (Variables|Default|GetDefaultSceneRoot) (* (Math|Vector|Normalize (Transformation|GetWorldScale (Variables|Default|GetDefaultSceneRoot))) (+ (Math|Float|Sqrt (Math|Vector|VectorLengthSquared (Transformation|GetWorldScale (Variables|Default|GetDefaultSceneRoot)))) (* (Variables|Default|GetGrowthRate) dTime)))))

(fn Activate
  (Variables|Default|SetbActive true))