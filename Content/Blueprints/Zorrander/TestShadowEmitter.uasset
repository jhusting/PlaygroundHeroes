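; Enemy character that stalks JHero players, blinking in a burst of shadow particles when none stay within range.
; Tick usually steers it toward a sweet-spot distance from the closest player and runs the blink check.
; Timers drive vanishing, reappearing at a random line-traced point around that player, and a looping flag-only melee attack.
; CastSpell picks a random spell function by name, though nothing here calls it.
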(event OnSystemFinished(Shadowos)
  (params (PSystem :type Particle%20System%20Component%20Object%20Reference))
  (Components|Activation|SetActive (Variables|Default|GetShadowos) false true))

(event EventBeginPlay
  (|CallParentFunction)
  (Utilities|FlowControl|Delay 0.2)
  (bind _outactors (Actor|GetAllActorsOfClass "/Script/PlaygroundHeroes.JHero"))
  (Variables|Default|SetPlayers _outactors)
  (CallFunction|QueueAttack))

(event Collision|EventActorBeginOverlap
  (params (OtherActor :type Actor%20Object%20Reference)))

(event EventTick
  (params (DeltaSeconds :type Float%20%28single-precision%29))
  (|CallParentFunction DeltaSeconds)
  (CallFunction|TestforBlink)
  (if (Math|Boolean|ANDBoolean (Variables|Default|GetIsBlinking) (Variables|Default|GetCasting) (Variables|Default|GetbAttacking))
    (bind _closest (CallFunction|GetClosestPlayer))
    (CallFunction|RotateTowardsTarget DeltaSeconds _closest)
    (else
      (bind _closest_2 (CallFunction|GetClosestPlayer))
      (CallFunction|MoveTowardsPlayer _closest_2))))

(fn ConstructionScript)

(fn MakeShadows
  (Components|Activation|Activate (Variables|Default|GetShadowos) true))

(fn IsAnyPlayerinRange
  (bind _closest (CallFunction|GetClosestPlayer))
  (return (< (Transformation|GetDistanceTo _closest) (Variables|Default|GetMinDist))))

(fn Disappear
  (Variables|Default|SetIsBlinking true)
  (CallFunction|MakeShadows)
  (Rendering|SetVisibility (Variables|Character|GetMesh) false true)
  (Utilities|Time|SetTimerbyFunctionName 0 "Reappear" 3.0)
  (Utilities|Time|PauseTimerbyHandle (Variables|Default|GetAttackTimer)))

(fn Reappear
  (bind _closest (CallFunction|GetClosestPlayer))
  (LocalVariables|SetBlinkTarget _closest)
  (if (Utilities|IsValid (LocalVariables|GetBlinkTarget))
    (while (not (LocalVariables|GetPointValid))
      (bind _output_get (LocalVariables|SetBlinkLocation (+ (Math|Vector|RotateVector (* (Transformation|GetActorForwardVector (LocalVariables|GetBlinkTarget)) (Variables|Default|GetRange)) (Math|Rotator|MakeRotator 0.0 0.0 (Math|Random|RandomFloatinRange 0.0 3.6e+02))) (Transformation|GetActorLocation (LocalVariables|GetBlinkTarget)))))
      (bind _returnvalue (Collision|LineTraceByChannel (Transformation|GetActorLocation) _output_get "TraceTypeQuery1" true 0 "None"))
      (LocalVariables|SetPointValid (not _returnvalue)))
    ;[1 1 1] Do the actual blinking once you've figured out a good blink location
    (Transformation|SetActorLocation (LocalVariables|GetBlinkLocation) true true)
    (Transformation|SetActorRotation (Math|Rotator|FindLookatRotation (Transformation|GetActorLocation) (Transformation|GetActorLocation (LocalVariables|GetBlinkTarget))))
    (Variables|Default|SetIsBlinking false)
    (Rendering|SetVisibility (Variables|Character|GetMesh) true true)
    (CallFunction|MakeShadows)
    (Utilities|Time|SetTimerbyFunctionName 0 "MeleeAttack" 0.2)))

(fn GetClosestPlayer
  ;[1 1 1] PickClosestPlayer
  (for _array_element (Variables|Default|GetPlayers)
    (if (<= (Transformation|GetDistanceTo _array_element) (LocalVariables|GetClosestDistance))
      (LocalVariables|SetClosestPlayer _array_element)
      (LocalVariables|SetClosestDistance (Transformation|GetDistanceTo _array_element))))
  (return (LocalVariables|GetClosestPlayer)))

(fn TestforBlink
  (bind _out (CallFunction|IsAnyPlayerinRange))
  (if (and (not _out) (not (Variables|Default|GetIsBlinking)))
    (if (not (Utilities|Time|IsTimerActivebyHandle (Variables|Default|GetDisappearTimer)))
      (bind _returnvalue (Utilities|Time|SetTimerbyFunctionName 0 "Disappear" 1.7))
      (Variables|Default|SetDisappearTimer _returnvalue))
    (elif (and _out (not (Variables|Default|GetIsBlinking)))
      (Utilities|Time|ClearandInvalidateTimerbyHandle (Variables|Default|GetDisappearTimer)))))

(fn MeleeAttack
  (Variables|Default|SetbAttacking true))

(fn QueueAttack
  (Utilities|Time|ClearandInvalidateTimerbyHandle (Variables|Default|GetAttackTimer))
  (bind _returnvalue (Utilities|Time|SetTimerbyFunctionName 0 "MeleeAttack" (Variables|Default|GetAttackSpeed) true))
  (Variables|Default|SetAttackTimer _returnvalue))

(fn CastSpell
  (Utilities|Time|SetTimerbyFunctionName 0 (Utilities|Array|Get(acopy) (Variables|Default|GetSpellNames) (Math|Random|RandomIntegerinRange 0 (- (Utilities|Array|Length (Variables|Default|GetSpellNames)) 1))) 0.3))

(fn DarkHook
  (Game|SpawnActorfromClass "/Game/Blueprints/Zorrander/Dark_Hook.Dark_Hook_C" (Transformation|GetActorTransform) "Undefined" 0 0)
  (Development|PrintString "Dark Hook")
  (CallFunction|QueueAttack))

(fn EvilOrb
  (Animation|Montage|MontagePlay (Components|SkeletalMesh|GetAnimInstance (Variables|Character|GetMesh)) "/Game/ZorranderAssets/Animations/OrbMontage.OrbMontage" 0.4 "MontageLength" 0.0 true)
  (Development|PrintString "Evil Orb")
  (CallFunction|QueueAttack))

(fn DarkBolt
  (Game|SpawnActorfromClass "/Game/Blueprints/Zorrander/Dark_Bolt.Dark_Bolt_C" (Transformation|GetActorTransform) "Undefined" 0 0)
  (Development|PrintString "Dark Bolt")
  (CallFunction|QueueAttack))

(fn MoveTowardsPlayer
  (params (Target :type J%20Hero%20Object%20Reference))
  (bind _returnvalue (Transformation|GetActorRotation))
  (bind (_roll _pitch) (Math|Rotator|BreakRotator _returnvalue))
  (if (Utilities|IsValid Target)
    (LocalVariables|SetPlayer Target)
    (LocalVariables|SetDiff (- (Transformation|GetActorLocation Target) (Transformation|GetActorLocation)))
    (LocalVariables|SetSweetSpotRange (* 0.8 (Variables|Default|GetRange)))
    (Transformation|SetActorRotation (Math|Rotator|Lerp(Rotator) _returnvalue (Math|Rotator|MakeRotator _roll _pitch (.Yaw (Math|Rotator|BreakRotator (Math|Rotator|FindLookatRotation (Transformation|GetActorLocation) (Transformation|GetActorLocation (LocalVariables|GetPlayer)))))) 0.2))
    (if (not (<= (Math|Float|Absolute(Float) (- (Math|Vector|VectorLength (LocalVariables|GetDiff)) (LocalVariables|GetSweetSpotRange))) 25.0))
      (if (< (Math|Vector|VectorLength (LocalVariables|GetDiff)) (LocalVariables|GetSweetSpotRange))
        (Class|PawnMovementComponent|AddInputVector (Variables|Character|GetCharacterMovement) (* (Math|Vector|Normalize (LocalVariables|GetDiff)) -0.2) false)
        (else
          (Class|PawnMovementComponent|AddInputVector (Variables|Character|GetCharacterMovement) (* (Math|Vector|Normalize (LocalVariables|GetDiff)) 0.2) false))))))