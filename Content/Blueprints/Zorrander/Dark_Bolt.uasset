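; Dark Bolt is a homing projectile that chases a JHero, picking one at random if no victim is set.
; Overlapping a standing hero hides the bolt and, unless they are dodging, applies damage and stagger.
; Tick then pushes the victim along the bolt's forward vector, using line traces to stop at walls, before unstunning them and destroying itself.
; Hitting static meshes destroys the bolt unless it is pushing.
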(event OnProjectileStop(ProjectileMovement)
  (params (ImpactResult :type Hit%20Result%20Structure%20%28by%20ref%29))
  (Actor|DestroyActor))

(event OnComponentBeginOverlap(Capsule)
  (params (OverlappedComponent :type Primitive%20Component%20Object%20Reference) (OtherActor :type Actor%20Object%20Reference) (OtherComp :type Primitive%20Component%20Object%20Reference) (OtherBodyIndex :type Integer) (bFromSweep :type Boolean) (SweepResult :type Hit%20Result%20Structure%20%28by%20ref%29))
  (bind _asjhero (Utilities|Casting|CastToJHero OtherActor))
  (if (not (Variables|/Script/PlaygroundHeroes.JHero|GetbHasFallen _asjhero))
    (Variables|Default|Setvictim _asjhero)
    (CallFunction|KnockbackHit)
    (Components|DestroyComponent (Variables|Default|GetCapsule))
    (Rendering|SetActorHiddenInGame true)))

(event OnComponentHit(Cylinder)
  (params (HitComponent :type Primitive%20Component%20Object%20Reference) (OtherActor :type Actor%20Object%20Reference) (OtherComp :type Primitive%20Component%20Object%20Reference) (NormalImpulse :type Vector :default "0, 0, 0") (Hit :type Hit%20Result%20Structure%20%28by%20ref%29))
  (Utilities|Casting|CastToStaticMeshActor OtherActor)
  (if (not (Variables|Default|Getpushing))
    (Actor|DestroyActor)))

(event OnComponentHit(Sphere)
  (params (HitComponent :type Primitive%20Component%20Object%20Reference) (OtherActor :type Actor%20Object%20Reference) (OtherComp :type Primitive%20Component%20Object%20Reference) (NormalImpulse :type Vector :default "0, 0, 0") (Hit :type Hit%20Result%20Structure%20%28by%20ref%29))
  (Utilities|Casting|CastToStaticMeshActor OtherActor)
  (if (not (Variables|Default|Getpushing))
    (Actor|DestroyActor)))

(event EventBeginPlay
  (bind _projectilemovement (Variables|Default|GetProjectileMovement))
  (if (Utilities|IsValid (Variables|Default|Getvictim))
    _
    (else
      (CallFunction|RandomVictim)))
  (Variables|/Script/Engine.ProjectileMovementComponent|SetbIsHomingProjectile (Variables|Default|GetProjectileMovement) true)
  (Variables|/Script/Engine.ProjectileMovementComponent|SetHomingTargetComponent _projectilemovement (Variables|/Script/Engine.Character|GetCapsuleComponent (Variables|Default|Getvictim)))
  (Variables|/Script/Engine.ProjectileMovementComponent|SetProjectileGravityScale _projectilemovement 0.0)
  (Variables|/Script/Engine.MovementComponent|SetVelocity _projectilemovement "0, 0, 0")
  (Variables|/Script/Engine.ProjectileMovementComponent|SetMaxSpeed _projectilemovement (Variables|Default|GetMaxSpeed))
  (Variables|/Script/Engine.ProjectileMovementComponent|SetHomingAccelerationMagnitude _projectilemovement (Variables|Default|GethomingSpped)))

(event Collision|EventActorBeginOverlap
  (params (OtherActor :type Actor%20Object%20Reference)))

(event EventTick
  (params (DeltaSeconds :type Float%20%28single-precision%29))
  (bind _victim (Variables|Default|Getvictim))
  (if (Variables|Default|Getpushing)
    (CallFunction|LerptoKnockback DeltaSeconds)
    (if (>= (Variables|Default|GetcountUp) (Variables|Default|GetpushTime))
      (if (Variables|/Script/PlaygroundHeroes.JHero|GetbHasFallen _victim)
        _
        (else
          (Class|JHero|UnStun _victim)))
      (Actor|DestroyActor))))

(fn ConstructionScript)

(fn LerptoKnockback
  (params (deltaSeconds :type Float%20%28single-precision%29))
  (bind _forwardvectorofhit (Variables|Default|GetforwardVectorOfHit))
  (bind _victim (Variables|Default|Getvictim))
  (bind _pushtime (Variables|Default|GetpushTime))
  (bind _pushdistance (Variables|Default|GetpushDistance))
  (bind _returnvalue (Transformation|GetActorLocation _victim))
  (bind _returnvalue_2 (/ _pushdistance _pushtime))
  (bind _returnvalue_3 (* deltaSeconds _returnvalue_2))
  (bind _returnvalue_4 (* _forwardvectorofhit _returnvalue_3))
  (Variables|Default|SetcountUp (+ (Variables|Default|GetcountUp) deltaSeconds))
  (bind _output_get (LocalVariables|SetpushToLocation (+ _returnvalue (Math|Vector|MakeVector (.x _returnvalue_4) (.y _returnvalue_4) 0.0))))
  (bind (_outhit _returnvalue_5) (Collision|LineTraceByChannel _returnvalue _output_get "TraceTypeQuery1" false (Utilities|Array|MakeArray (Variables|Default|Getvictim)) "None"))
  (if _returnvalue_5 ; If Victim would be push inside a wall, push them to the wall instead
    (bind _output_get_2 (LocalVariables|SetpushToLocation (.location _outhit)))
    (Transformation|SetActorLocation (Variables|Default|Getvictim) _output_get_2 false false)
    (else
      (Transformation|SetActorLocation (Variables|Default|Getvictim) (LocalVariables|GetpushToLocation) false false))))

(fn KnockbackHit
  (bind _victim (Variables|Default|Getvictim))
  (if (not (Variables|/Script/PlaygroundHeroes.JHero|GetbDodging _victim))
    (Class|JHero|AddHealth _victim (Variables|Default|Getdamage) (Variables|Default|GetpushTime))
    (Variables|Default|Setpushing true)
    (Variables|Default|SetforwardVectorOfHit (Transformation|GetActorForwardVector))))

(fn RandomVictim
  (Development|PrintString "Bolt gets target")
  (bind _outactors (Actor|GetAllActorsOfClass "/Script/PlaygroundHeroes.JHero"))
  (bind _output_get (Variables|Default|Setvictim (Utilities|Array|Get(acopy) _outactors (Math|Random|RandomInteger (Utilities|Array|Length _outactors)))))
  ;[1 1 1] If random victim has fallen, get the other player
  (if (Variables|/Script/PlaygroundHeroes.JHero|GetbHasFallen _output_get)
    (if (== (Math|Random|RandomInteger (Utilities|Array|Length _outactors)) 0)
      (Variables|Default|Setvictim (Utilities|Array|Get(acopy) _outactors 1))
      (else
        (Variables|Default|Setvictim (Utilities|Array|Get(acopy) _outactors))))))