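; Baleful Grasp dummy caster that repeatedly targets one of two JHero players with the grasp attack while both are standing.
; Tick, gated by BalefulGraspActive, picks a random victim after a delay and spawns a Baleful_Grasp_Helper on them.
; Distant victims trigger a blink: it vanishes with a shadow effect, then reappears at a trace-validated random point around the victim.
; Facing changes only yaw, avoiding tilt as the victim lifts.
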(event EventBeginPlay
  (|CallParentFunction)
  (Utilities|FlowControl|Delay 0.2)
  (bind _asjhero (Utilities|Casting|CastToJHero (Game|Player|GetPlayerPawn 0)))
  (Utilities|Array|AddUnique (Variables|Default|GetPlayers) _asjhero)
  (bind _asjhero_2 (Utilities|Casting|CastToJHero (Game|Player|GetPlayerPawn 1)))
  (Utilities|Array|AddUnique (Variables|Default|GetPlayers) _asjhero_2))

(event Collision|EventActorBeginOverlap
  (params (OtherActor :type Actor%20Object%20Reference))
  (|CallParentFunction OtherActor) ; This node is disabled and will not be called.\nDrag off pins to build functionality.
)

(event EventTick
  (params (DeltaSeconds :type Float%20%28single-precision%29))
  (|CallParentFunction DeltaSeconds)
  (if (not (Variables|Default|GetbalefulGraspActive))
    (Utilities|FlowControl|Delay 2.0)
    (CallFunction|BalefulGrasp)))

(fn ConstructionScript
  (|CallParentFunction))

(fn ChooseRandomVictim
  (bind _players (Variables|Default|GetPlayers))
  (bind _players_2 (Variables|Default|GetPlayers))
  (bind _returnvalue (Utilities|Array|Length _players))
  (bind _returnvalue_2 (Math|Random|RandomInteger _returnvalue))
  (bind _output (Utilities|Array|Get(acopy) _players _returnvalue_2))
  (if (not (Variables|/Script/PlaygroundHeroes.JHero|GetbHasFallen _output)) ; if player has not fallen
    (return _output)
    (elif (== _returnvalue_2 0)
      (return (Utilities|Array|Get(acopy) _players_2 1))
      (else
        (return (Utilities|Array|Get(acopy) _players_2))))))

(fn Reappear
  (bind _returnvalue (Transformation|GetActorRotation))
  (bind (_roll _pitch) (Math|Rotator|BreakRotator _returnvalue))
  (LocalVariables|SetBlinkTarget (Variables|Default|GetCurrentVictim))
  (if (Utilities|IsValid (LocalVariables|GetBlinkTarget))
    (while (not (LocalVariables|GetPointValid))
      (bind _output_get (LocalVariables|SetBlinkLocation (+ (Math|Vector|RotateVector (* (Transformation|GetActorForwardVector (LocalVariables|GetBlinkTarget)) (Variables|Default|GetRange)) (Math|Rotator|MakeRotator 0.0 0.0 (Math|Random|RandomFloatinRange 0.0 3.6e+02))) (Transformation|GetActorLocation (LocalVariables|GetBlinkTarget)))))
      (bind _returnvalue_2 (Collision|LineTraceByChannel (Transformation|GetActorLocation) _output_get "TraceTypeQuery1" true 0 "None"))
      (LocalVariables|SetPointValid (not _returnvalue_2)))
    ;[1 1 1] Do the actual blinking once you've figured out a good blink location
    (Transformation|SetActorLocation (LocalVariables|GetBlinkLocation) true true)
    (Transformation|SetActorRotation (Math|Rotator|MakeRotator _roll _pitch (.Yaw (Math|Rotator|BreakRotator (Math|Rotator|FindLookatRotation (Transformation|GetActorLocation) (Transformation|GetActorLocation (Variables|Default|GetCurrentVictim)))))))
    (Variables|Default|SetIsBlinking false)
    (Rendering|SetVisibility (Variables|Default|GetSkeletalMesh) true false)
    (CallFunction|MakeShadows)))

(fn Dissapear
  (Variables|Default|SetIsBlinking true)
  (CallFunction|MakeShadows)
  (Rendering|SetVisibility (Variables|Default|GetSkeletalMesh) false false)
  (Utilities|Time|SetTimerbyFunctionName 0 "Reappear" 1.0))

(fn MakeShadows
  (Components|Activation|Activate (Variables|Default|Getshadows) true))

(fn BalefulGrasp
  (bind _returnvalue (Transformation|GetActorRotation))
  (bind _players (Variables|Default|GetPlayers))
  (bind (_roll _pitch) (Math|Rotator|BreakRotator _returnvalue))
  (if (not (or (Variables|/Script/PlaygroundHeroes.JHero|GetbHasFallen (Utilities|Array|Get(acopy) _players)) (Variables|/Script/PlaygroundHeroes.JHero|GetbHasFallen (Utilities|Array|Get(acopy) _players 1)))) ; don't do this attack if either have fallen
    (if (not (Variables|Default|GetisBlinking))
      (bind _graspvictim (CallFunction|ChooseRandomVictim))
      (if (Utilities|IsValid _graspvictim)
        (bind _output_get (Variables|Default|SetCurrentVictim _graspvictim))
        (Variables|Default|SetbalefulGraspActive true)
        (if (>= (Transformation|GetDistanceTo _output_get) (LocalVariables|GetgraspNeedTeleportRange))
          (CallFunction|Dissapear)
          (Game|SpawnActorfromClass "/Game/Blueprints/Zorrander/Baleful_Grasp_Helper.Baleful_Grasp_Helper_C" (Transformation|GetActorTransform (Variables|Default|GetCurrentVictim)) "Undefined" 0 (Variables|Default|GetCurrentVictim) self 1e+01 1.0 0)
          (else
            (Transformation|SetActorRotation (Math|Rotator|MakeRotator _roll _pitch (.Yaw (Math|Rotator|BreakRotator (Math|Rotator|FindLookatRotation (Transformation|GetActorLocation) (Transformation|GetActorLocation (Variables|Default|GetCurrentVictim)))))))
            (Game|SpawnActorfromClass "/Game/Blueprints/Zorrander/Baleful_Grasp_Helper.Baleful_Grasp_Helper_C" (Transformation|GetActorTransform (Variables|Default|GetCurrentVictim)) "Undefined" 0 (Variables|Default|GetCurrentVictim) self 1e+01 0.0 0)))))))