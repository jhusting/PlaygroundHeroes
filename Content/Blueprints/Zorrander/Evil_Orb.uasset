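; Evil orb hazard that swells over time, then explodes to damage any JHero caught in the blast; it is destroyed without exploding if its health runs out.
; Tick grows the sphere until DetonateTime, then shrinks SubSphere as a warning countdown.
; Below the threshold, it plays a sound, expands ExplosionSphere for overlap damage and spawns particles, repeating each tick until the delayed destroy.
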(event OnComponentBeginOverlap(explosionSphere)
  (params (OverlappedComponent :type Primitive%20Component%20Object%20Reference) (OtherActor :type Actor%20Object%20Reference) (OtherComp :type Primitive%20Component%20Object%20Reference) (OtherBodyIndex :type Integer) (bFromSweep :type Boolean) (SweepResult :type Hit%20Result%20Structure%20%28by%20ref%29))
  (bind _asjhero (Utilities|Casting|CastToJHero OtherActor))
  (Class|JHero|AddHealth _asjhero (* (Variables|Default|Getdamage) -1.0) 0.0))

(event EventBeginPlay
  (|CallParentFunction) ; This node is disabled and will not be called.\nDrag off pins to build functionality.
)

(event Collision|EventActorBeginOverlap
  (params (OtherActor :type Actor%20Object%20Reference))
  (|CallParentFunction OtherActor) ; This node is disabled and will not be called.\nDrag off pins to build functionality.
)

(event EventTick
  (params (DeltaSeconds :type Float%20%28single-precision%29))
  (|CallParentFunction DeltaSeconds)
  (if (<= (Variables|Default|GetHealth) 0.0)
    (Actor|DestroyActor)
    (else
      (bind _output_get (Variables|Default|Settimer (+ DeltaSeconds (Variables|Default|Gettimer))))
      (if (<= _output_get (Variables|Default|GetdetonateTime))
        (Transformation|SetWorldScale3D (Variables|Default|GetSphere) (* (Variables|Default|GetbaseScale) (+ (* (Variables|Default|Gettimer) 1.0) 1.0)))
        (else
          (bind _output_get_2 (Variables|Default|SetwarningTime (- (Variables|Default|GetwarningTime) DeltaSeconds)))
          (Transformation|SetRelativeScale3D (Variables|Default|GetsubSphere) (Math|Conversions|ToVector(Float) _output_get_2))
          (if (not (>= _output_get_2 1.0))
            (Audio|Components|Audio|Play (Variables|Default|GetNUCLEAR_Quick_Impact_Long_Distorted_Tail_stereo) 0.0)
            (CallFunction|CastEXPULOSION!!!!)
            (Utilities|FlowControl|Delay 2.0)
            (Actor|DestroyActor)))))))

(fn ConstructionScript
  (|CallParentFunction)
  (Variables|Default|SetbaseScale (Transformation|GetWorldScale (Variables|Default|GetSphere)))
  (Class|JEnemy|SetHealth 5e+01))

(fn CastEXPULOSION!!!!
  (bind _returnvalue (Transformation|GetActorRotation))
  (bind (_roll _pitch _yaw) (Math|Rotator|BreakRotator _returnvalue))
  (Transformation|SetWorldScale3D (Variables|Default|GetexplosionSphere) (Math|Conversions|ToVector(Float) (Variables|Default|GetExplosionRadius)))
  (Effects|SpawnEmitteratLocation (Variables|Default|GetEXPULOSION!!!) (Transformation|GetActorLocation) (Math|Rotator|MakeRotator _roll (+ _pitch 9e+01) _yaw) (* (Variables|Default|GetbaseScale) (/ (Variables|Default|GetexplosionRadius) 5.0))))