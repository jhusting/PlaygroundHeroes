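; Level dialogue script for the Zorrander story, holding the scripted conversations between Leila, Abigail and Zorrander.
; Events Dialog1 to Dialog4 play the tower approach, tower entry, playground pre-fight and epilogue scenes, while Dialog5 has no scene.
; Each event re-fetches the dialogue handler, as the BeginPlay lookup alone is noted as insufficient.
; Scene functions pass parallel arrays of lines, durations, fonts and speakers to PrintDialog.
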(event EventDialog1
  (CallFunction|GetDialogHandlerReference) ; You need this for some reason, even though it is called in Begin Play
  (CallFunction|TowerApproach))

(event EventDialog2
  (CallFunction|GetDialogHandlerReference) ; You need this for some reason, even though it is called in Begin Play
  (CallFunction|TowerEnter))

(event EventDialog3
  (CallFunction|GetDialogHandlerReference) ; You need this for some reason, even though it is called in Begin Play
  (CallFunction|PlaygroundPreFight))

(event EventDialog4
  (CallFunction|GetDialogHandlerReference) ; You need this for some reason, even though it is called in Begin Play
  (CallFunction|Epilogue))

(event EventDialog5
  (CallFunction|GetDialogHandlerReference) ; You need this for some reason, even though it is called in Begin Play
)

(event EventBeginPlay
  (|CallParentFunction)
  (CallFunction|GetDialogHandlerReference)
  (Utilities|IsValid (Variables|Default|GetDialogueHandler)
    (:Is%20Not%20Valid
      (Development|PrintString (Utilities|String|Append (Utilities|GetDisplayName self) ": Dialog Handler Invalid")))))

(fn ConstructionScript)

(fn TowerApproach
  (Utilities|IsValid (Variables|Default|GetDialogueHandler)
    (:Is%20Valid
      (CallFunction|PrintDialog (Utilities|Array|MakeArray "Here it is, Zorrander's lair... " " we're almost done with our quest, Abigail! Zorrander is weak and has no more monsters to hide behind." "Everyone is counting on us… but as long as we're brave and work together we can defeat him. " " We're going to bring happiness back to the realm.") (Utilities|Array|MakeArray 3.0 4.0 4.0 4.0) (Utilities|Array|MakeArray 1 1 1 1) (Utilities|Array|MakeArray "LEILA" "LEILA" "LEILA" "LEILA") false false))
    (:Is%20Not%20Valid
      (Development|PrintString "INVALID"))))

(fn TowerEnter
  (Utilities|IsValid (Variables|Default|GetDialogueHandler)
    (:Is%20Valid
      (CallFunction|PrintDialog (Utilities|Array|MakeArray "ABIGAIL: But he’s not here!" "LEILA: He’s not? What do you mean he’s not here?" "ABIGAIL: He knew we were coming for him, that’s why he sent his monsters after us. " "ABIGAIL: They were a distraction.... " "ABIGAIL: What he really wanted was to keep us occupied so he could run away..." "LEILA: Well he’s a coward then. We’ll find him, he can’t run for long!" "ABIGAIL: No,it’s a trick! We’ve done exactly what he wanted us to do. " "ABIGAIL: He could be waiting for us somewhere... He’s been watching us and laughing as we walked right into his trap!" "LEILA: *sighs*... Okay, but it doesn’t matter. " "LEILA: He can’t trick us forever. " "LEILA: We’re going to defeat him no matter what. Okay Abigail? " "LEILA: We’re the brave strong heroes, remember? " "LEILA: And heroes never lose... we can’t lose... " "LEILA: I promise we’ll beat Zorrander." "... " "ABIGAIL: Alright... " "ABIGAIL: Leila are you okay? " "ABIGAIL: Calm down it’s just a game, jeez. " "ABIGAIL: Every story has to have the part where the heroes almost lose." "LEILA: Yeah... " "LEILA: sorry I’m fine. Just a little hungry. " "LEILA: C’mon let’s start heading home, it’s getting dark and we should be eating dinner soon.") (Utilities|Array|MakeArray 2.0 3.0 4.0 3.0 4.0 4.0 4.0 5.0 3.0 2.0 2.0 2.0 3.0 4.0 2.0 2.0 3.0 3.0 4.0 3.0 4.0 5.0) (Utilities|Array|MakeArray 2 1 2 2 2 1 2 2 1 1 1 1 1 1 2 2 2 2 2 1 1 1) (Utilities|Array|MakeArray "ABIGAIL" "LEILA" "ABIGAIL" "ABIGAIL" "ABIGAIL" "LEILA" "ABIGAIL" "ABIGAIL" "LEILA" "LEILA" "LEILA" "LEILA" "LEILA" "LEILA" "ABIGAIL" "ABIGAIL" "ABIGAIL" "ABIGAIL" "ABIGAIL" "LEILA" "LEILA" "LEILA") true false))))

(fn PlaygroundPreFight
  (Utilities|IsValid (Variables|Default|GetDialogueHandler)
    (:Is%20Valid
      (CallFunction|PrintDialog (Utilities|Array|MakeArray "ABIGAIL: *whispers* Look...it’s him. " "ABIGAIL: Zorrander has taken over our castle!" "LEILA: Abigail, c’mon, I don’t wanna play anymore. I just want to go home." "ABIGAIL: But we need to defeat the bad guy and save the day, remember? We need to save the kingdom from the curse!" "LEILA: But-" "ZORRANDER: Hello brave heroes. Quite a nice castle you have here, I may take it for myself. " "ZORRANDER: I’m getting rather tired of my tower in the forest." "LEILA: ...You’ve made a huge mistake by setting foot into our castle Zorrander. " "LEILA: This is our territory." "ZORRANDER: *slow sadistic chuckles* Oh but you see, while you two were out frolicing through the forest, " "ZORRANDER: I was here invading your home. " "ZORRANDER: A place that is so bright and full of cheerful memories was the perfect place to plant my curse." "ABIGAIL: No.. you couldn’t have.." "ZORRANDER: I did. The seed of the curse is planted, and it is growing as we speak. " "ZORRANDER: It’s roots will feed off your life and your happiness," "ZORRANDER: slowly sucking out your joy until you feel nothing but fear and despair. " "ZORRANDER: You will be prisoners of your own misery." "LEILA: Don’t listen to him Abigial! We can still stop the curse before it takes over the land! " "LEILA: It’s time to end this Zorrander!" "ZORRANDER: You think you can stop me with your puny weapons? " "ZORRANDER: *laughs* How entertaining. " "ZORRANDER: Oh, I almost forgot. You’re little adventure through the forest wasn’t entirely meaningless. " "ZORRANDER: Yes, through my minions I was able to study you two. I know both your strengths and weaknesses, " "ZORRANDER: and I know your greatest fears.") (Utilities|Array|MakeArray 3.0 3.0 4.0 4.0 2.0 4.0 4.0 4.0 3.0 4.0 3.0 4.0 3.0 4.0 3.0 4.0 3.0 4.0 3.0 3.0 3.0 4.0 4.0 3.0) (Utilities|Array|MakeArray 2 2 1 2 1 2 0 1 1 0 0 0 2 0 0 0 0 1 1 0 0 0 0 0) (Utilities|Array|MakeArray "ABIGAIL" "ABIGAIL" "LEILA" "ABIGAIL" "LEILA" "ABIGAIL" "ZORRANDER" "LEILA" "LEILA" "ZORRANDER" "ZORRANDER" "ZORRANDER" "ABIGAIL" "ZORRANDER" "ZORRANDER" "ZORRANDER" "ZORRANDER" "LEILA" "LEILA" "ZORRANDER" "ZORRANDER" "ZORRANDER" "ZORRANDER" "ZORRANDER") true false))))

(fn Epilogue
  (Utilities|IsValid (Variables|Default|GetDialogueHandler)
    (:Is%20Valid
      (CallFunction|PrintDialog (Utilities|Array|MakeArray "ABIGAIL: It’s over, the kingdom is safe. We’re heroes!" "LEILA: Yup, it was a tough battle but we did it. " "LEILA: Did you have fun on our adventure?" "ABIGAIL: Of course! It was awesome just like all the adventures you used to take us on! " "ABIGAIL: We stopped going on adventures for a while… let’s go on more from now on, ok?" "LEILA: We can go on as many adventures as you want. " "..." "LEILA: Y’know, I think I learned something from Zorrander…" "ABIGAIL: What could you ever learn from that guy?" "LEILA: I learned that even when times get tough we can still make the best of the situation. " "LEILA: We can’t let the negativity bring us down and make us lose hope… that’s what Zorrander would have wanted." "LEILA: So from now on we should always stay positive and remember what makes us happy." "ABIGAIL: You’re right.. We’re heroes, we can make it through anything!" "LEILA: So, you wanna go home now and eat some dinner?" "ABIGAIL: Let’s just stay here a little longer… until the sun goes down.") (Utilities|Array|MakeArray 4.0 4.0 3.0 4.0 4.0 3.0 1.0 3.0 3.0 4.0 4.0 4.0 4.0 3.0 4.0) (Utilities|Array|MakeArray 2 1 1 2 2 1 1 1 2 1 1 1 2 1 2) (Utilities|Array|MakeArray "ABIGAIL" "LEILA" "LEILA" "ABIGAIL" "ABIGAIL" "LEILA" "LEILA" "LEILA" "ABIGAIL" "LEILA" "LEILA" "LEILA" "ABIGAIL" "LEILA" "ABIGAIL") true false))))