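; Helper actor for the boss Zorrander's fireball smash attack, which the player must interrupt before it lands.
; Activate plays a random companion warning, then Tick lerps the meteor particle between two heights while watching Zorrander's recent hits and damage buildup.
; Enough damage or specific hits trigger Cancel, stopping the montage; otherwise Explode resumes it.
; In one boss phase, a timer makes Zorrander invincible behind a barrier and spawns a guarding archer and knight.
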(event EventBeginPlay
  (bind _returnvalue (Transformation|GetActorLocation))
  (bind _returnvalue_2 (Transformation|GetActorLocation))
  (bind (_x _y _z) (Math|Vector|BreakVector _returnvalue))
  (bind (_x_2 _y_2 _z_2) (Math|Vector|BreakVector _returnvalue_2))
  (bind _outactors (Actor|GetAllActorsOfClass "/Game/Blueprints/UI/JDialogueHandler.JDialogueHandler_C"))
  (Variables|Default|SetDialogHandler (Utilities|Array|Get(acopy) _outactors))
  (Rendering|SetVisibility (Variables|Default|Getbarrier) false true)
  (Utilities|FlowControl|Delay 0.5)
  (bind _outactors_2 (Actor|GetAllActorsOfClass "/Game/Blueprints/Zorrander/Zorrander.Zorrander_C"))
  (Variables|Default|SetZorReference (Utilities|Array|Get(acopy) _outactors_2))
  (Variables|Default|SetStartLocation (Math|Vector|MakeVector _x_2 _y_2 (+ _z_2 (Variables|Default|GetStartHeight))))
  (Variables|Default|SetEndLocation (Math|Vector|MakeVector _x _y (+ _z (Variables|Default|GetEndHeight)))))

(event Collision|EventActorBeginOverlap
  (params (OtherActor :type Actor%20Object%20Reference)))

(event EventTick
  (params (DeltaSeconds :type Float%20%28single-precision%29))
  (bind _zorreference (Variables|Default|GetZorReference))
  (bind _recentlyhitby (Variables|/Script/PlaygroundHeroes.JEnemy|GetRecentlyHitBy _zorreference))
  (if (Variables|Default|GetbActive)
    (Variables|Default|SetCurrTime (Math|Float|Clamp(Float) (+ DeltaSeconds (Variables|Default|GetCurrTime)) 0.0 (Variables|Default|GetTravelTime)))
    (Transformation|SetWorldLocation (Variables|Default|GetPar_Meteora_01) (Math|Vector|Lerp(Vector) (Variables|Default|GetStartLocation) (Variables|Default|GetEndLocation) (/ (Variables|Default|GetCurrTime) (Variables|Default|GetTravelTime))) false false)
    (if (Math|Boolean|ORBoolean (Utilities|Array|ContainsItem _recentlyhitby "ArcherCrit") (Utilities|Array|ContainsItem _recentlyhitby "KnightAttack3") (>= (Math|Float|Absolute(Float) (Variables|/Game/Blueprints/Zorrander/Zorrander.Zorrander_C|GetDamageBuildUp _zorreference)) (Variables|Default|GetCumulativeDamageToInterrupt)))
      (CallFunction|Cancel)
      (elif (>= (Variables|Default|GetCurrTime) (Variables|Default|GetTravelTime))
        (CallFunction|Explode)))))

(fn ConstructionScript
  (switch int (Math|Random|RandomIntegerinRange 0 1)
    (:0
      (Variables|Default|SetBreakNoise "/Game/Audio/Dialog/Zorrander_Single_Lines/Damage_Noises/Z__getting_hit_2_moan.Z__getting_hit_2_moan"))
    (:1
      (Variables|Default|SetBreakNoise "/Game/Audio/Dialog/Zorrander_Single_Lines/Damage_Noises/Z__getting_hit_4_ahhh.Z__getting_hit_4_ahhh"))))

(fn Activate
  (params (activeZor :type Zorrander%20Object%20Reference))
  (Variables|Default|SetZorReference activeZor)
  (Variables|Default|SetbActive true)
  (Transformation|SetWorldLocation (Variables|Default|GetCurrentLoc) (Variables|Default|GetStartLocation) false false)
  (Rendering|SetVisibility (Variables|Default|GetPar_Meteora_01) true false)
  (Development|PrintString "should be visible")
  (Variables|Default|SetCurrTime 0.0)
  (CallFunction|MegaSmashSounds)
  (if (Utilities|Enum|Equal(Enum) (Variables|/Game/Blueprints/Zorrander/Zorrander.Zorrander_C|GetCurrentPhase (Variables|Default|GetZorReference)) "NewEnumerator2")
    (Utilities|Time|SetTimerbyFunctionName 0 "spawnGuardingHeroes" 2.0)))

(fn Explode
  (bind _zorreference (Variables|Default|GetZorReference))
  (bind _guardingarcher (Variables|Default|GetguardingArcher))
  (bind _guardingknight (Variables|Default|GetguardingKnight))
  (Variables|Default|SetbActive false)
  (Default|PlaySoundHaHaHa _zorreference)
  (Class|AnimInstance|MontageResume (Components|SkeletalMesh|GetAnimInstance (Variables|/Script/Engine.Character|GetMesh _zorreference)) "/Game/ZorranderAssets/Animations/SmashMontage.SmashMontage")
  (Rendering|SetVisibility (Variables|Default|GetPar_Meteora_01) false false)
  (Rendering|SetVisibility (Variables|Default|Getbarrier) false true)
  (if (Utilities|IsValid _guardingarcher)
    (Default|Die _guardingarcher)
    (if (Utilities|IsValid _guardingknight)
      (Default|Die _guardingknight))))

(fn Cancel
  (bind _zorreference (Variables|Default|GetZorReference))
  (bind _zorreference_2 (Variables|Default|GetZorReference))
  (Variables|Default|SetbActive false)
  (Rendering|SetVisibility (Variables|Default|GetPar_Meteora_01) false false)
  (Variables|/Game/Blueprints/Zorrander/Zorrander.Zorrander_C|SetSmashing _zorreference false)
  (Variables|/Game/Blueprints/Zorrander/Zorrander.Zorrander_C|SetCasting _zorreference false)
  (Animation|Montage|MontageStop (Components|SkeletalMesh|GetAnimInstance (Variables|/Script/Engine.Character|GetMesh (Variables|Default|GetZorReference))) 0.3 "/Game/ZorranderAssets/Animations/SmashMontage.SmashMontage")
  (Audio|PlaySoundatLocation (Variables|Default|GetBreakNoise) (Transformation|GetActorLocation _zorreference_2) "0, 0, 0" (Variables|/Game/Blueprints/Zorrander/Zorrander.Zorrander_C|GetvoiceVolumeMult _zorreference_2) 1.0 0.0 0 0 0)
  (Default|Disappear (Variables|Default|GetZorReference)))

(fn SpawnGuardingHeroes
  (bind _returnvalue (Transformation|GetActorLocation))
  (bind _returnvalue_2 (Transformation|GetActorRotation))
  (bind _returnvalue_3 (Transformation|GetActorRotation))
  (bind _returnvalue_4 (Transformation|GetActorLocation))
  (bind _returnvalue_5 (+ (.yaw _returnvalue_3) -35.0))
  (bind _returnvalue_6 (+ (.yaw _returnvalue_2) 35.0))
  (bind _returnvalue_7 (Math|Vector|GetForwardVector (Math|Rotator|MakeRotator (.roll _returnvalue_3) (.pitch _returnvalue_3) _returnvalue_5)))
  (bind _returnvalue_8 (Math|Vector|GetForwardVector (Math|Rotator|MakeRotator (.roll _returnvalue_2) (.pitch _returnvalue_2) _returnvalue_6)))
  (bind _returnvalue_9 (* _returnvalue_8 5e+02))
  (bind _returnvalue_10 (* _returnvalue_7 5e+02))
  (bind _returnvalue_11 (+ _returnvalue_4 _returnvalue_10))
  (bind _returnvalue_12 (+ _returnvalue _returnvalue_9))
  (Variables|/Game/Blueprints/Enemies/JEnemyBP_Bar.JEnemyBP_Bar_C|Setinvincible (Variables|Default|GetZorReference) true)
  (Variables|Default|SetguardingArcherDead false)
  (bind _returnvalue_13 (Game|SpawnActorfromClass "/Game/Blueprints/Zorrander/SmashArcher.SmashArcher_C" (Math|Transform|MakeTransform (Math|Vector|MakeVector (.x _returnvalue_12) (.y _returnvalue_12) (.z _returnvalue_12)) (Transformation|GetActorRotation)) "Undefined" 0 self 0))
  (Variables|Default|SetguardingArcher _returnvalue_13)
  (Variables|Default|SetguardingKnightDead false)
  (bind _returnvalue_14 (Game|SpawnActorfromClass "/Game/Blueprints/Zorrander/SmashKnight.SmashKnight_C" (Math|Transform|MakeTransform (Math|Vector|MakeVector (.x _returnvalue_11) (.y _returnvalue_11) (.z _returnvalue_11)) (Transformation|GetActorRotation)) "Undefined" 0 self 0))
  (Variables|Default|SetguardingKnight _returnvalue_14)
  (CallFunction|PlaceBarrier))

(fn PlaceBarrier
  (bind _zorreference (Variables|Default|GetZorReference))
  (bind _barrier (Variables|Default|Getbarrier))
  (bind _returnvalue (Transformation|GetActorLocation _zorreference))
  (Rendering|SetVisibility _barrier true true)
  (Transformation|SetWorldLocation _barrier (Math|Vector|MakeVector (.x _returnvalue) (.y _returnvalue) (+ (.z _returnvalue) 2e+01)) false true))

(fn MegaSmashSounds
  (bind _zorreference (Variables|Default|GetZorReference))
  (bind _voicevolumemult (Variables|/Game/Blueprints/Zorrander/Zorrander.Zorrander_C|GetvoiceVolumeMult _zorreference))
  (switch int (Math|Random|RandomIntegerinRange 0 3)
    (:0
      (Audio|PlaySound2D "/Game/Audio/Dialog/Leila_Single_Lines/L__hurry_stop_his_attack.L__hurry_stop_his_attack" _voicevolumemult 1.0 0.0 0 0)
      (LocalVariables|Setline (Utilities|Array|MakeArray "Hurry stop his attack!"))
      (LocalVariables|Setduration (Utilities|Array|MakeArray 2.4))
      (LocalVariables|Setcharacter (Utilities|Array|MakeArray "LEILA")))
    (:1
      (Audio|PlaySound2D "/Game/Audio/Dialog/Leila_Single_Lines/L__hit_him_before_he_attacks_us.L__hit_him_before_he_attacks_us" _voicevolumemult 1.0 0.0 0 0)
      (LocalVariables|Setline (Utilities|Array|MakeArray " Hit him before he attacks us!"))
      (LocalVariables|Setduration (Utilities|Array|MakeArray 2.5))
      (LocalVariables|Setcharacter (Utilities|Array|MakeArray "LEILA")))
    (:2
      (Audio|PlaySound2D "/Game/Audio/Dialog/Abigail_Single_lines/A__look_out_for_the_fireball.A__look_out_for_the_fireball" _voicevolumemult 1.0 0.0 0 0)
      (LocalVariables|Setline (Utilities|Array|MakeArray " Look out for the fireball! "))
      (LocalVariables|Setduration (Utilities|Array|MakeArray 2.2))
      (LocalVariables|Setcharacter (Utilities|Array|MakeArray "ABIGAIL")))
    (:3
      (Audio|PlaySound2D "/Game/Audio/Dialog/Abigail_Single_lines/A__quick____stop_him_from_using_his_fireball.A__quick____stop_him_from_using_his_fireball" _voicevolumemult 1.0 0.0 0 0)
      (LocalVariables|Setline (Utilities|Array|MakeArray "Quick, stop him from using his fireball!"))
      (LocalVariables|Setduration (Utilities|Array|MakeArray 3.05))
      (LocalVariables|Setcharacter (Utilities|Array|MakeArray "ABIGAIL"))))
  (Class|DialogueHandler|SendNewdialogueSequence (Variables|Default|GetDialogHandler) (LocalVariables|Getline) (LocalVariables|Getduration) (Utilities|Array|MakeArray 1) (LocalVariables|Getcharacter)))