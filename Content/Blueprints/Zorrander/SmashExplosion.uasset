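; SmashExplosion is an expanding, short-lived explosion actor that affects JHero characters it touches.
; Each tick lengthens the root component's scale vector by a growth rate while keeping its proportions.
; Beginning an overlap with a JHero sets that hero's Health to a fixed value rather than subtracting damage.
; A timer started on BeginPlay destroys the actor once its lifetime elapses.
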(event EventBeginPlay
  (Utilities|Time|SetTimerbyFunctionName 0 "DestroySelf" (Variables|Default|GetLifeTime)))

(event Collision|EventActorBeginOverlap
  (params (OtherActor :type Actor%20Object%20Reference))
  (bind _asjhero (Utilities|Casting|CastToJHero OtherActor))
  (Variables|/Script/PlaygroundHeroes.JHero|SetHealth _asjhero 5.0))

(event EventTick
  (params (DeltaSeconds :type Float%20%28single-precision%29))
  (Transformation|SetWorldScale3D (Variables|Default|GetDefaultSceneRoot) (* (Math|Vector|Normalize (Transformation|GetWorldScale (Variables|Default|GetDefaultSceneRoot))) (+ (Math|Float|Sqrt (Math|Vector|VectorLengthSquared (Transformation|GetWorldScale (Variables|Default|GetDefaultSceneRoot)))) (* (Variables|Default|GetGrowthRate) DeltaSeconds)))))

(fn ConstructionScript)

(fn DestroySelf
  (Actor|DestroyActor))