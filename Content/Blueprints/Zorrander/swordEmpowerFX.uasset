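; swordEmpowerFX is a short-lived visual effect actor, apparently for empowering Zorrander's sword.
; It records its Sphere component's starting scale on BeginPlay, then each Tick lerps that scale toward the world scale of the sword on the referenced Zor character over LifeTime.
; When the elapsed time reaches LifeTime, the actor destroys itself.
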(event EventBeginPlay
  (Variables|Default|SetstartingScale (Transformation|GetWorldScale (Variables|Default|GetSphere))))

(event Collision|EventActorBeginOverlap
  (params (OtherActor :type Actor%20Object%20Reference)))

(event EventTick
  (params (DeltaSeconds :type Float%20%28single-precision%29))
  (Variables|Default|SettimePassed (+ DeltaSeconds (Variables|Default|GettimePassed)))
  (Transformation|SetWorldScale3D (Variables|Default|GetSphere) (Math|Vector|Lerp(Vector) (Variables|Default|GetstartingScale) (Transformation|GetWorldScale (Variables|/Game/Blueprints/Zorrander/Zorrander.Zorrander_C|GetSword (Variables|Default|GetZorRef))) (/ (Variables|Default|GettimePassed) (Variables|Default|GetlifeTime))))
  (if (>= (Variables|Default|GettimePassed) (Variables|Default|GetlifeTime))
    (Actor|DestroyActor)))

(fn ConstructionScript)