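; Helper actor for the Baleful Grasp spell that stuns a victim, lifts it into the air and drains its health.
; After a short delay it snaps to the victim, plays a random hurt voice and shadow effect.
; Each tick it raises itself and the victim up to a height cap, draining max health over TimeToKill.
; It releases the victim and destroys itself when the victim falls or the caster takes specific hits.
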(event EventBeginPlay
  (Utilities|FlowControl|Delay (Variables|Default|GetdissapearDelay))
  (Variables|/Game/Blueprints/Zorrander/Zorrander.Zorrander_C|SetGrasping (Variables|Default|GetspellCaster) true)
  (CallFunction|GraspStart)
  (Variables|Default|Setready true))

(event EventTick
  (params (DeltaSeconds :type Float%20%28single-precision%29))
  (bind _spellcaster (Variables|Default|GetspellCaster))
  (bind _recentlyhitby (Variables|/Script/PlaygroundHeroes.JEnemy|GetRecentlyHitBy _spellcaster))
  (if (Variables|Default|Getready)
    (if (or (Variables|/Script/PlaygroundHeroes.JHero|GetbHasFallen (Variables|Default|Getvictim)) (or (Utilities|Array|ContainsItem _recentlyhitby "ArcherCrit") (Utilities|Array|ContainsItem _recentlyhitby "KnightAttack3")))
      (CallFunction|GraspEnd)
      (else
        (CallFunction|GraspDamage DeltaSeconds)))))

(fn ConstructionScript)

(fn GraspStart
  (bind _victim (Variables|Default|Getvictim))
  (bind _returnvalue (Transformation|GetActorLocation _victim))
  (if (Utilities|IsValid (Variables|Default|Getvictim))
    (Class|JHero|Stun (Variables|Default|Getvictim))
    (Transformation|SetActorLocation _returnvalue false false)
    (Variables|Default|SetvictimSuspendLocation _returnvalue)
    (switch int (Math|Random|RandomIntegerinRange 0 1)
      (:Default
        (Audio|Components|Audio|Play (Variables|Default|GetVOICE_Girl_4yo_Hurt_Long_01_mono) 0.0 :!label _label))
      (:0
        (goto _label))
      (:1
        (Audio|Components|Audio|Play (Variables|Default|GetVOICE_Girl_4yo_Hurt_Long_02_mono) 0.0)))
    (Components|Activation|Activate (Variables|Default|GetgraspShadows) false)))

(fn GraspEnd
  (bind _spellcaster (Variables|Default|GetspellCaster))
  (Class|JHero|Unstun (Variables|Default|Getvictim))
  (Variables|/Game/Blueprints/Zorrander/Zorrander.Zorrander_C|SetCasting _spellcaster false)
  (Variables|/Game/Blueprints/Zorrander/Zorrander.Zorrander_C|SetGrasping _spellcaster false)
  (Actor|DestroyActor))

(fn GraspDamage
  (params (deltaSeconds :type Float%20%28single-precision%29))
  (bind _victim (Variables|Default|Getvictim))
  (bind _victimsuspendlocation (Variables|Default|GetvictimSuspendLocation))
  (bind (_x _y _z) (Math|Vector|BreakVector _victimsuspendlocation))
  (LocalVariables|SetdeltaTime deltaSeconds)
  (Variables|Default|SettimeHeld (+ deltaSeconds (Variables|Default|GettimeHeld)))
  (Transformation|SetActorLocation (Variables|Default|Getvictim) (Math|Vector|MakeVector _x _y (Math|Float|Clamp(Float) (+ _z (* (Variables|Default|GettimeHeld) 1e+02)) _z (Variables|Default|GetsuspendMaxHeight))) false false)
  (Transformation|SetActorLocation (Math|Vector|MakeVector _x _y (Math|Float|Clamp(Float) (+ _z (* (Variables|Default|GettimeHeld) 1e+02)) _z (Variables|Default|GetsuspendMaxHeight))) false false)
  (Class|JHero|AddHealth _victim (* (/ (Variables|/Script/PlaygroundHeroes.JHero|GetMaxHealth _victim) (Variables|Default|GetTimeToKill)) (* -1.0 (LocalVariables|GetdeltaTime))) 0.0))