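; Arena separation wall actor that sizes itself to the floor and rises vertically into place once play begins.
; On BeginPlay it finds the StaticMeshActor whose mesh component is tagged "floor", then scales its width to that floor's Y bounds and sets a fixed height.
; It derives start and end heights half its scaled height below and above its placed position.
; Tick lerps between them over RiseTime, moving by teleport.
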(event EventBeginPlay
  (bind _outactors (Actor|GetAllActorsOfClass "/Script/Engine.StaticMeshActor"))
  (for _array_element _outactors
    (if (Components|ComponentHasTag (Variables|/Script/Engine.StaticMeshActor|GetStaticMeshComponent _array_element) "floor")
      (Variables|Default|SetArenaFloor _array_element)))
  (CallFunction|CalculateNeededSize)
  (Variables|Default|SetinitZLocation (+ (.z (Transformation|GetActorLocation)) (/ (* (.z (Transformation|GetActorScale3D)) -1e+02) 2.0)))
  (Variables|Default|SetfinalZLocation (+ (.z (Transformation|GetActorLocation)) (/ (* (.z (Transformation|GetActorScale3D)) 1e+02) 2.0))))

(event Collision|EventActorBeginOverlap
  (params (OtherActor :type Actor%20Object%20Reference)))

(event EventTick
  (params (DeltaSeconds :type Float%20%28single-precision%29))
  (bind _returnvalue (Transformation|GetActorLocation))
  (if (not (>= (Variables|Default|GetriseProgress) (Variables|Default|GetriseTime)))
    (Variables|Default|SetriseProgress (+ DeltaSeconds (Variables|Default|GetriseProgress)))
    (Transformation|SetActorLocation (Math|Vector|MakeVector (.x _returnvalue) (.y _returnvalue) (Math|Float|Lerp (Variables|Default|GetinitZLocation) (Variables|Default|GetfinalZLocation) (/ (Variables|Default|GetriseProgress) (Variables|Default|GetriseTime)))) false true)))

(fn ConstructionScript)

(fn CalculateNeededSize
  (bind _arenafloor (Variables|Default|GetArenaFloor))
  (if (Utilities|IsValid _arenafloor)
    (Transformation|SetActorScale3D (Math|Vector|MakeVector (.x (Transformation|GetActorScale3D)) (* (/ (.y (.BoxExtent (Collision|GetActorBounds _arenafloor true))) 1e+02) 2.0) 5.0))))