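; Zorrander sound controller actor for cave ambience music (UneaseDarkCave) and random sound effects.
; PlayRandomSFX picks an SFX array entry and plays it on SoundEffects with randomized pitch and volume.
; Its random index range includes the array length, so it can land out of bounds.
; The music start and looping timer for PlayRandomSFX are disconnected, so nothing in this graph triggers playback.
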(event EventBeginPlay)

(event Collision|EventActorBeginOverlap
  (params (OtherActor :type Actor%20Object%20Reference)))

(event EventTick
  (params (DeltaSeconds :type Float%20%28single-precision%29)))

(fn ConstructionScript)

(fn PlayRandomSFX
  (bind _sfx (Variables|Default|GetSFX))
  (bind _sound_effects (Variables|Default|Getsound%20effects))
  (Audio|Components|Audio|SetSound _sound_effects (Utilities|Array|Get(acopy) _sfx (Math|Random|RandomIntegerinRange 0 (Utilities|Array|Length _sfx))))
  (Audio|Components|Audio|SetPitchMultiplier _sound_effects (Math|Random|RandomFloatinRange 0.5 1.5))
  (Audio|Components|Audio|SetVolumeMultiplier _sound_effects (Math|Random|RandomFloatinRange 1.0 5.0) :!class /Script/Engine.AudioComponent)
  (Audio|Components|Audio|Play _sound_effects 0.0))