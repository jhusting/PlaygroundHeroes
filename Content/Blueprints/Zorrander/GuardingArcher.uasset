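; GuardingArcher is one of two guards, alongside a guarding knight, whose deaths remove the invincibility of Zor.
; On Die, it records its death on SmashHelper and, if the knight is also flagged dead, clears Invincible on the helper's ZorReference.
; It then destroys itself; its other events and construction script add no logic of their own.
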(event EventBeginPlay
  (|CallParentFunction) ; This node is disabled and will not be called.\nDrag off pins to build functionality.
)

(event Collision|EventActorBeginOverlap
  (params (OtherActor :type Actor%20Object%20Reference))
  (|CallParentFunction OtherActor) ; This node is disabled and will not be called.\nDrag off pins to build functionality.
)

(event EventTick
  (params (DeltaSeconds :type Float%20%28single-precision%29))
  (|CallParentFunction DeltaSeconds) ; This node is disabled and will not be called.\nDrag off pins to build functionality.
)

(event EventDie
  (bind _smashhelper (Variables|Default|GetsmashHelper))
  (bind _output_get (Variables|/Game/Blueprints/Zorrander/SmashHelper.SmashHelper_C|SetguardingArcherDead _smashhelper true))
  (if (and _output_get (Variables|/Game/Blueprints/Zorrander/SmashHelper.SmashHelper_C|GetguardingKnightDead _smashhelper))
    (Variables|/Game/Blueprints/Enemies/JEnemyBP_Bar.JEnemyBP_Bar_C|Setinvincible (Variables|/Game/Blueprints/Zorrander/SmashHelper.SmashHelper_C|GetZorReference _smashhelper) false))
  (Actor|DestroyActor))

(fn ConstructionScript
  (|CallParentFunction))