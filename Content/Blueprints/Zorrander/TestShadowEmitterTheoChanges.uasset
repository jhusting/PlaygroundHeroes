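; Test variant of the Zorrander boss, an enemy that stalks JHero players, melees them and drains the focused hero's max stamina.
; Tick picks a target by distance and angle, holds a preferred range, and triggers a vanish-and-teleport when the target stays out of reach.
; Function-name timers drive attacks, blinks and recurring growing damage zones.
; Spells include montage casts, Baleful Grasp via a helper actor, and MegaSmash from the farthest SmashHelper.
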(event OnSystemFinished(Shadowos)
  (params (PSystem :type Particle%20System%20Component%20Object%20Reference))
  (Components|Activation|SetActive (Variables|Default|GetShadowos) false true))

(event OnComponentBeginOverlap(Box)
  (params (OverlappedComponent :type Primitive%20Component%20Object%20Reference) (OtherActor :type Actor%20Object%20Reference) (OtherComp :type Primitive%20Component%20Object%20Reference) (OtherBodyIndex :type Integer) (bFromSweep :type Boolean) (SweepResult :type Hit%20Result%20Structure%20%28by%20ref%29))
  (bind _heroeshit (Variables|Default|GetHeroesHit))
  (if (Variables|Default|GetcanMeleeDamage)
    (bind _asjhero (Utilities|Casting|CastToJHero OtherActor))
    (if (== -1 (Utilities|Array|FindItem _heroeshit _asjhero))
      (Utilities|Array|Add _heroeshit _asjhero)
      (Class|JHero|AddHealth _asjhero (* (Variables|Default|GetMeleeDamage) -1.0))
      (switch int (Math|Random|RandomIntegerinRange 0 2)
        (:Default
          (Audio|Components|Audio|Play (Variables|Default|GetVOICE_Girl_4yo_Hurt_Short_01_mono) 0.0 :!label _label))
        (:0
          (goto _label))
        (:1
          (Audio|Components|Audio|Play (Variables|Default|GetVOICE_Girl_4yo_Hurt_Short_04_mono) 0.0))
        (:2
          (Audio|Components|Audio|Play (Variables|Default|GetVOICE_Girl_4yo_Hurt_Short_06_mono) 0.0))))))

(event EventBeginPlay
  (|CallParentFunction)
  (Utilities|FlowControl|Delay 0.2)
  (bind _outactors (Actor|GetAllActorsOfClass "/Script/PlaygroundHeroes.JHero"))
  (Variables|Default|SetPlayers _outactors)
  (CallFunction|QueueAttack)
  (bind _returnvalue (UserInterface|CreateWidget "/Game/Blueprints/UI/ZorranderHealthBar.ZorranderHealthBar_C"))
  (Variables|/Game/Blueprints/UI/ZorranderHealthBar.ZorranderHealthBar_C|SetBoss _returnvalue self)
  (UserInterface|Viewport|AddtoViewport _returnvalue 0)
  (bind _outactors_2 (Actor|GetAllActorsOfClass "/Game/Blueprints/Zorrander/SmashHelper.SmashHelper_C"))
  (Variables|Default|SetSmashPoints _outactors_2)
  (Utilities|Time|SetTimerbyFunctionName 0 "SpawnGrowZone" 8.0))

(event Collision|EventActorBeginOverlap
  (params (OtherActor :type Actor%20Object%20Reference)))

(event EventTick
  (params (DeltaSeconds :type Float%20%28single-precision%29))
  (|CallParentFunction DeltaSeconds)
  (bind _closest (CallFunction|GetClosestPlayer))
  (CallFunction|StaminaDrain DeltaSeconds)
  (if (Math|Boolean|ANDBoolean (Utilities|IsValid _closest) (not (Variables|Default|GetCasting)) (not (Variables|Default|GetSmashing)))
    (Variables|Default|SetClosestHero _closest)
    (CallFunction|TestforBlink)
    (if (Math|Boolean|ORBoolean (Variables|Default|GetIsBlinking) (Variables|Default|GetbAttacking) (Variables|Default|GetCasting))
      (CallFunction|RotateTowardsTarget DeltaSeconds (Variables|Default|GetClosestHero) false)
      (else
        (CallFunction|MoveTowardsPlayer (Variables|Default|GetClosestHero))
        (if (not (Utilities|Time|IsTimerActivebyHandle (Variables|Default|GetAttackTimer)))
          (CallFunction|QueueAttack))))))

(event EventAddHealthBP
  (params (Change :type Float%20%28single-precision%29) (MoveName :type String))
  ;[1 1 1] This calls JEnemy BP Bar's AddHealthBP function
  (|CallParentFunction Change MoveName)
  (Variables|Default|SetDamageBuildUp%20MOVE%20OVER (+ Change (Variables|Default|GetDamageBuildUp%20MOVE%20OVER)))
  (Utilities|Time|SetTimerbyFunctionName 0 "ResetDamageBuildup" 1.5))

(fn ConstructionScript)

(fn MakeShadows
  (Components|Activation|Activate (Variables|Default|GetShadowos) true))

(fn IsAnyPlayerinRange
  (bind _closest (CallFunction|GetClosestPlayer))
  (return (< (Transformation|GetDistanceTo _closest) (Variables|Default|GetMinDist))))

(fn Disappear
  (params (MoveToPoint :type Boolean))
  (if MoveToPoint
    (Utilities|Time|SetTimerbyFunctionName 0 "ReappearAtPoint" 1.5)
    (else
      (Utilities|Time|SetTimerbyFunctionName 0 "Reappear" 3.0)))
  (Variables|Default|SetIsBlinking true)
  (CallFunction|MakeShadows)
  (Rendering|SetVisibility (Variables|Character|GetMesh) false true)
  (Audio|Components|Audio|Play (Variables|Default|GetVOICE_Male_B_Haha_Evil_01_mono) 0.0)
  (Utilities|Time|PauseTimerbyHandle (Variables|Default|GetAttackTimer))
  (Variables|/Script/Engine.PrimitiveComponent|SetbGenerateOverlapEvents (Variables|Default|GetCapsuleComponent) false))

(fn Reappear
  (CallFunction|GetClosestPlayer)
  (LocalVariables|SetBlinkTarget (Variables|Default|GetClosestHero))
  (if (Utilities|IsValid (LocalVariables|GetBlinkTarget))
    (Audio|Components|Audio|Play (Variables|Default|GetMAGIC_SPELL_Teleport_mono) 0.0)
    (while (not (LocalVariables|GetPointValid))
      (bind _output_get (LocalVariables|SetBlinkLocation (+ (Math|Vector|RotateVector (* (Transformation|GetActorForwardVector (LocalVariables|GetBlinkTarget)) (Variables|Default|GetRange)) (Math|Rotator|MakeRotator 0.0 0.0 (Math|Random|RandomFloatinRange 0.0 3.6e+02))) (Transformation|GetActorLocation (LocalVariables|GetBlinkTarget)))))
      (bind _returnvalue (Collision|LineTraceByChannel (Transformation|GetActorLocation) _output_get "TraceTypeQuery1" true 0 "None"))
      (LocalVariables|SetPointValid (not _returnvalue)))
    ;[1 1 1] Do the actual blinking once you've figured out a good blink location
    (Transformation|SetActorLocation (LocalVariables|GetBlinkLocation) false true)
    (Transformation|SetActorRotation (Math|Rotator|FindLookatRotation (Transformation|GetActorLocation) (Transformation|GetActorLocation (LocalVariables|GetBlinkTarget))))
    (Variables|Default|SetIsBlinking false)
    (Rendering|SetVisibility (Variables|Character|GetMesh) true true)
    (CallFunction|MakeShadows)
    (Variables|/Script/Engine.PrimitiveComponent|SetbGenerateOverlapEvents (Variables|Default|GetCapsuleComponent) true)
    (if (not (Variables|Default|GetCasting))
      (Utilities|Time|SetTimerbyFunctionName 0 "MeleeAttack" 0.2))))

(fn GetClosestPlayer
  (for _array_element (Variables|Default|GetPlayers)
    (LocalVariables|Setcurr _array_element)
    ;[1 1 1] Figure out if the current player is the closest player
    (if (and (<= (Transformation|GetDistanceTo (LocalVariables|Getcurr)) (LocalVariables|GetClosestDistance)) (not (Variables|/Script/PlaygroundHeroes.JHero|GetbHasFallen (LocalVariables|Getcurr))))
      (LocalVariables|SetClosestPlayer (LocalVariables|Getcurr))
      (LocalVariables|SetClosestDistance (Transformation|GetDistanceTo (LocalVariables|Getcurr)))
      ;[1 1 1] If any player is out of zorrander's range, we only care about how far they are so we'll ignore the second part of seeing the delta angle
      (if (< (Transformation|GetDistanceTo (LocalVariables|Getcurr)) (Variables|Default|GetRange))
        (LocalVariables|SetBothInRange false)
        (elif (<= (.Yaw (Math|Rotator|BreakRotator (Math|Rotator|Delta(Rotator) (Transformation|GetActorRotation) (Math|Rotator|FindLookatRotation (Transformation|GetActorLocation) (Transformation|GetActorLocation (LocalVariables|Getcurr)))))) (LocalVariables|GetLowestAngleDiff))
          (LocalVariables|SetLowestAnglePlayer (LocalVariables|Getcurr))
          (LocalVariables|SetLowestAngleDiff (.Yaw (Math|Rotator|BreakRotator (Math|Rotator|Delta(Rotator) (Transformation|GetActorRotation) (Math|Rotator|FindLookatRotation (Transformation|GetActorLocation) (Transformation|GetActorLocation (LocalVariables|Getcurr)))))))
          (else
            ;[1 1 1] If they are both in front of zorrander, we only care about the closest player
            (if (> (.Yaw (Math|Rotator|BreakRotator (Math|Rotator|Delta(Rotator) (Transformation|GetActorRotation) (Math|Rotator|FindLookatRotation (Transformation|GetActorLocation) (Transformation|GetActorLocation (LocalVariables|Getcurr)))))) 15.0)
              (LocalVariables|SetBothLessThan15 false)))))))
  (if (LocalVariables|GetBothInRange)
    (return (LocalVariables|GetClosestPlayer))
    (elif (LocalVariables|GetBothLessThan15)
      (return (LocalVariables|GetClosestPlayer))
      (else
        (LocalVariables|SetClosestPlayer (LocalVariables|GetLowestAnglePlayer))))))

(fn TestforBlink
  (bind _out (CallFunction|IsAnyPlayerinRange))
  (if (and (not _out) (not (Variables|Default|GetIsBlinking)))
    (if (not (Utilities|Time|IsTimerActivebyHandle (Variables|Default|GetDisappearTimer)))
      (bind _returnvalue (Utilities|Time|SetTimerbyFunctionName 0 "Disappear" 1.7))
      (Variables|Default|SetDisappearTimer _returnvalue))
    (elif (and _out (not (Variables|Default|GetIsBlinking)))
      (Utilities|Time|ClearandInvalidateTimerbyHandle (Variables|Default|GetDisappearTimer)))))

(fn MeleeAttack
  (Variables|Default|SetbAttacking true))

(fn QueueAttack
  (Utilities|Time|ClearandInvalidateTimerbyHandle (Variables|Default|GetAttackTimer))
  (bind _returnvalue (Utilities|Time|SetTimerbyFunctionName 0 "MeleeAttack" (Variables|Default|GetAttackSpeed)))
  (Variables|Default|SetAttackTimer _returnvalue))

(fn CastSpell
  (Utilities|Time|SetTimerbyFunctionName 0 (Utilities|Array|Get(acopy) (Variables|Default|GetSpellNames) (Math|Random|RandomIntegerinRange 0 (- (Utilities|Array|Length (Variables|Default|GetSpellNames)) 1))) 0.3))

(fn DarkHook
  (Animation|Montage|MontagePlay (Components|SkeletalMesh|GetAnimInstance (Variables|Character|GetMesh)) "/Game/ZorranderAssets/Animations/DarkHookMontage.DarkHookMontage" 1.0 "MontageLength" 0.0 true)
  (Audio|Components|Audio|Play (Variables|Default|GetMAGIC_SPELL_Passing_Tunnel_Sci-Fi_Fast_Rapid_Echo_stereo) 0.0)
  (CallFunction|QueueAttack))

(fn EvilOrb
  (Animation|Montage|MontagePlay (Components|SkeletalMesh|GetAnimInstance (Variables|Character|GetMesh)) "/Game/ZorranderAssets/Animations/OrbMontage.OrbMontage" 0.4 "MontageLength" 0.0 true)
  (Audio|Components|Audio|Play (Variables|Default|GetMAGIC_SPELL_Rumble_Spooky_Vibrato_Fade_In_Out_stereo) 0.0)
  (CallFunction|QueueAttack))

(fn DarkBolt
  (Animation|Montage|MontagePlay (Components|SkeletalMesh|GetAnimInstance (Variables|Character|GetMesh)) "/Game/ZorranderAssets/Animations/DarkBoltMontage.DarkBoltMontage" 1.0 "MontageLength" 0.0 true)
  (CallFunction|QueueAttack))

(fn MoveTowardsPlayer
  (params (Target :type J%20Hero%20Object%20Reference))
  (if (Utilities|IsValid Target)
    (LocalVariables|SetPlayer Target)
    (LocalVariables|SetDiff (- (Transformation|GetActorLocation Target) (Transformation|GetActorLocation)))
    (LocalVariables|SetSweetSpotRange (* 0.8 (Variables|Default|GetRange)))
    (CallFunction|RotateTowardsTarget (Utilities|Time|GetWorldDeltaSeconds) (LocalVariables|GetPlayer) true)
    (if (not (<= (Math|Float|Absolute(Float) (- (Math|Vector|VectorLength (LocalVariables|GetDiff)) (LocalVariables|GetSweetSpotRange))) 25.0))
      (if (< (Math|Vector|VectorLength (LocalVariables|GetDiff)) (LocalVariables|GetSweetSpotRange))
        (Class|PawnMovementComponent|AddInputVector (Variables|Character|GetCharacterMovement) (* (Math|Vector|Normalize (LocalVariables|GetDiff)) -0.2) false)
        (else
          (Class|PawnMovementComponent|AddInputVector (Variables|Character|GetCharacterMovement) (* (Math|Vector|Normalize (LocalVariables|GetDiff)) 0.2) false))))))

(fn ClearHeroesHit
  (Utilities|Array|Clear (Variables|Default|GetHeroesHit)))

(fn StaminaDrain
  (params (DeltaTime :type Float%20%28single-precision%29))
  (LocalVariables|SetLDeltaTime DeltaTime)
  (if (Utilities|IsValid (Variables|Default|GetClosestHero))
    (if (Variables|Default|GetCasting)
      (Rendering|SetVisibility (Variables|Default|GetStamDrain) false true)
      (for _array_element (Variables|Default|GetPlayers)
        (Class|JHero|SetMaxStamina _array_element (+ (Variables|/Script/PlaygroundHeroes.JHero|GetMaxStamina _array_element) (* 6e+01 (LocalVariables|GetLDeltaTime)))))
      (else
        (bind _out (CallFunction|IsAnyPlayerinRange))
        (if (and _out (not (Variables|Default|GetIsBlinking)))
          (Rendering|SetVisibility (Variables|Default|GetStamDrain) true true)
          (Class|JHero|SetMaxStamina (Variables|Default|GetClosestHero) (- (Variables|/Script/PlaygroundHeroes.JHero|GetMaxStamina (Variables|Default|GetClosestHero)) (* (LocalVariables|GetLDeltaTime) 5.0)))
          (Transformation|SetWorldScale3D (Variables|Default|GetStamDrain) (Math|Vector|MakeVector (/ (Transformation|GetDistanceTo (Variables|Default|GetClosestHero)) 1e+02) 0.5 0.5))
          (Transformation|SetWorldRotation (Variables|Default|GetStamDrain) (Math|Rotator|FindLookatRotation (Transformation|GetActorLocation) (Transformation|GetActorLocation (Variables|Default|GetClosestHero))) false false)
          (Transformation|SetWorldLocation (Variables|Default|GetStamDrain) (Math|Vector|Lerp(Vector) (Transformation|GetActorLocation) (Transformation|GetActorLocation (Variables|Default|GetClosestHero)) 0.5) false false)
          (else
            (Rendering|SetVisibility (Variables|Default|GetStamDrain) false true)))
        (for (_array_element_2 _array_index) (Variables|Default|GetPlayers)
          (if (== _array_element_2 (Variables|Default|GetClosestHero))
            (Utilities|Array|SetArrayElem (Variables|Default|GetDrainedTimers) _array_index -1.0)
            (elif (< (Utilities|Array|Get(acopy) (Variables|Default|GetDrainedTimers) _array_index) 0.5)
              (Utilities|Array|SetArrayElem (Variables|Default|GetDrainedTimers) _array_index (+ (Utilities|Array|Get(acopy) (Variables|Default|GetDrainedTimers) _array_index) (LocalVariables|GetLDeltaTime)))
              (else
                (Class|JHero|SetMaxStamina _array_element_2 (+ (Variables|/Script/PlaygroundHeroes.JHero|GetMaxStamina _array_element_2) (* 6e+01 (LocalVariables|GetLDeltaTime))))))))))))

(fn ChooseRandomVictim
  (bind _players (Variables|Default|GetPlayers))
  (bind _players_2 (Variables|Default|GetPlayers))
  (bind _returnvalue (Utilities|Array|Length _players))
  (bind _returnvalue_2 (Math|Random|RandomInteger _returnvalue))
  (bind _output (Utilities|Array|Get(acopy) _players _returnvalue_2))
  (if (not (Variables|/Script/PlaygroundHeroes.JHero|GetbHasFallen _output)) ; if player has not fallen
    (return _output)
    (elif (== _returnvalue_2 0)
      (return (Utilities|Array|Get(acopy) _players_2 1))
      (else
        (return (Utilities|Array|Get(acopy) _players_2))))))

(fn MegaSmash
  (for _array_element (Variables|Default|GetSmashPoints)
    (if (>= (Transformation|GetDistanceTo _array_element) (LocalVariables|GetFurthestDistance))
      (LocalVariables|SetFurthestDistance (Transformation|GetDistanceTo _array_element))
      (LocalVariables|SetFurthestPoint _array_element)))
  (CallFunction|Disappear true)
  (Audio|Components|Audio|Play (Variables|Default|GetFIRE_Campfire_Active_02_loop_mono) 0.0)
  (Audio|Components|Audio|Play (Variables|Default|GetCHARGE_Complex_Wet_12_Semi_Up_8000ms_stereo) 0.0)
  (Animation|Montage|MontagePlay (Components|SkeletalMesh|GetAnimInstance (Variables|Character|GetMesh)) "/Game/ZorranderAssets/Animations/SmashMontage.SmashMontage" 1.0 "MontageLength" 0.0 true)
  (Variables|Default|SetSmashing true)
  (Default|Activate (LocalVariables|GetFurthestPoint))
  (Audio|Components|Audio|Play (Variables|Default|GetCHARGE_Complex_Wet_12_Semi_Down_1000ms_stereo) 0.0)
  (Variables|Default|SetManualTPPoint (Math|Vector|MakeVector (.X (Math|Vector|BreakVector (Transformation|GetActorLocation (LocalVariables|GetFurthestPoint)))) (.Y (Math|Vector|BreakVector (Transformation|GetActorLocation (LocalVariables|GetFurthestPoint)))) (.Z (Math|Vector|BreakVector (Transformation|GetActorLocation))))))

(fn ReappearatPoint
  ;[1 1 1] Do the actual blinking once you've figured out a good blink location
  (Transformation|SetActorLocation (Variables|Default|GetManualTPPoint) false true)
  (Transformation|SetActorRotation (Math|Rotator|FindLookatRotation (Transformation|GetActorLocation) (Transformation|GetActorLocation (Variables|Default|GetClosestHero))))
  (Variables|Default|SetIsBlinking false)
  (Rendering|SetVisibility (Variables|Character|GetMesh) true true)
  (CallFunction|MakeShadows)
  (Variables|/Script/Engine.PrimitiveComponent|SetbGenerateOverlapEvents (Variables|Default|GetCapsuleComponent) true)
  (if (not (or (Variables|Default|GetCasting) (Variables|Default|GetSmashing)))
    (Utilities|Time|SetTimerbyFunctionName 0 "MeleeAttack" 0.2)))

(fn SpawnGrowZone
  (bind _newvictim (CallFunction|ChooseRandomVictim))
  (Game|SpawnActorfromClass "/Game/Blueprints/Zorrander/GrowingDamageZone.GrowingDamageZone_C" (Math|Transform|MakeTransform (Math|Vector|MakeVector (.X (Math|Vector|BreakVector (Transformation|GetActorLocation _newvictim))) (.Y (Math|Vector|BreakVector (Transformation|GetActorLocation _newvictim))) (.Z (Math|Vector|BreakVector (Transformation|GetWorldLocation (Variables|Default|GetFloorLocation))))) (Transformation|GetActorRotation)) "Undefined" 0 0.5 0)
  (Utilities|Time|SetTimerbyFunctionName 0 "SpawnGrowZone" (+ (Math|Random|RandomFloatinRange -0.5 0.5) 8.0)))

(fn BalefulGrasp
  (bind _returnvalue (Transformation|GetActorRotation))
  (bind _players (Variables|Default|GetPlayers))
  (bind (_roll _pitch) (Math|Rotator|BreakRotator _returnvalue))
  (if (not (or (Variables|/Script/PlaygroundHeroes.JHero|GetbHasFallen (Utilities|Array|Get(acopy) _players)) (Variables|/Script/PlaygroundHeroes.JHero|GetbHasFallen (Utilities|Array|Get(acopy) _players 1)))) ; don't do this attack if either have fallen
    (if (not (Variables|Default|GetisBlinking))
      (bind _newvictim (CallFunction|ChooseRandomVictim))
      (if (Utilities|IsValid _newvictim)
        (bind _output_get (Variables|Default|SetClosestHero _newvictim))
        (Variables|Default|SetCasting true)
        (if (>= (Transformation|GetDistanceTo _output_get) (LocalVariables|GetgraspNeedTeleportRange))
          (CallFunction|Disappear false)
          (Game|SpawnActorfromClass "/Game/Blueprints/Zorrander/Baleful_Grasp_Helper.Baleful_Grasp_Helper_C" (Transformation|GetActorTransform (Variables|Default|GetClosestHero)) "Undefined" 0 (Variables|Default|GetClosestHero) self 1e+01 3.0 0)
          (Audio|Components|Audio|Play (Variables|Default|GetVOICE_Girl_4yo_Hurt_Long_02_mono) 0.0)
          (else
            (Transformation|SetActorRotation (Math|Rotator|MakeRotator _roll _pitch (.Yaw (Math|Rotator|BreakRotator (Math|Rotator|FindLookatRotation (Transformation|GetActorLocation) (Transformation|GetActorLocation (Variables|Default|GetClosestHero)))))))
            (Game|SpawnActorfromClass "/Game/Blueprints/Zorrander/Baleful_Grasp_Helper.Baleful_Grasp_Helper_C" (Transformation|GetActorTransform (Variables|Default|GetClosestHero)) "Undefined" 0 (Variables|Default|GetClosestHero) self 1e+01 0.0 0)))))))

(fn ResetDamageBuildupMOVEOVER
  (Development|PrintString "Reset")
  (Variables|Default|SetDamageBuildUp%20MOVE%20OVER 0.0))