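; Manages the Zorrander Jr split phase of the Zorrander boss fight for two players, archer and knight.
; On BeginPlay it teleports both to tagged split points, then activates the placed Zorrander_Jr actors after a delay.
; Tick ends the phase at two clears, destroying remaining juniors, flagging Zorrander, returning players and destroying itself.
; A helper computes the juniors' combined health, but is not called here, and the health widget creation is unwired.
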(event EventBeginPlay
  (CallFunction|TeleportPlayers) ; Requires Tagged Teleport points
  (Utilities|FlowControl|Delay 1.0)
  (CallFunction|SpawnMiniZorranders))

(event Collision|EventActorBeginOverlap
  (params (OtherActor :type Actor%20Object%20Reference)))

(event EventTick
  (params (DeltaSeconds :type Float%20%28single-precision%29))
  (if (== (Variables|Default|GetminiZorsCleared) 2)
    (CallFunction|EndPhase)))

(fn ConstructionScript
  (bind _outactors (Actor|GetAllActorsOfClass "/Game/Blueprints/UI/JDialogueHandler.JDialogueHandler_C"))
  (Variables|Default|SetDialogHandler (Utilities|Array|Get(acopy) _outactors)))

(fn TeleportPlayers
  (bind _outactors (Actor|GetAllActorsOfClass "/Game/Blueprints/Zorrander/teleportPoint.teleportPoint_C"))
  (for _array_element _outactors
    (if (Actor|ActorHasTag _array_element "archerSplitPoint")
      (Transformation|SetActorLocationAndRotation (Game|Player|GetPlayerPawn 0) (.location (Transformation|GetActorTransform _array_element)) (.rotation (Transformation|GetActorTransform _array_element)) false true)
      (elif (Actor|ActorHasTag _array_element "knightSplitPoint")
        (Transformation|SetActorLocationAndRotation (Game|Player|GetPlayerPawn 1) (.location (Transformation|GetActorTransform _array_element)) (.rotation (Transformation|GetActorTransform _array_element)) false true)))))

(fn SpawnMiniZorranders
  (bind _outactors (Actor|GetAllActorsOfClass "/Game/Blueprints/Zorrander/Zorrander_Jr.Zorrander_Jr_C"))
  (bind _output_get (Variables|Default|SetZorranderJrs _outactors))
  (for _array_element _output_get
    (Default|BattleActivate _array_element)))

(fn UpdateCollectiveHealth
  (bind _zorranderjrs (Variables|Default|GetZorranderJrs))
  (bind _collectivehealthmax (Variables|Default|GetcollectiveHealthMax))
  (bind _output (Utilities|Array|Get(acopy) _zorranderjrs))
  (bind _output_2 (Utilities|Array|Get(acopy) _zorranderjrs 1))
  (if (and (Utilities|IsValid _output) (Utilities|IsValid _output_2))
    (LocalVariables|SetFirstZorDamage (- (Variables|/Script/PlaygroundHeroes.JEnemy|GetmaxHealth _output) (Variables|/Script/PlaygroundHeroes.JEnemy|GetHealth _output)))
    (LocalVariables|SetSecondZorDamage (- (Variables|/Script/PlaygroundHeroes.JEnemy|GetmaxHealth _output_2) (Variables|/Script/PlaygroundHeroes.JEnemy|GetHealth _output_2)))
    (bind _output_get (Variables|Default|SetcollectiveHealth (Math|Float|Clamp(Float) (- _collectivehealthmax (+ (LocalVariables|GetFirstZorDamage) (LocalVariables|GetSecondZorDamage))) 0.0 _collectivehealthmax)))
    (Variables|Default|SetCollectiveHealthPercent (/ _output_get (Variables|Default|GetcollectiveHealthMax)))))

(fn EndPhase
  (bind _zorranderjrs (Variables|Default|GetZorranderJrs))
  (bind _output (Utilities|Array|Get(acopy) _zorranderjrs))
  (bind _output_2 (Utilities|Array|Get(acopy) _zorranderjrs 1))
  ;[1 1 1] If either Zorrander Jr is still Alive, kill them
  (if (Utilities|IsValid _output)
    (Actor|DestroyActor _output))
  (if (Utilities|IsValid _output_2)
    (Actor|DestroyActor _output_2))
  (Variables|/Game/Blueprints/Zorrander/Zorrander.Zorrander_C|SetZorChilldrenKilled (Variables|Default|GetZorrander) true)
  ;[1 1 1] Return players to main Arena
  (bind _outactors (Actor|GetAllActorsOfClass "/Game/Blueprints/Zorrander/teleportPoint.teleportPoint_C"))
  (for _array_element _outactors
    (if (Actor|ActorHasTag _array_element "archerReturnPoint")
      (Transformation|SetActorLocation (Game|Player|GetPlayerPawn 0) (Transformation|GetActorLocation _array_element) false true)
      (elif (Actor|ActorHasTag _array_element "knightReturnPoint")
        (Transformation|SetActorLocation (Game|Player|GetPlayerPawn 1) (Transformation|GetActorLocation _array_element) false true))))
  (Variables|/Game/Blueprints/Zorrander/Zorrander.Zorrander_C|SetZorChilldrenKilled (Variables|Default|GetZorrander) true)
  (Actor|DestroyActor))