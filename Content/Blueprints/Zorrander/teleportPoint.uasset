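; Teleport point actor for the Zorrander level that sends a Zorrander Jr. Wall back when the hero passes through.
; On BeginPlay, if flagged as a teleport-back point, it finds the first Zorrander_Jr_Wall sharing its LevelZone and caches it.
; When a JHero enters DetectPassageBox, the box destroys itself, making it one-shot, and calls TeleportBack on the cached wall if valid.
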(event OnComponentBeginOverlap(DetectPassageBox)
  (params (OverlappedComponent :type Primitive%20Component%20Object%20Reference) (OtherActor :type Actor%20Object%20Reference) (OtherComp :type Primitive%20Component%20Object%20Reference) (OtherBodyIndex :type Integer) (bFromSweep :type Boolean) (SweepResult :type Hit%20Result%20Structure%20%28by%20ref%29))
  (bind _zorjrref (Variables|Default|GetZorJrRef))
  (Utilities|Casting|CastToJHero OtherActor)
  (Components|DestroyComponent (Variables|Default|GetDetectPassageBox))
  (if (Utilities|IsValid _zorjrref)
    (Default|TeleportBack _zorjrref)))

(event EventBeginPlay
  (if (Variables|Default|GetteleportBackPoint)
    (bind _outactors (Actor|GetAllActorsOfClass "/Game/Blueprints/Zorrander/Zorrander_Jr_Wall.Zorrander_Jr_Wall_C"))
    (bind _array_element (Utilities|Array|ForEachLoopwithBreak _outactors :!label _label)
      (:LoopBody
        (if (Utilities|Name|Equal(Name) (Variables|/Game/Blueprints/Zorrander/Zorrander_Jr_Wall.Zorrander_Jr_Wall_C|GetlevelZone _array_element) (Variables|Default|GetlevelZone))
          (Variables|Default|SetZorJrRef _array_element)
          (goto _label Break))))))

(event Collision|EventActorBeginOverlap
  (params (OtherActor :type Actor%20Object%20Reference)))

(event EventTick
  (params (DeltaSeconds :type Float%20%28single-precision%29)))

(fn ConstructionScript)