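; SmashKnight is a guardian knight that, with a guarding archer, keeps Zor invincible and shows a beam linking itself to Zor.
; Each tick, ChangeBeam centers the Beam component between knight and Zor, rotates it toward Zor and scales its length by their distance.
; On death it flags itself dead in SmashHelper, clears Zor's invincibility if the archer is also dead, then destroys itself.
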(event EventBeginPlay
  (|CallParentFunction) ; This node is disabled and will not be called.\nDrag off pins to build functionality.
)

(event Collision|EventActorBeginOverlap
  (params (OtherActor :type Actor%20Object%20Reference))
  (|CallParentFunction OtherActor) ; This node is disabled and will not be called.\nDrag off pins to build functionality.
)

(event EventTick
  (params (DeltaSeconds :type Float%20%28single-precision%29))
  (|CallParentFunction DeltaSeconds)
  (CallFunction|ChangeBeam))

(event EventDie
  (bind _smashhelper (Variables|Default|GetsmashHelper))
  (bind _output_get (Variables|/Game/Blueprints/Zorrander/SmashHelper.SmashHelper_C|SetguardingKnightDead _smashhelper true))
  (if (and _output_get (Variables|/Game/Blueprints/Zorrander/SmashHelper.SmashHelper_C|GetguardingArcherDead _smashhelper))
    (Variables|/Game/Blueprints/Enemies/JEnemyBP_Bar.JEnemyBP_Bar_C|Setinvincible (Variables|/Game/Blueprints/Zorrander/SmashHelper.SmashHelper_C|GetZorReference _smashhelper) false))
  (Actor|DestroyActor))

(fn ConstructionScript
  (|CallParentFunction))

(fn ChangeBeam
  (bind _returnvalue (Transformation|GetActorLocation))
  (bind _beam (Variables|Default|Getbeam))
  (LocalVariables|SetzorRef (Variables|/Game/Blueprints/Zorrander/SmashHelper.SmashHelper_C|GetZorReference (Variables|Default|GetsmashHelper)))
  (Transformation|SetWorldScale3D (Variables|Default|Getbeam) (Math|Vector|MakeVector (/ (Transformation|GetDistanceTo (LocalVariables|GetzorRef)) 1e+02) 0.5 0.5))
  (Transformation|SetWorldLocation _beam (+ (* (Math|Vector|GetForwardVector (Math|Rotator|FindLookatRotation _returnvalue (Transformation|GetActorLocation (LocalVariables|GetzorRef)))) (/ (Transformation|GetDistanceTo (LocalVariables|GetzorRef)) 2.0)) _returnvalue) false false)
  (Transformation|SetWorldRotation _beam (Math|Rotator|FindLookatRotation _returnvalue (Transformation|GetActorLocation (LocalVariables|GetzorRef))) false false))