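; Fireball projectile that arcs toward a hero, either a preset Victim or a random pick, and applies Damage with a stagger on overlap.
; BeginPlay ground-traces a point leading the victim's velocity, spawns an indicator there and derives TravelTime, though the lead reads TravelTime before that update.
; Tick moves it along a computed parabola until arrival or hit, then removes indicator and spheres, triggers particles and self-destroys when they finish.
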(event OnComponentBeginOverlap(SphereCollider)
  (params (OverlappedComponent :type Primitive%20Component%20Object%20Reference) (OtherActor :type Actor%20Object%20Reference) (OtherComp :type Primitive%20Component%20Object%20Reference) (OtherBodyIndex :type Integer) (bFromSweep :type Boolean) (SweepResult :type Hit%20Result%20Structure%20%28by%20ref%29))
  (bind _asjhero (Utilities|Casting|CastToJHero OtherActor))
  (Class|JHero|AddHealth _asjhero (Variables|Default|Getdamage) 0.3)
  (Variables|Default|Settravelling false))

(event OnSystemFinished(ParticleSystem)
  (params (PSystem :type Particle%20System%20Component%20Object%20Reference))
  (Actor|DestroyActor))

(event EventBeginPlay
  (Variables|Movement|SetstartingPoint (Transformation|GetActorLocation))
  (if (Utilities|IsValid (Variables|Default|Getvictim))
    _
    (else
      (bind _outactors (Actor|GetAllActorsOfClass "/Script/PlaygroundHeroes.JHero"))
      (Variables|Default|Setvictim (Utilities|Array|Get(acopy) _outactors (Math|Random|RandomInteger 2)))))
  (CallFunction|CalculateTargetPoint)
  (bind _returnvalue (Game|SpawnActorfromClass "/Game/Blueprints/Zorrander/targetingFireballIndicator.targetingFireballIndicator_C" (Math|Transform|MakeTransform (Variables|Movement|GettargetPoint) "0, 0, 0" "3.000000,3.000000,2.000000") "Undefined" 0 0))
  (bind _output_get (Variables|Default|Setindicator _returnvalue))
  (Variables|Movement|SettravelTime (Math|Float|Clamp(Float) (/ (Transformation|GetHorizontalDistanceTo _output_get) (Variables|Movement|Getspeed)) 0.0 7.0)))

(event Collision|EventActorBeginOverlap
  (params (OtherActor :type Actor%20Object%20Reference)))

(event EventTick
  (params (DeltaSeconds :type Float%20%28single-precision%29))
  (Variables|Movement|SettimeTravelled (+ DeltaSeconds (Variables|Movement|GettimeTravelled)))
  (if (and (<= (Variables|Movement|GettimeTravelled) (Variables|Movement|GettravelTime)) (Variables|Default|Gettravelling))
    (CallFunction|CalculateNewLocation)
    (else
      (Utilities|FlowControl|DoOnce false
        (:Completed
          (Actor|DestroyActor (Variables|Default|Getindicator))
          (Components|Activation|Activate (Variables|Default|GetParticleSystem) false)
          (Components|DestroyComponent (Variables|Default|GetSphere))
          (Components|DestroyComponent (Variables|Default|GetSphereCollider))
          (Components|DestroyComponent (Variables|Default|GetSphere1)))))))

(fn ConstructionScript)

(fn CalculateTargetPoint
  (bind _traveltime (Variables|Movement|GettravelTime))
  (bind _victim (Variables|Default|Getvictim))
  (bind _victim_2 (Variables|Default|Getvictim))
  (bind _returnvalue (Transformation|GetActorForwardVector _victim))
  (bind _returnvalue_2 (Transformation|GetVelocity _victim))
  (bind _returnvalue_3 (Transformation|GetActorLocation _victim_2))
  (bind _returnvalue_4 (* _traveltime 0.6))
  (bind _returnvalue_5 (* _returnvalue_2 _returnvalue_4))
  (bind _returnvalue_6 (+ _returnvalue _returnvalue_5))
  (bind _returnvalue_7 (+ _returnvalue_6 _returnvalue_3))
  (bind _outhit (Collision|LineTraceByChannel _returnvalue_7 (- _returnvalue_7 "0, 0,500.000000") "TraceTypeQuery1" false 0 "None")) ; get location flush to the ground
  (Variables|Movement|SettargetPoint (.location _outhit)))

(fn CalculateNewLocation
  (bind _startingpoint (Variables|Movement|GetstartingPoint))
  (bind _targetpoint (Variables|Movement|GettargetPoint))
  (bind _timetravelled (Variables|Movement|GettimeTravelled))
  (bind _traveltime (Variables|Movement|GettravelTime))
  (bind _returnvalue (/ _timetravelled _traveltime))
  (bind _returnvalue_2 (Math|Vector|Lerp(Vector) _startingpoint _targetpoint _returnvalue))
  (Transformation|SetActorLocation (Math|Vector|MakeVector (.x _returnvalue_2) (.y _returnvalue_2) (+ (* (* (+ (Variables|Movement|GettimeTravelled) 1.0) (- (Variables|Movement|GettimeTravelled) (Variables|Movement|GettravelTime))) (* (Variables|Movement|GetriseFactor) -1.0)) (.z (Variables|Movement|GettargetPoint)) (* (- (.z (Variables|Movement|GetstartingPoint)) (.z (Variables|Movement|GettargetPoint))) (- 1.0 (/ (Variables|Movement|GettimeTravelled) (Variables|Movement|GettravelTime)))))) false false))

(fn Detonate
  (params (NewParam :type Actor%20Object%20Reference)))