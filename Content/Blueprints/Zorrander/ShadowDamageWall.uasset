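; Shadow damage wall that closes in along X toward world zero and hurts JHero characters inside its box.
; Activate starts moving it after a short delay, with Tick lerping its position over CloseInTime.
; Box overlaps track heroes and their looping one-second timers in parallel arrays.
; Timer function names are built from array index, so only DoDamage0 and DoDamage1 exist, applying damage and random hurt sounds for two heroes.
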(event OnComponentBeginOverlap(Box)
  (params (OverlappedComponent :type Primitive%20Component%20Object%20Reference) (OtherActor :type Actor%20Object%20Reference) (OtherComp :type Primitive%20Component%20Object%20Reference) (OtherBodyIndex :type Integer) (bFromSweep :type Boolean) (SweepResult :type Hit%20Result%20Structure%20%28by%20ref%29))
  (bind _asjhero (Utilities|Casting|CastToJHero OtherActor))
  (if (== (Utilities|Array|FindItem (Variables|Default|GetHeroes) _asjhero) -1)
    (bind _returnvalue (Utilities|Array|Add (Variables|Default|GetHeroes) _asjhero))
    (bind _returnvalue_2 (Utilities|Time|SetTimerbyFunctionName 0 (Utilities|String|Append "DoDamage" (Utilities|String|ToString(Integer) _returnvalue)) 1.0 true))
    (Utilities|Array|Insert (Variables|Default|GetDamageHandles) _returnvalue_2 _returnvalue)))

(event OnComponentEndOverlap(Box)
  (params (OverlappedComponent :type Primitive%20Component%20Object%20Reference) (OtherActor :type Actor%20Object%20Reference) (OtherComp :type Primitive%20Component%20Object%20Reference) (OtherBodyIndex :type Integer))
  (bind _asjhero (Utilities|Casting|CastToJHero OtherActor))
  (if (!= (Utilities|Array|FindItem (Variables|Default|GetHeroes) _asjhero) -1)
    (Utilities|Time|ClearandInvalidateTimerbyHandle (Utilities|Array|Get(acopy) (Variables|Default|GetDamageHandles) (Utilities|Array|FindItem (Variables|Default|GetHeroes) _asjhero)))
    (Utilities|Array|RemoveIndex (Variables|Default|GetDamageHandles) (Utilities|Array|FindItem (Variables|Default|GetHeroes) _asjhero))
    (Utilities|Array|RemoveIndex (Variables|Default|GetHeroes) (Utilities|Array|FindItem (Variables|Default|GetHeroes) _asjhero))))

(event EventBeginPlay
  (Variables|Default|SetinitXLocation (.x (Transformation|GetActorLocation)))
  (Variables|Default|SetfinalXLocation 0.0))

(event EventTick
  (params (DeltaSeconds :type Float%20%28single-precision%29))
  (bind _returnvalue (Transformation|GetActorLocation))
  (if (Variables|Default|GetbActive)
    (Variables|Default|SetriseProgress (+ DeltaSeconds (Variables|Default|GetriseProgress)))
    (Transformation|SetActorLocation (Math|Vector|MakeVector (Math|Float|Lerp (Variables|Default|GetinitXLocation) (Variables|Default|GetfinalXLocation) (/ (Variables|Default|GetriseProgress) (Variables|Default|GetcloseInTime))) (.y _returnvalue) (.z _returnvalue)) false false)))

(fn ConstructionScript)

(fn DoDamage0
  (bind _heroes (Variables|Default|GetHeroes))
  (bind _output (Utilities|Array|Get(acopy) _heroes))
  (if (Utilities|IsValid _output)
    (Class|JHero|AddHealth _output (* -1.0 (Variables|Default|GetDamage)) 0.0)
    (if (not (Variables|/Script/PlaygroundHeroes.JHero|GetbHasFallen _output))
      (switch int (Math|Random|RandomIntegerinRange 0 2)
        (:Default
          (Audio|Components|Audio|Play (Variables|Default|Gethurt%20short%201) 0.0 :!label _label))
        (:0
          (goto _label))
        (:1
          (Audio|Components|Audio|Play (Variables|Default|Gethurt%20short%204) 0.0))
        (:2
          (Audio|Components|Audio|Play (Variables|Default|GetHurt_Short%206) 0.0))))))

(fn DoDamage1
  (bind _heroes (Variables|Default|GetHeroes))
  (bind _output (Utilities|Array|Get(acopy) _heroes 1))
  (if (Utilities|IsValid _output)
    (Class|JHero|AddHealth _output (* -1.0 (Variables|Default|GetDamage)) 0.0)
    (if (not (Variables|/Script/PlaygroundHeroes.JHero|GetbHasFallen _output))
      (switch int (Math|Random|RandomIntegerinRange 0 2)
        (:Default
          (Audio|Components|Audio|Play (Variables|Default|Gethurt%20short%201) 0.0 :!label _label))
        (:0
          (goto _label))
        (:1
          (Audio|Components|Audio|Play (Variables|Default|Gethurt%20short%204) 0.0))
        (:2
          (Audio|Components|Audio|Play (Variables|Default|GetHurt_Short%206) 0.0))))))

(fn Activate
  (Utilities|Time|SetTimerbyFunctionName 0 "becomeActive" 3.0))

(fn BecomeActive
  (Variables|Default|SetbActive true)
  (Development|PrintString "becameActive"))