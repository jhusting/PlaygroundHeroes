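; Child variant of Zorrander, apparently a boss, that is bound to one player and one side of the arena.
; It overrides phase switching and stamina drain with empty events.
; Closest-player and random-victim selection both return the hero at the TargetPlayer index, printing a warning if the cast fails.
; PointInMyHalf tests points against a box spanning from an origin to an arena-floor bounds corner, chosen by TargetPlayer.
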(event EventBeginPlay
  (|CallParentFunction))

(event Collision|EventActorBeginOverlap
  (params (OtherActor :type Actor%20Object%20Reference))
  (|CallParentFunction OtherActor) ; This node is disabled and will not be called.\nDrag off pins to build functionality.
)

(event EventTick
  (params (DeltaSeconds :type Float%20%28single-precision%29))
  (|CallParentFunction DeltaSeconds) ; This node is disabled and will not be called.\nDrag off pins to build functionality.
)

(event EventPhaseSwitcher)

(event EventStaminaDrain
  (params (DeltaTime :type Float%20%28single-precision%29)))

(fn ConstructionScript
  (|CallParentFunction))

(fn GetClosestPlayer
  (bind _targetplayer (Variables|Default|GettargetPlayer))
  (bind _asjhero (Utilities|Casting|CastToJHero (Game|Player|GetPlayerPawn _targetplayer))
    (:then
      (return _asjhero))
    (:CastFailed
      (Development|PrintString (Utilities|String|Append (Utilities|String|Append (Utilities|String|MakeLiteralString "Warning: Player ") (Utilities|String|ToString(Integer) _targetplayer)) " missing!")))))

(fn ChooseRandomVictim
  (bind _targetplayer (Variables|Default|GettargetPlayer))
  (bind _asjhero (Utilities|Casting|CastToJHero (Game|Player|GetPlayerPawn _targetplayer))
    (:then
      (return _asjhero))
    (:CastFailed
      (Development|PrintString (Utilities|String|Append (Utilities|String|Append (Utilities|String|MakeLiteralString "Warning: Player ") (Utilities|String|ToString(Integer) _targetplayer)) " missing!")))))

(fn PointinMyHalf
  (params (testPoint :type Vector))
  (bind (_x _y) (Math|Vector|BreakVector testPoint))
  (bind _arenafloor (Variables|Default|GetArenaFloor))
  (bind _originpointy (LocalVariables|GetoriginPointY))
  (bind _originpointx (LocalVariables|GetoriginPointX))
  (bind (_origin _boxextent) (Collision|GetActorBounds _arenafloor true))
  (if (== (Variables|Default|GettargetPlayer) 0)
    (LocalVariables|Setside 1)
    (else
      (LocalVariables|Setside -1)))
  (LocalVariables|SetextentPointX (+ (.x _origin) (* (LocalVariables|Getside) (.x _boxextent))))
  (LocalVariables|SetextentPointY (+ (.y _origin) (* (LocalVariables|Getside) (.y _boxextent))))
  (return (and (or (and (>= _x _originpointx) (<= _x (LocalVariables|GetextentPointX))) (and (<= _x _originpointx) (>= _x (LocalVariables|GetextentPointX)))) (or (and (>= _y _originpointy) (<= _y (LocalVariables|GetextentPointY))) (and (<= _y _originpointy) (>= _y (LocalVariables|GetextentPointY)))))))