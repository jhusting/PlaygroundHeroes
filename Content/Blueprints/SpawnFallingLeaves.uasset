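; Spawner actor that continually drops FireLeaf actors into the level at random horizontal positions around itself.
; Tick runs through a Delay of SpawnRate, which acts as a repeating timer between spawns.
; Each spawn randomizes X and Y within the MaxXDistanceAwaySpawn and MaxYDistanceAwaySpawn ranges, keeping the spawner's height with zero rotation and unit scale.
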(event EventBeginPlay)

(event Collision|EventActorBeginOverlap
  (params (OtherActor :type Actor%20Object%20Reference)))

(event EventTick
  (params (DeltaSeconds :type Float%20%28single-precision%29))
  (bind _self self)
  (bind _maxxdistanceawayspawn (Variables|Default|GetMaxXDistanceAwaySpawn))
  (bind _maxydistanceawayspawn (Variables|Default|GetMaxYDistanceAwaySpawn))
  (bind _returnvalue (Transformation|GetActorLocation _self))
  (bind (_x _y _z) (Math|Vector|BreakVector _returnvalue))
  (Utilities|FlowControl|Delay (Variables|Default|GetSpawnRate))
  (Game|SpawnActorfromClass "/Game/Blueprints/FireLeaf.fireLeaf_C" (Math|Transform|MakeTransform (Math|Vector|MakeVector (+ (Math|Random|RandomFloatinRange (* _maxxdistanceawayspawn -1.0) _maxxdistanceawayspawn) _x) (+ (Math|Random|RandomFloatinRange (* _maxydistanceawayspawn -1.0) _maxydistanceawayspawn) _y) _z) "0, 0,0.000000") "Undefined" 0 0))

(fn ConstructionScript)