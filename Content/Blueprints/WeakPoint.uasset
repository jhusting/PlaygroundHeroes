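; WeakPoint is an actor that repeatedly spews Sap actors from an offset to its location.
; Tick runs through a Delay, so each shot fires roughly once per FireRate interval.
; CreateFiringProperties randomizes each Sap's launch speed and upward direction, biased toward positive X and independent of the actor's rotation.
; An alternative countdown timer based on DeltaSeconds is left disconnected and never runs.
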(event EventBeginPlay)

(event Collision|EventActorBeginOverlap
  (params (OtherActor :type Actor%20Object%20Reference)))

(event EventTick
  (params (DeltaSeconds :type Float%20%28single-precision%29))
  (Utilities|FlowControl|Delay (Variables|Default|GetfireRate))
  (bind (_directionvector _speed) (CallFunction|CreateFiringProperties))
  ;[1 1 1] Spawn at an offset location
  (Game|SpawnActorfromClass "/Game/Blueprints/Sap.Sap_C" (Math|Transform|MakeTransform (+ (Variables|Default|GetSpawnOffset) (Transformation|GetActorLocation)) (Transformation|GetActorRotation) (Transformation|GetActorScale3D)) "Undefined" 0 _directionvector _speed 0))

(fn ConstructionScript)

(fn CreateFiringProperties
  (return (Math|Vector|MakeVector (Math|Random|RandomFloatinRange 0.0 1e+01) (Math|Random|RandomFloatinRange -1e+01 1e+01) 1e+01) (Math|Random|RandomFloatinRange 3.5e+02 8e+02)))