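; Player 1 knight Blueprint that shows health and stamina bars and applies sword damage to JEnemy actors.
; Sword capsule overlap and overlap-style custom events call CauseDamage while CanDamage is set, ignoring JKnight hits.
; The custom events use DoOnce gates that reset after a short delay once CanDamage is off.
; CauseDamage has a hardcoded true branch, so only sword-tip damage applies; some disconnected nodes remain.
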(event OnComponentBeginOverlap(SwordBodyCollisionCapsule)
  (params (OverlappedComponent :type Primitive%20Component%20Object%20Reference) (OtherActor :type Actor%20Object%20Reference) (OtherComp :type Primitive%20Component%20Object%20Reference) (OtherBodyIndex :type Integer) (bFromSweep :type Boolean) (SweepResult :type Hit%20Result%20Structure%20%28by%20ref%29))
  (if (Variables|Default|GetbCanDamage self)
    (bind _asjenemy (Utilities|Casting|CastToJEnemy OtherActor)
      (:then
        (CallFunction|CauseDamage _asjenemy))
      (:CastFailed
        ;[1 1 1] Did you hit yourself?
        (Utilities|Casting|CastToJKnight OtherActor
          (:CastFailed
            (Development|PrintString "JKnightSwordCollision: Cast Failed") ; You hit something that isn't a JEnemy or Yourself
          ))))))

(event OnComponentEndOverlap(SwordBodyCollisionCapsule)
  (params (OverlappedComponent :type Primitive%20Component%20Object%20Reference) (OtherActor :type Actor%20Object%20Reference) (OtherComp :type Primitive%20Component%20Object%20Reference) (OtherBodyIndex :type Integer)))

(event Custom|CustomEvent
  (params (OverlappedComponent :type Primitive%20Component%20Object%20Reference) (OtherActor :type Actor%20Object%20Reference) (OtherComp :type Primitive%20Component%20Object%20Reference) (OtherBodyIndex :type Integer) (bFromSweep :type Boolean) (SweepResult :type Hit%20Result%20Structure%20%28by%20ref%29))
  (Utilities|FlowControl|DoOnce false
    (:Completed
      (if (Variables|Default|GetbCanDamage)
        (Variables|Default|SetSwordBodyHit true)
        (bind _asjenemy (Utilities|Casting|CastToJEnemy OtherActor)
          (:then
            (CallFunction|CauseDamage _asjenemy))
          (:CastFailed
            ;[1 1 1] Did you hit yourself?
            (Utilities|Casting|CastToJKnight OtherActor
              (:CastFailed
                (Development|PrintString "JKnightSwordCollision: Cast Failed") ; You hit something that isn't a JEnemy or Yourself
              ))))))))

(event Custom|CustomEvent_1
  (params (OverlappedComponent :type Primitive%20Component%20Object%20Reference) (OtherActor :type Actor%20Object%20Reference) (OtherComp :type Primitive%20Component%20Object%20Reference) (OtherBodyIndex :type Integer) (bFromSweep :type Boolean) (SweepResult :type Hit%20Result%20Structure%20%28by%20ref%29))
  (Utilities|FlowControl|DoOnce false
    (:Completed
      (if (Variables|Default|GetbCanDamage)
        (bind _asjenemy (Utilities|Casting|CastToJEnemy OtherActor)
          (:then
            (CallFunction|CauseDamage _asjenemy))
          (:CastFailed
            ;[1 1 1] Did you hit yourself?
            (Utilities|Casting|CastToJKnight OtherActor
              (:CastFailed
                (Development|PrintString "JKnightSwordCollision: Cast Failed") ; You hit something that isn't a JEnemy or Yourself
              ))))))))

(event Custom|CustomEvent_2
  (params (OverlappedComponent :type Primitive%20Component%20Object%20Reference) (OtherActor :type Actor%20Object%20Reference) (OtherComp :type Primitive%20Component%20Object%20Reference) (OtherBodyIndex :type Integer))
  (bind _bcandamage (Variables|Default|GetbCanDamage))
  (if (not _bcandamage)
    (Utilities|FlowControl|Delay 0.5)
    (Utilities|FlowControl|DoOnce false) ; enters at Reset
  ))

(event Custom|CustomEvent_3
  (params (OverlappedComponent :type Primitive%20Component%20Object%20Reference) (OtherActor :type Actor%20Object%20Reference) (OtherComp :type Primitive%20Component%20Object%20Reference) (OtherBodyIndex :type Integer))
  (bind _bcandamage (Variables|Default|GetbCanDamage))
  (if (not _bcandamage)
    (Utilities|FlowControl|Delay 0.3)
    (Utilities|FlowControl|DoOnce false) ; enters at Reset
  ))

(event EventBeginPlay
  (bind _returnvalue (UserInterface|CreateWidget "/Game/Blueprints/Player1HealthBar.Player1HealthBar_C"))
  (UserInterface|Viewport|AddtoViewport _returnvalue 0)
  (bind _returnvalue_2 (UserInterface|CreateWidget "/Game/Blueprints/Player1StaminaBar.Player1StaminaBar_C"))
  (UserInterface|Viewport|AddtoViewport _returnvalue_2 0))

(event Collision|EventActorBeginOverlap
  (params (OtherActor :type Actor%20Object%20Reference)))

(event EventTick
  (params (DeltaSeconds :type Float%20%28single-precision%29)))

(fn ConstructionScript)

(fn CauseDamage
  (params (Enemy%20Hit :type J%20Enemy%20Object%20Reference))
  (if true ; Only hit with tip??
    ;[1 1 1] Sword Tip Only Hit Damage
    (Class|JEnemy|AddHealth Enemy%20Hit (* (* (Variables|Default|GetSwordTipDamage) (Variables|Default|GetSwordTipDamageModifier)) -1.0))
    (Development|PrintString "Tip")
    (else
      ;[1 1 1] Sword Body Hit Damage
      (Class|JEnemy|AddHealth Enemy%20Hit (* (* (Variables|Default|GetSwordBodyDamage) (Variables|Default|GetSwordBodyDamageMultiplier)) -1.0))))
  ;[1 1 1] Reset JustTheTip and SwordBodyHit
  (Variables|Default|SetJustTheTip false)
  (Variables|Default|SetSwordBodyHit false))