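; shadowCaster is a short-lived actor whose Cylinder mesh grows over time and then removes itself.
; Construction records the cylinder's world scale as BaseScale and sets the actor's rotation to SpawnRotation.
; Tick accumulates time and multiplies BaseScale by time squared times GrowthRate, clamped to MaxScale.
; Once that multiplier reaches MaxScale, scaling stops and the actor is destroyed after a short delay.
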(event EventBeginPlay)

(event Collision|EventActorBeginOverlap
  (params (OtherActor :type Actor%20Object%20Reference)))

(event EventTick
  (params (DeltaSeconds :type Float%20%28single-precision%29))
  (bind _maxscale (Variables|Default|GetmaxScale))
  ;[1 1 1] .5x^2 - x
  (bind _output_get (Variables|Default|SettimeTrack (+ DeltaSeconds (Variables|Default|GettimeTrack))))
  (if (== (Math|Float|Clamp(Float) (* (* (Math|Float|Power _output_get 2.0) 1.0) (Variables|Default|GetGrowthRate)) 0.0 _maxscale) _maxscale)
    (Utilities|FlowControl|Delay 0.2)
    (Actor|DestroyActor)
    (else
      (Transformation|SetWorldScale3D (Variables|Default|GetCylinder) (* (Variables|Default|GetBaseScale) (Math|Float|Clamp(Float) (* (* (Math|Float|Power _output_get 2.0) 1.0) (Variables|Default|GetGrowthRate)) 0.0 _maxscale))))))

(fn ConstructionScript
  (Variables|Default|SetBaseScale (Transformation|GetWorldScale (Variables|Default|GetCylinder)))
  (Transformation|SetActorRotation (Variables|Default|GetspawnRotation) true))